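; BP_Gatherable is an interactable resource in Racketeers that awards a point to the player who gathers it.
; On authority, Interact runs once, sets GatherState to gathered and adds score through BP_BaseGameMode.
; Remote calls increment the instigator's PlayerScore locally, without the once-only guard.
; OnRep_GatherState swaps the Resource mesh to show the gathered state, while CanInteract simply returns its variable.
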(event EventInteract
  (params (Instigator :type Actor%20Object%20Reference))
  (Networking|SwitchHasAuthority
    (:Authority
      ;[1 1 1] Server Logic
      (Utilities|FlowControl|DoOnce false
        (:Completed
          (Utilities|FlowControl|Sequence
            (:then_0
              (Variables|Default|SetGatherState "NewEnumerator2"))
            (:then_1
              (bind _asbp_player (Utilities|Casting|CastToBP_Player Instigator))
              (bind _asbp_player_state (Utilities|Casting|CastToBP_PlayerState (Variables|/Script/Engine.Pawn|GetPlayerState _asbp_player)))
              (bind _asbp_gm_base (Utilities|Casting|CastToBP_BaseGameMode (Game|GetGameMode)))
              (Default|AddScore _asbp_gm_base 1 _asbp_player_state))))))
    (:Remote
      ;[1 1 1] Client Logic
      (bind _asbp_player_2 (Utilities|Casting|CastToBP_Player Instigator))
      (bind _asbp_player_state_2 (Utilities|Casting|CastToBP_PlayerState (Variables|/Script/Engine.Pawn|GetPlayerState _asbp_player_2)))
      (Variables|/Game/Racketeers/BP_PlayerState.BP_PlayerState_C|SetPlayerScore _asbp_player_state_2 (+ (Variables|/Game/Racketeers/BP_PlayerState.BP_PlayerState_C|GetPlayerScore _asbp_player_state_2) 1)))))

(fn ConstructionScript)

(fn CanInteract
  (return (Variables|Default|GetbCanInteract)))

(fn OnRepGatherState
  (switch Utilities|FlowControl|Switch|SwitchonE_GatherableStates (Variables|Default|GetGatherState)
    (:NewEnumerator2
      (Components|StaticMesh|SetStaticMesh (Variables|Default|GetResource) "/ControlRig/Controls/ControlRig_Box_3mm.ControlRig_Box_3mm"))))