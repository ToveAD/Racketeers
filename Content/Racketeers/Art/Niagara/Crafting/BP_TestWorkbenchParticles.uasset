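; BP_TestWorkbenchParticles is a test actor for previewing the workbench crafting Niagara effect.
; BeginPlay caches the world locations of six spawn point components into an array.
; Tick accumulates elapsed time and, each time TimeBetweenSpawn is reached, spawns FXS_Workbench at a randomly chosen cached location and reinitializes the new system.
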(event EventBeginPlay
  (Variables|Default|SetSpawnPoints (Utilities|Array|MakeArray (Transformation|GetWorldLocation (Variables|Default|GetSpawnpoint6)) (Transformation|GetWorldLocation (Variables|Default|GetSpawnpoint5)) (Transformation|GetWorldLocation (Variables|Default|GetSpawnpoint4)) (Transformation|GetWorldLocation (Variables|Default|GetSpawnpoint3)) (Transformation|GetWorldLocation (Variables|Default|GetSpawnpoint2)) (Transformation|GetWorldLocation (Variables|Default|GetSpawnpoint1)))))

(event EventTick
  (params (DeltaSeconds :type Float%20%28single-precision%29))
  (bind _output_get (Variables|Default|SetElapsedTime (+ DeltaSeconds (Variables|Default|GetElapsedTime))))
  (if (>= _output_get (Variables|Default|GetTimeBetweenSpawn))
    (Variables|Default|SetElapsedTime 0.0)
    (bind _returnvalue (Niagara|SpawnSystematLocation "/Game/Racketeers/Art/Niagara/Crafting/FXS_Workbench.FXS_Workbench" (.OutItem (Utilities|Array|Random (Variables|Default|GetSpawnPoints)))))
    (Niagara|ReinitializeSystem _returnvalue)))

(fn ConstructionScript)