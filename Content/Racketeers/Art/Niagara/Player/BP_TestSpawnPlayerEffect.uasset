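; Test Blueprint for previewing a player spawn effect, pairing a Niagara system with a Player component whose visibility it toggles.
; Spawn restarts the Niagara system and sets a timer of SpawnDelay that shows the player through SpawnPlayer.
; SetDespawn hides the player immediately, and a separate SpawnFunc shows it and prints a debug message.
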(event Custom|SetDespawn
  (Rendering|SetVisibility (Variables|Default|GetPlayer) false false))

(event Custom|SpawnPlayer
  (Rendering|SetVisibility (Variables|Default|GetPlayer) true false))

(event Custom|Spawn
  (Niagara|ReinitializeSystem (Variables|Default|GetNiagara))
  (Utilities|Time|SetTimerbyEvent (delegate Custom|SpawnPlayer) (Variables|Default|GetSpawnDelay)))

(event EventBeginPlay)

(event EventTick
  (params (DeltaSeconds :type Float%20%28single-precision%29)))

(fn ConstructionScript)

(fn SpawnFunc
  (Rendering|SetVisibility (Variables|Default|GetPlayer) true false)
  (Development|PrintString "Spawn player"))