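; BP_Boat is the player-controlled boat in Racketeers, adding the IMC_Boat input mapping on BeginPlay.
; Enhanced Input move and steer feed the BoatMovement component and add fixed pitch or roll to the mesh, identical for either input direction; look turns the controller.
; Accelerating past an X-velocity threshold plays a one-shot Fire01 sound.
; CheckForCollisionWater, uncalled here, only prints when CollisionCheck is off the ocean.
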(event Input|EnhancedActionEvents|EnhancedInputActionIA_Look_Boat
  (params (ActionValue :type Vector%202D%20Structure) (ElapsedSeconds :type Float%20%28double-precision%29) (TriggeredSeconds :type Float%20%28double-precision%29) (InputAction :type Input%20Action%20Object%20Reference :default "/Game/IA_Look_Boat.IA_Look_Boat"))
  (Pawn|Input|AddControllerPitchInput (.y ActionValue))
  (Pawn|Input|AddControllerYawInput (.x ActionValue)))

(event Input|EnhancedActionEvents|EnhancedInputActionIA_Move_Boat
  (params (ActionValue :type Float%20%28double-precision%29) (ElapsedSeconds :type Float%20%28double-precision%29) (TriggeredSeconds :type Float%20%28double-precision%29) (InputAction :type Input%20Action%20Object%20Reference :default "/Game/TopDown/Input/Actions/IA_Move_Boat.IA_Move_Boat"))
  (bind _staticmesh (Variables|Default|GetStaticMesh))
  (bind _staticmesh_2 (Variables|Default|GetStaticMesh))
  (bind _returnvalue (Transformation|GetWorldRotation _staticmesh))
  (bind _returnvalue_2 (Transformation|GetComponentVelocity _staticmesh_2))
  (Class|BoatMovement|Accelerate (Variables|Default|GetBoatMovement) ActionValue)
  (if (> ActionValue 0.0)
    (Variables|Default|SetBoatAccelerationRotation 1.0)
    (else
      (Variables|Default|SetBoatAccelerationRotation 1.0)))
  (Transformation|SetWorldRotation (Variables|Default|GetStaticMesh) (Math|Rotator|MakeRotator (.roll _returnvalue) (+ (.pitch _returnvalue) (Variables|Default|GetBoatAccelerationRotation)) (.yaw _returnvalue)) false false)
  (Development|PrintString (Utilities|String|ToString(Float) (.x _returnvalue_2)))
  (if (> (.x _returnvalue_2) 3e+03)
    (Utilities|FlowControl|DoOnce false
      (:Completed
        (Audio|PlaySound2D "/Game/StarterContent/Audio/Fire01.Fire01" 4.0 1.0 0.0 0 0)))))

(event Input|EnhancedActionEvents|EnhancedInputActionIA_Steer_Boat
  (params (ActionValue :type Float%20%28double-precision%29) (ElapsedSeconds :type Float%20%28double-precision%29) (TriggeredSeconds :type Float%20%28double-precision%29) (InputAction :type Input%20Action%20Object%20Reference :default "/Game/TopDown/Input/Actions/IA_Steer_Boat.IA_Steer_Boat"))
  (bind _staticmesh (Variables|Default|GetStaticMesh))
  (bind _returnvalue (Transformation|GetWorldRotation _staticmesh))
  (Class|BoatMovement|Steer (Variables|Default|GetBoatMovement) ActionValue)
  (if (> ActionValue 0.0)
    (Variables|Default|SetBoatSteerRotation 2.0)
    (else
      (Variables|Default|SetBoatSteerRotation 2.0)))
  (Transformation|SetWorldRotation (Variables|Default|GetStaticMesh) (Math|Rotator|MakeRotator (+ (.roll _returnvalue) (Variables|Default|GetBoatSteerRotation)) (.pitch _returnvalue) (.yaw _returnvalue)) false false))

(event EventBeginPlay
  (bind _returnvalue (Game|Player|GetPlayerPawn 0))
  (bind _playerstate (Variables|/Script/Engine.Pawn|GetPlayerState _returnvalue))
  (bind _returnvalue_2 (Game|GetPlayerController _playerstate))
  (Variables|Default|SetBoatMovementRef (Utilities|Array|Get(acopy) (Actor|GetComponentsByClass "/Script/PROJ_Test.BoatMovement")))
  (Input|EnableInput _returnvalue_2 0)
  (Input|AddMappingContext (PlayerController|LocalPlayerSubsystems|GetEnhancedInputLocalPlayerSubsystem _returnvalue_2) "/Game/TopDown/Input/IMC_Boat.IMC_Boat" 1 "(bIgnoreAllPressedKeysUntilRelease=True,bForceImmediately=False,bNotifyUserSettings=False)"))

(fn ConstructionScript)

(fn CheckforCollisionWater
  (bind _returnvalue (Actor|GetActorOfClass "/Script/Water.WaterBodyOcean"))
  (if (not (Collision|IsOverlappingActor (Variables|Default|GetCollisionCheck) _returnvalue :!class /Script/Engine.PrimitiveComponent))
    (Development|PrintString "NO FORCE" true true "(R=1.000000,G=0.018033,B=0.000000,A=1.000000)")))