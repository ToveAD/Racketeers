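; BP_Gatherable is an interactable resource actor that players can gather, with a replicated gather state.
; On authority, StartInteract sets GatherState to HasBeenGathered once, and its OnRep swaps the Resource mesh to a box.
; On remote instances, the same event adds one to the instigating player's PlayerScore on BP_PlayerState, outside the once-only gate.
; CanInteract simply returns a variable that these graphs never change.
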(event EventStartInteract
  (params (Instigator :type Actor%20Object%20Reference) (bIsServer :type Boolean))
  (Networking|SwitchHasAuthority
    (:Authority
      ;[1 1 1] Server Logic
      (Utilities|FlowControl|DoOnce false
        (:Completed
          (Utilities|FlowControl|Sequence
            (:then_0
              (Variables|Default|SetGatherState "NewEnumerator2"))))))
    (:Remote
      ;[1 1 1] Client Logic
      (bind _asbp_player (Utilities|Casting|CastToBP_Player Instigator))
      (bind _asbp_player_state (Utilities|Casting|CastToBP_PlayerState (Variables|/Script/Engine.Pawn|GetPlayerState _asbp_player)))
      (Variables|/Game/Racketeers/Characters/Blueprints/BP_PlayerState.BP_PlayerState_C|SetPlayerScore _asbp_player_state (+ (Variables|/Game/Racketeers/Characters/Blueprints/BP_PlayerState.BP_PlayerState_C|GetPlayerScore _asbp_player_state) 1)))))

(fn ConstructionScript)

(fn CanInteract
  (return (Variables|Default|GetbCanInteract)))

(fn OnRepGatherState
  (switch Utilities|FlowControl|Switch|SwitchonEGatherableStates (Variables|Default|GetGatherState)
    (:NewEnumerator2
      (Components|StaticMesh|SetStaticMesh (Variables|Default|GetResource) "/ControlRig/Controls/ControlRig_Box_3mm.ControlRig_Box_3mm"))))