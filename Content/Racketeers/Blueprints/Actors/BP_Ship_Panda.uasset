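; Playtest version of the Panda team's ship, with Enhanced Input driving its BoatMovement component for acceleration and steering.
; Left and right fire inputs share a CanShoot gate and spawn BP_Projectile from that side's spawn point, pitched 15 degrees above turret rotation.
; The cooldown timer targets "Timer", while the reset function here is named TimerShoot.
; Player attachment and mapping-context switching are left unwired.
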(event Custom|AttachPlayerToBoat)

(event Input|EnhancedActionEvents|EnhancedInputActionIA_DriverAccelerate
  (params (ActionValue :type Float%20%28double-precision%29) (ElapsedSeconds :type Float%20%28double-precision%29) (TriggeredSeconds :type Float%20%28double-precision%29) (InputAction :type Input%20Action%20Object%20Reference :default "/Game/Racketeers/Characters/Input/Actions/IA_DriverAccelerate.IA_DriverAccelerate"))
  ;[1 1 1] Ship Inputs (For playtest)
  (Class|BoatMovement|Accelerate (Variables|Default|GetBoatMovement) ActionValue)
  (Development|PrintString "AAccelll"))

(event Input|EnhancedActionEvents|EnhancedInputActionIA_DriverSteer
  (params (ActionValue :type Float%20%28double-precision%29) (ElapsedSeconds :type Float%20%28double-precision%29) (TriggeredSeconds :type Float%20%28double-precision%29) (InputAction :type Input%20Action%20Object%20Reference :default "/Game/Racketeers/Characters/Input/Actions/IA_DriverSteer.IA_DriverSteer"))
  ;[1 1 1] Ship Inputs (For playtest)
  (Class|BoatMovement|Steer (Variables|Default|GetBoatMovement) ActionValue))

(event Input|EnhancedActionEvents|EnhancedInputActionIA_Boat_ShootLeft
  (params (ActionValue :type Vector%202D%20Structure) (ElapsedSeconds :type Float%20%28double-precision%29) (TriggeredSeconds :type Float%20%28double-precision%29) (InputAction :type Input%20Action%20Object%20Reference :default "/Game/Racketeers/Characters/Input/Actions/IA_Boat_ShootLeft.IA_Boat_ShootLeft"))
  ;[1 1 1] Ship Inputs (For playtest)
  (:Started
    (if (Variables|Default|GetbCanShoot)
      (Variables|Default|SetbCanShoot false)
      (Utilities|Time|SetTimerbyFunctionName 0 "Timer" 1.0)
      (CallFunction|Shoot true))))

(event Input|EnhancedActionEvents|EnhancedInputActionIA_Boat_ShootRight
  (params (ActionValue :type Vector%202D%20Structure) (ElapsedSeconds :type Float%20%28double-precision%29) (TriggeredSeconds :type Float%20%28double-precision%29) (InputAction :type Input%20Action%20Object%20Reference :default "/Game/Racketeers/Characters/Input/Actions/IA_Boat_ShootRight.IA_Boat_ShootRight"))
  ;[1 1 1] Ship Inputs (For playtest)
  (:Started
    (if (Variables|Default|GetbCanShoot)
      (Variables|Default|SetbCanShoot false)
      (Utilities|Time|SetTimerbyFunctionName 0 "Timer" 1.0)
      (CallFunction|Shoot false))))

(event Collision|EventActorBeginOverlap
  (params (OtherActor :type Actor%20Object%20Reference)))

(event EventTick
  (params (DeltaSeconds :type Float%20%28single-precision%29))
  (|CallParentFunction DeltaSeconds) ; This node is disabled and will not be called.\nDrag off pins to build functionality.
)

(event EventBeginPlay)

(fn ConstructionScript
  (|CallParentFunction))

(fn TimerShoot
  (Variables|Default|SetbCanShoot true))

(fn Shoot
  (params (ShootLeft :type Boolean))
  (bind _turretone_right (Variables|Default|GetTurretOne_Right))
  (bind _turretone_left (Variables|Default|GetTurretOne_Left))
  (bind _returnvalue (Transformation|GetWorldRotation _turretone_left))
  (bind _returnvalue_2 (Transformation|GetWorldRotation _turretone_right))
  (if ShootLeft
    (Game|SpawnActorfromClass "/Game/Racketeers/Blueprints/Actors/BP_Projectile.BP_Projectile_C" (Math|Transform|MakeTransform (Transformation|GetWorldLocation (Variables|Default|GetProjectileSpawnOne_Left)) (Math|Rotator|MakeRotator (.roll _returnvalue) (+ (.pitch _returnvalue) 15.0) (.yaw _returnvalue)) "1.000000,1.000000,1.000000") "Undefined" "MultiplyWithRoot" 0 0)
    (else
      (Game|SpawnActorfromClass "/Game/Racketeers/Blueprints/Actors/BP_Projectile.BP_Projectile_C" (Math|Transform|MakeTransform (Transformation|GetWorldLocation (Variables|Default|GetProjectileSpawnTwo_Right)) (Math|Rotator|MakeRotator (.roll _returnvalue_2) (+ (.pitch _returnvalue_2) 15.0) (.yaw _returnvalue_2)) "1.000000,1.000000,1.000000") "Undefined" "MultiplyWithRoot" 0 0))))