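; Shared camera rig, apparently for the game's first phase, that keeps all actors of the player class framed.
; Each tick it moves to the players' average XY position, deriving height from a 300-unit seed and player count rather than their actual Z.
; It then scales the spring arm length with the distance to the furthest player, zooming out as players spread apart.
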(event EventTick
  (params (DeltaSeconds :type Float%20%28single-precision%29))
  (bind _outactors (Actor|GetAllActorsOfClass (Variables|Default|GetPlayer%20Class)))
  (for _array_element _outactors
    (Variables|Default|SetPosition (+ (Math|Vector|MakeVector (.x (Transformation|GetActorLocation _array_element)) (.y (Transformation|GetActorLocation _array_element)) (.z (Variables|Default|GetPosition))) (Variables|Default|GetPosition))))
  (Transformation|SetActorLocation (/ (Variables|Default|GetPosition) (Utilities|Array|Length _outactors)) false false)
  (for _array_element_2 _outactors
    (if (>= (Math|Vector|Distance(Vector) (Transformation|GetActorLocation _array_element_2) (Transformation|GetActorLocation)) (Variables|Default|GetDistance%20To%20Furthest%20Player))
      (Variables|Default|SetDistance%20To%20Furthest%20Player (Math|Vector|Distance(Vector) (Transformation|GetActorLocation _array_element_2) (Transformation|GetActorLocation)))))
  (Variables|/Script/Engine.SpringArmComponent|SetTargetArmLength (Variables|Default|GetSpringArm) (* (Variables|Default|GetDistance%20To%20Furthest%20Player) 1.75))
  (Variables|Default|SetPosition "0.000000,0.000000,300.000000")
  (Variables|Default|SetDistance%20To%20Furthest%20Player 0.0))

(fn ConstructionScript)