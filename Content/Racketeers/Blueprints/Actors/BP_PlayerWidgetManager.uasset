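; Player widget manager for Racketeers that registers the game's player widgets with the widget subsystem.
; The construction script builds a name-to-widget map for winner, score, team resources and health.
; When the local controller's begin-player event fires, it hands the map to the subsystem and activates TeamResources.
; The older game-mode-driven logic for loading and unloading widgets on every player's controller is disconnected, leaving those events empty.
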(event Custom|LoadWidget)

(event Custom|LoadWidgeToClients)

(event Custom|OnUnloadWidget
  (CallFunction|UnloadWidgettoClients))

(event Custom|UnloadWidgetToClients)

(event Custom|OnLoadWidget
  (params (Name :type Name)))

(event Custom|OnUnload
  (params (Name :type Name)))

(event Custom|OnBeginPlayerEvent_Event
  (bind _returnvalue (Subsystems|GetWidgetSubsystem))
  (Development|PrintString (Utilities|String|Append "FROM PLAYE WIDGET:  " (Class|AdvancedSessionsLibrary|UniqueNetIdtoString (Class|AdvancedSessionsLibrary|GetUniqueNetID (stale EventBeginPlay _asracketeers_controller)))))
  (Variables|/Script/Racketeers.WidgetSubsystem|SetMapOfAllPlayerWidget _returnvalue (Variables|Default|GetWidgetByNameMap))
  (bind _asracketeers_gmbase (Utilities|Casting|CastToRacketeersGMBase (Game|GetGameMode))
    (:then
      (Variables|Default|SetGM _asracketeers_gmbase))
    (:CastFailed
      _))
  (Class|WidgetSubsystem|ActivateWidget _returnvalue "TeamResources"))

(event EventBeginPlay
  (bind _asracketeers_controller (Utilities|Casting|CastToRacketeersController (Game|GetPlayerController 0)))
  (EventDispatchers|BindEventtoOnBeginPlayerEvent _asracketeers_controller (delegate Custom|OnBeginPlayerEvent_Event)))

(fn ConstructionScript
  (bind _widgetbynamemap (Variables|Default|GetWidgetByNameMap))
  (Utilities|Map|Add _widgetbynamemap "WinnerWidget" (Variables|Default|GetWinnerWidget))
  (Utilities|Map|Add _widgetbynamemap "ShowScore" (Variables|Default|GetShowScore))
  (Utilities|Map|Add _widgetbynamemap "TeamResources" (Variables|Default|GetTeamResource))
  (Utilities|Map|Add _widgetbynamemap "Health" (Variables|Default|GetHealth)))

(fn GetWidgetbyClassName
  (params (Name :type Name))
  (return (.Value (Utilities|Map|Find (Variables|Default|GetWidgetByNameMap) Name))))