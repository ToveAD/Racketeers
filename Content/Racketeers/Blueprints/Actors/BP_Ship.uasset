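; BP_Ship is a crewed ship with accelerate, steer and gunner stations, but all its gameplay logic is currently disconnected and its events are empty.
; The unwired graph attaches each player's pawn to a station by TeamPlayerID, disabling collision and switching to ship input mapping.
; Other orphaned chains forward driver input to proxy components and spawn cursor-aimed projectiles for the gunner.
; Only the CanInteract getter returns anything; the role OnRep is empty.
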(event Custom|Server)

(event Custom|Multi)

(event Input|EnhancedActionEvents|EnhancedInputActionIA_GunnerShootLeft
  (params (ActionValue :type Vector%202D%20Structure) (ElapsedSeconds :type Float%20%28double-precision%29) (TriggeredSeconds :type Float%20%28double-precision%29) (InputAction :type Input%20Action%20Object%20Reference :default "/Game/Racketeers/Characters/Input/Actions/IA_GunnerShootLeft.IA_GunnerShootLeft")))

(event Input|EnhancedActionEvents|EnhancedInputActionIA_GunnerShoot
  (params (ActionValue :type Vector%202D%20Structure) (ElapsedSeconds :type Float%20%28double-precision%29) (TriggeredSeconds :type Float%20%28double-precision%29) (InputAction :type Input%20Action%20Object%20Reference :default "/Game/Racketeers/Characters/Input/Actions/IA_GunnerShoot.IA_GunnerShoot")))

(event Input|EnhancedActionEvents|EnhancedInputActionIA_DriverAccelerate
  (params (ActionValue :type Float%20%28double-precision%29) (ElapsedSeconds :type Float%20%28double-precision%29) (TriggeredSeconds :type Float%20%28double-precision%29) (InputAction :type Input%20Action%20Object%20Reference :default "/Game/Racketeers/Characters/Input/Actions/IA_DriverAccelerate.IA_DriverAccelerate")))

(event Input|EnhancedActionEvents|EnhancedInputActionIA_DriverSteer
  (params (ActionValue :type Float%20%28double-precision%29) (ElapsedSeconds :type Float%20%28double-precision%29) (TriggeredSeconds :type Float%20%28double-precision%29) (InputAction :type Input%20Action%20Object%20Reference :default "/Game/Racketeers/Characters/Input/Actions/IA_DriverSteer.IA_DriverSteer")))

(event EventBeginPlay)

(fn ConstructionScript)

(fn OnRepCurrentRole)

(fn CanInteract
  (return (Variables|Default|GetbCanInteract)))