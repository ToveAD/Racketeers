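; DUMMY is a player-style actor that enables its player indicator on BeginPlay and resets any held resource at phase changes.
; It binds to the Racketeers game state's incoming Phase Two and Phase Three events, both calling ResetHoldingResource.
; A server-to-multicast event pair can clear an instigator's holding state and mesh, but its only call here is unconnected, as is a running-effects call.
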(event Custom|MultiResetHoldingObject
  (params (Instigator :type BP%20Player%20Object%20Reference))
  (Variables|/Game/Racketeers/Core/BP_Player.BP_Player_C|SetIsHoldingResource Instigator false)
  (Variables|/Game/Racketeers/Core/BP_Player.BP_Player_C|SetHoldingResourceInfo Instigator (Utilities|Struct|MakeFCraftableResource "NONE" 0))
  (Components|StaticMesh|SetStaticMesh (Variables|/Game/Racketeers/Core/BP_Player.BP_Player_C|GetHoldingObject Instigator) 0))

(event Custom|OnIncomingPhaseTwoActive_Event
  (CallFunction|ResetHoldingResource))

(event Custom|OnIncomingPhaseThreeActive_Event
  (CallFunction|ResetHoldingResource))

(event Custom|ServerResetHoldinObject
  (params (Instigator :type BP%20Player%20Object%20Reference))
  (CallFunction|MultiResetHoldingObject Instigator))

(event EventBeginPlay
  (CallFunction|EnablePlayerIndicator)
  (bind _asracketeers_game_state_base (Utilities|Casting|CastToRacketeersGameStateBase (Game|GetGameState)))
  (EventDispatchers|AssignOnIncomingPhaseTwoActive _asracketeers_game_state_base (delegate Custom|OnIncomingPhaseTwoActive_Event))
  (EventDispatchers|AssignOnIncomingPhaseThreeActive _asracketeers_game_state_base (delegate Custom|OnIncomingPhaseThreeActive_Event)))

(fn ConstructionScript)