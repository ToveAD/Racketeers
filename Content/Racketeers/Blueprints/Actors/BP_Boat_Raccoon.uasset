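; BP_Boat_Raccoon is the Raccoon team's boat actor, which takes damage when projectiles hit it.
; Mesh hits are routed to a server-side damage event that only reacts to BP_Projectile actors.
; That event zeroes the boat's physics velocities and has RacketeersController deduct team boat health.
; It then prints the health from RacketeersGameStateBase and destroys the projectile.
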(event OnComponentHit(StaticMesh)
  (params (HitComponent :type Primitive%20Component%20Object%20Reference) (OtherActor :type Actor%20Object%20Reference) (OtherComp :type Primitive%20Component%20Object%20Reference) (NormalImpulse :type Vector :default "0, 0, 0") (Hit :type Hit%20Result%20Structure%20%28by%20ref%29))
  ;[1 1 1] Take damage from BP_Projectile
  ;;[1 1 1] Tell boat to take damage
  (CallFunction|TakeDamage OtherActor))

(event Custom|Server_TakeDamage
  (params (OtherActor :type Object%20Object%20Reference))
  (bind _staticmesh (Variables|Default|GetStaticMesh))
  ;[1 1 1] Take damage from BP_Projectile
  ;;[1 1 1] Run on Server
  (if (Utilities|ClassIsChildOf (Utilities|GetClass OtherActor) "/Game/Racketeers/Blueprints/Actors/BP_Projectile.BP_Projectile_C")
    (Physics|SetPhysicsLinearVelocity _staticmesh "0, 0, 0" false "None")
    (Class|PrimitiveComponent|SetPhysicsAngularVelocityinDegrees _staticmesh "0, 0, 0" false "None")
    (Development|PrintString (Utilities|GetDisplayName OtherActor) true true "(R=0.000000,G=0.000000,B=0.000000,A=1.000000)")
    (bind _returnvalue (Actor|GetActorOfClass "/Script/Racketeers.RacketeersController"))
    (Class|RacketeersController|DamageBoat _returnvalue 1 "Team_Racoon")
    (bind _asracketeers_game_state_base (Utilities|Casting|CastToRacketeersGameStateBase (Game|GetGameState))
      (:then
        (Development|PrintString (Utilities|String|ToString(Float) (Variables|/Script/Racketeers.RacketeersGameStateBase|GetRacconsBoatHealth _asracketeers_game_state_base)) true true "(R=0.097860,G=1.000000,B=0.000000,A=1.000000)")
        (bind _asbp_projectile (Utilities|Casting|CastToBP_Projectile OtherActor))
        (Actor|DestroyActor _asbp_projectile))
      (:CastFailed
        (Development|PrintString "Cast failed" true true "(R=1.000000,G=0.032542,B=0.000000,A=1.000000)" 1e+01)))))

(event Custom|Take%20Damage
  (params (OtherActor :type Object%20Object%20Reference))
  ;[1 1 1] Take damage from BP_Projectile
  ;;[1 1 1] Call on Server
  (CallFunction|ServerTakeDamage OtherActor))

(event EventBeginPlay
  (|CallParentFunction) ; This node is disabled and will not be called.\nDrag off pins to build functionality.
)

(event Collision|EventActorBeginOverlap
  (params (OtherActor :type Actor%20Object%20Reference)))

(event EventTick
  (params (DeltaSeconds :type Float%20%28single-precision%29)))

(fn ConstructionScript
  (|CallParentFunction))