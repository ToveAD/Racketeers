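; Gatherable resource actor for Racketeers that tracks its gathering Instigators and loses ItemHP while being gathered.
; StartGathering and StopGathering update that list and set State, whose RepNotify starts or clears a looping damage timer.
; Each tick subtracts GatheringDamage, which also serves as the timer interval, and depletion only prints a message.
; Interact events are empty, CanInteract returns false, and damage scaling by gatherer count is left unconnected.
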(event Custom|StartGathering
  (params (Instigator :type Actor%20Object%20Reference))
  (Utilities|Array|AddUnique (Variables|Default|GetInstigators) Instigator)
  (Variables|Default|SetState "NewEnumerator1"))

(event Custom|StopGathering
  (params (Instigator :type Actor%20Object%20Reference))
  (Utilities|Array|RemoveItem (Variables|Default|GetInstigators) Instigator)
  (Variables|Default|SetState "NewEnumerator0"))

(event EventBeginPlay)

(event Collision|EventActorBeginOverlap
  (params (OtherActor :type Actor%20Object%20Reference)))

(event EventTick
  (params (DeltaSeconds :type Float%20%28single-precision%29)))

(event EventStartInteract
  (params (Instigator :type Actor%20Object%20Reference)))

(event EventStopInteract)

(fn ConstructionScript)

(fn ApplyGatheringdamage
  (bind _output_get (Variables|Default|SetItemHP (- (Variables|Default|GetItemHP) (Variables|Default|GetGatheringDamage))))
  (if (<= _output_get 0.0)
    (Development|PrintString "ResourceFinish")
    (else
      (Development|PrintString (Utilities|String|ToString(Float) _output_get)))))

(fn OnRepState
  (switch Utilities|FlowControl|Switch|SwitchonEGatherableStates (Variables|Default|GetState)
    (:NewEnumerator0
      (if (Utilities|Time|IsValidTimerHandle (Variables|Default|GetGatheringTimerHandle))
        (Utilities|Time|ClearandInvalidateTimerbyHandle (Variables|Default|GetGatheringTimerHandle))))
    (:NewEnumerator1
      (bind _returnvalue (Utilities|Time|SetTimerbyFunctionName 0 "ApplyGatheringdamage" (Variables|Default|GetGatheringDamage) true))
      (Variables|Default|SetGatheringTimerHandle _returnvalue))))

(fn CanInteract
  (return false))