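; Player-drivable boat for Racketeers that can be boarded, steered and used to fire cannon projectiles from either side.
; Interaction is multicast to attach the player, disable their movement and swap input mapping, while BoatMovement handles acceleration and steering.
; Shots spawn server-side on a cooldown, with effects sent through EffectsComponent.
; Leaving requires a box trace hit on an Island-tagged actor, but map unload from the GameMode also detaches the player.
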(event Custom|Client_BoatShootLeft
  ;[1 1 1] Inputs (Are Called From BP_Player)
)

(event Custom|Server_BoatShootLeft
  ;[1 1 1] Inputs (Are Called From BP_Player)
  (if (Variables|Default|GetbCanShoot)
    (Variables|Default|SetbCanShoot false)
    (Utilities|Time|SetTimerbyFunctionName 0 "TimerShoot" (Variables|Default|GetShootCooldown))
    (CallFunction|Shoot true)))

(event Custom|Multi_StartInteract
  (params (Instigator :type Actor%20Object%20Reference))
  ;[1 1 1] Start Interact
  ;;[1 1 1] 2. Send to all clients
  (CallFunction|SetReferences Instigator)
  (CallFunction|EnterBoat))

(event Custom|BoatShootRight
  ;[1 1 1] Inputs (Are Called From BP_Player)
  (CallFunction|ServerBoatShootRight)
  (Default|ServerOneEffectCall (Variables|Default|GetEffectsComponent) (Variables|Default|GetShootingEffectRight)))

(event Custom|Unload
  ;[1 1 1] Detach Player When Switching Level
  ;;[1 1 1] Unload On Server (Game Mode Already Runs On Server)
  (CallFunction|MultiUnload))

(event Custom|Multi_StopInteract
  ;[1 1 1] Stop Interact
  ;;[1 1 1] 3. Send to all clients
  (CallFunction|StopInteract)
  (Collision|SetActorEnableCollision (Variables|Default|GetPlayerRef) true))

(event Custom|BoatAccelerate
  (params (ActionValue :type Float%20%28double-precision%29))
  ;[1 1 1] Inputs (Are Called From BP_Player)
  ;;[1 1 1] Move Boat
  (if (Variables|Default|GetbCanAccelerate)
    (Variables|Default|SetbCanAccelerate false)
    (Utilities|Time|SetTimerbyFunctionName 0 "TimerAccelerate" 0.001)
    (Class|BoatMovement|Accelerate (Variables|Default|GetBoatMovement) ActionValue)))

(event Custom|Server_StopInteract
  (params (Target :type Actor%20Object%20Reference))
  ;[1 1 1] Stop Interact
  ;;[1 1 1] 2. Server telling Multicast to send to all clients
  (CallFunction|MultiStopInteract))

(event Custom|SteerBoat
  (params (ActionValue :type Float%20%28single-precision%29))
  ;[1 1 1] Inputs (Are Called From BP_Player)
  ;;[1 1 1] Steer Boat
  (Class|BoatMovement|Steer (Variables|Default|GetBoatMovement) ActionValue))

(event Custom|Multi_Unload
  ;[1 1 1] Detach Player When Switching Level
  ;;[1 1 1] Send To All Clients
  (CallFunction|StopInteract (Variables|Default|GetPlayerRef))
  (Development|PrintString "Unload"))

(event Custom|Server_BoatShootRight
  ;[1 1 1] Inputs (Are Called From BP_Player)
  (if (Variables|Default|GetbCanShoot)
    (Variables|Default|SetbCanShoot false)
    (Utilities|Time|SetTimerbyFunctionName 0 "TimerShoot" (Variables|Default|GetShootCooldown))
    (CallFunction|Shoot false)))

(event Custom|LeaveBoatInteract
  ;[1 1 1] Stop Interact
  ;;[1 1 1] 1. Player sending to server
  (if (Variables|Default|GetShouldDetach)
    (bind _returnvalue (CallFunction|CanLeaveBoatCheck))
    (if _returnvalue
      (CallFunction|ServerStopInteract))))

(event Custom|BoatShootLeft
  ;[1 1 1] Inputs (Are Called From BP_Player)
  (CallFunction|ServerBoatShootLeft)
  (Default|ServerOneEffectCall (Variables|Default|GetEffectsComponent) (Variables|Default|GetShootingEffectLeft)))

(event EventStartInteract
  (params (Instigator :type Actor%20Object%20Reference) (bIsServer :type Boolean))
  ;[1 1 1] Start Interact
  ;;[1 1 1] 1. Run On Server & Send To Multicast (Already Runs On Server In BP_Player)
  (CallFunction|MultiStartInteract Instigator))

(event EventStopInteract
  (params (Instigator :type Actor%20Object%20Reference))
  ;[1 1 1] Stop Interact
  ;;[1 1 1] 4: Hande logic
  (CallFunction|LeaveBoat))

(event EventBeginPlay
  ;[1 1 1] Detach Player When Switching Level
  ;;[1 1 1] Unload On Server (Game Mode Already Runs On Server)
  (bind _asracketeers_gmbase (Utilities|Casting|CastToRacketeersGMBase (Game|GetGameMode)))
  (EventDispatchers|BindEventtoOnUnloadingMap _asracketeers_gmbase (delegate Custom|Unload)))

(fn ConstructionScript)

(fn CheckforCollisionWater
  (bind _returnvalue (Actor|GetActorOfClass 0))
  (if (not (Collision|IsOverlappingActor (Variables|Default|GetCollisionCheck) _returnvalue :!class /Script/Engine.PrimitiveComponent))
    (Development|PrintString "NO FORCE" true true "(R=1.000000,G=0.018033,B=0.000000,A=1.000000)")))

(fn Timer
  (Variables|Default|SetbCanAccelerate true))

(fn EnterBoat
  (Collision|SetActorEnableCollision (Variables|Default|GetInstigatorRef) false)
  (Transformation|AttachComponentToComponent (Variables|Default|GetPlayerRef) (Variables|Default|GetPlayerPos) "None" "SnapToTarget" "SnapToTarget" "KeepWorld" false)
  (Actor|SetOwner self (Variables|Default|GetPlayerRef))
  (Pawn|Components|CharacterMovement|DisableMovement (Variables|/Script/Engine.Character|GetCharacterMovement (Variables|Default|GetPlayerRef)))
  (Class|BoatMovement|SwitchInputMapping (Variables|Default|GetBoatMovement) true "/Game/Racketeers/Characters/Input/IMC_Boat.IMC_Boat" "/Game/Racketeers/Characters/Input/IMC_Default.IMC_Default" (Variables|Default|GetPlayerController))
  (return))

(fn LeaveBoat
  (Transformation|DetachFromActor (Variables|Default|GetPlayerRef) "KeepWorld" "KeepWorld" "KeepWorld")
  (Actor|SetOwner self (Variables|Default|GetPlayerRef))
  (Utilities|IsValid (Variables|Default|GetPlayerRef)
    (:Is%20Valid
      (Utilities|IsValid (Variables|Default|GetPlayerController)
        (:Is%20Valid
          (Pawn|Components|CharacterMovement|SetMovementMode (Variables|/Script/Engine.Character|GetCharacterMovement (Variables|Default|GetPlayerRef)) "MOVE_Walking" 0)
          (Class|BoatMovement|SwitchInputMapping (Variables|Default|GetBoatMovement) false "/Game/Racketeers/Characters/Input/IMC_Boat.IMC_Boat" "/Game/Racketeers/Characters/Input/IMC_Default.IMC_Default" (Variables|Default|GetPlayerController))
          (Variables|Default|SetbCanInteract true))))))

(fn CanLeaveBoatCheck
  (bind _staticmesh (Variables|Default|GetStaticMesh))
  (bind _returnvalue (Transformation|GetWorldLocation _staticmesh))
  (bind _returnvalue_2 (Actor|GetActorOfClass "/Script/Water.WaterBodyCustom"))
  (bind (_outhits _returnvalue_3) (Class|KismetSystemLibrary|BoxTraceMultiforObjects _returnvalue _returnvalue (Variables|/Script/Engine.BoxComponent|GetBoxExtent (Variables|Default|GetIslandCheck)) (Transformation|GetActorRotation) (Utilities|Array|MakeArray "ObjectTypeQuery1") false (Utilities|Array|MakeArray _returnvalue_2 0) "ForDuration" true))
  (if _returnvalue_3
    (bind _array_element (Utilities|Array|ForEachLoopwithBreak _outhits)
      (:LoopBody
        (Development|PrintString (Utilities|GetDisplayName (.HitComponent (Collision|BreakHitResult _array_element))))
        (Development|PrintString (Utilities|String|ToString(Boolean) (Actor|ActorHasTag (.HitActor (Collision|BreakHitResult _array_element)) "Island"))))
      (:Completed
        (return (Actor|ActorHasTag (.HitActor (Collision|BreakHitResult _array_element)) "Island"))))))

(fn SetReferences
  (params (Instigator :type Actor%20Object%20Reference))
  (bind _output_get (Variables|Default|SetInstigatorRef Instigator))
  (bind _asbp_player (Utilities|Casting|CastToBP_Player _output_get))
  (bind _output_get_2 (Variables|Default|SetPlayerRef _asbp_player))
  (Utilities|IsValid _output_get_2
    (:Is%20Valid
      (bind _asbp_player_controller (Utilities|Casting|CastToBP_PlayerController (Pawn|GetController (Variables|Default|GetPlayerRef))))
      (bind _output_get_3 (Variables|Default|SetPlayerController _asbp_player_controller))
      (Utilities|IsValid _output_get_3
        (:Is%20Valid
          (Variables|Default|SetbCanInteract false)
          (return))
        (:Is%20Not%20Valid
          (Development|PrintString "Player Controller Not Valid" true true "(R=1.000000,G=0.154444,B=0.000000,A=1.000000)"))))
    (:Is%20Not%20Valid
      (Development|PrintString "PlayerRef Not Valid" true true "(R=1.000000,G=0.181028,B=0.000000,A=1.000000)"))))

(fn OnRepNewLocation
  (Transformation|SetActorLocation (Transformation|GetActorLocation) false false))

(fn OnRepNewRotation
  (Transformation|SetActorRotation (Transformation|GetActorRotation)))

(fn Shoot
  (params (ShootLeft :type Boolean))
  (bind _turretone_right (Variables|Default|GetTurretOne_Right))
  (bind _turretone_left (Variables|Default|GetTurretOne_Left))
  (bind _returnvalue (Transformation|GetWorldRotation _turretone_left))
  (bind _returnvalue_2 (Transformation|GetWorldRotation _turretone_right))
  (if ShootLeft
    (Game|SpawnActorfromClass "/Game/Racketeers/Blueprints/Actors/BP_Projectile.BP_Projectile_C" (Math|Transform|MakeTransform (Transformation|GetWorldLocation (Variables|Default|GetProjectileSpawnOne_Left)) (Math|Rotator|MakeRotator (.roll _returnvalue) (+ (.pitch _returnvalue) 15.0) (.yaw _returnvalue)) "1.000000,1.000000,1.000000") "Undefined" "MultiplyWithRoot" 0 0)
    (else
      (Game|SpawnActorfromClass "/Game/Racketeers/Blueprints/Actors/BP_Projectile.BP_Projectile_C" (Math|Transform|MakeTransform (Transformation|GetWorldLocation (Variables|Default|GetProjectileSpawnTwo_Right)) (Math|Rotator|MakeRotator (.roll _returnvalue_2) (+ (.pitch _returnvalue_2) 15.0) (.yaw _returnvalue_2)) "1.000000,1.000000,1.000000") "Undefined" "MultiplyWithRoot" 0 0))))

(fn TimerShoot
  (Variables|Default|SetbCanShoot true))

(fn TimerAccelerate
  (Variables|Default|SetbCanAccelerate true))

(fn CanInteract
  (return (Variables|Default|GetbCanInteract)))