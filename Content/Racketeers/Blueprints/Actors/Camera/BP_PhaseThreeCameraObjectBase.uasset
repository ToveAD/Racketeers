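; BP_PhaseThreeCameraObjectBase is a shared camera actor, named for phase three, that tracks the group of players along the X axis.
; On BeginPlay, if player 0's pawn is a BP_Racoon, it becomes that controller's view target after a short delay, then sets it again a second later.
; Each Tick it averages the locations of all PlayerClass actors, adds Offset, and smoothly interpolates its X toward that point, keeping Y and Z.
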(event EventTick
  (params (DeltaSeconds :type Float%20%28single-precision%29))
  (bind _returnvalue (Transformation|GetActorLocation))
  (bind _outactors (Actor|GetAllActorsOfClass (Variables|Default|GetPlayer%20Class)))
  (for _array_element _outactors
    (Variables|Default|SetPosition (+ (Transformation|GetActorLocation _array_element) (Variables|Default|GetPosition))))
  (if (> (Utilities|Array|Length _outactors) 0)
    (Transformation|SetActorLocation (Math|Interpolation|VInterpTo (Transformation|GetActorLocation) (Math|Vector|MakeVector (.x (+ (/ (Variables|Default|GetPosition) (Utilities|Array|Length _outactors)) (Variables|Default|GetOffset))) (.y _returnvalue) (.z _returnvalue)) (Utilities|Time|GetWorldDeltaSeconds) 2.6) false false)
    (Variables|Default|SetPosition "0, 0, 0")))

(event EventBeginPlay
  (Utilities|Casting|CastToBP_Racoon (Game|Player|GetPlayerPawn 0))
  (Utilities|FlowControl|Delay 0.7)
  (Game|Player|SetViewTargetwithBlend (Game|GetPlayerController 0) self 0.0 "VTBlend_Linear" 0.0 false)
  (Utilities|FlowControl|Delay 1.0)
  (Game|Player|SetViewTargetwithBlend (Game|GetPlayerController 0) self 0.0 "VTBlend_Linear" 0.0 false))

(fn ConstructionScript
  (|CallParentFunction))