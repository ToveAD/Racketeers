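; Phase 1 raccoon camera object that claims the view for the player matching its team and ID.
; Each Tick runs the parent logic, then, if the player is valid, compares the player state's team and team player ID to its own.
; On a match it calls SetViewTarget with player controller 0, repeating every frame rather than once.
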(event EventBeginPlay
  (|CallParentFunction) ; This node is disabled and will not be called.\nDrag off pins to build functionality.
)

(event Collision|EventActorBeginOverlap
  (params (OtherActor :type Actor%20Object%20Reference)))

(event EventTick
  (params (DeltaSeconds :type Float%20%28single-precision%29))
  (bind _playerstate (Variables|Default|GetPlayerState))
  (bind _playerinfo (Variables|/Script/Racketeers.PS_Base|GetPlayerInfo _playerstate))
  (|CallParentFunction DeltaSeconds)
  (Utilities|IsValid (Variables|Default|GetPlayer)
    (:Is%20Valid
      (if (and (Utilities|Enum|Equal(Enum) (Variables|Default|GetPlayerTeam) (.team _playerinfo)) (== (.teamplayerid _playerinfo) (Variables|Default|GetPlayerID)))
        (CallFunction|SetViewTarget (Game|GetPlayerController 0))))))

(fn ConstructionScript
  (|CallParentFunction))