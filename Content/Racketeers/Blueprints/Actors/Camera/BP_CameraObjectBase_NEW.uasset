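; BP_CameraObjectBase_NEW is a follow-camera actor assigned to a player slot by team and team player ID.
; It caches the first local player's pawn and PlayerState, re-fetching them on Tick while the pawn is invalid.
; When that PlayerState matches its slot, it interpolates toward the pawn's location plus an offset and makes itself the controller's view target if it is not already.
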(event EventBeginPlay
  (bind _asbp_player (Utilities|Casting|CastToBP_Player (Game|Player|GetPlayerPawn 0)))
  (bind _output_get (Variables|Default|SetPlayer _asbp_player))
  (bind _asbp_player_state (Utilities|Casting|CastToBP_PlayerState (Variables|/Script/Engine.Pawn|GetPlayerState _output_get)))
  (Variables|Default|SetPlayerState _asbp_player_state))

(event EventTick
  (params (DeltaSeconds :type Float%20%28single-precision%29))
  (Utilities|IsValid (Variables|Default|GetPlayer)
    (:Is%20Valid
      (if (and (== (.teamplayerid (Variables|/Script/Racketeers.PS_Base|GetPlayerInfo (Variables|Default|GetPlayerState))) (Variables|Default|GetPlayerID)) (Utilities|Enum|Equal(Enum) (.team (Variables|/Script/Racketeers.PS_Base|GetPlayerInfo (Variables|Default|GetPlayerState))) (Variables|Default|GetPlayerTeam)))
        (Transformation|SetActorLocation (Math|Interpolation|VInterpTo (Transformation|GetActorLocation) (+ (Transformation|GetActorLocation (Variables|Default|GetPlayer)) (Variables|Default|GetOffset)) DeltaSeconds (Variables|Default|GetInterp%20Speed)) false false)
        (if true
          (CallFunction|SetViewTarget (Game|GetPlayerController 0)))))
    (:Is%20Not%20Valid
      (bind _asbp_player (Utilities|Casting|CastToBP_Player (Game|Player|GetPlayerPawn 0)))
      (bind _output_get (Variables|Default|SetPlayer _asbp_player))
      (bind _asbp_player_state (Utilities|Casting|CastToBP_PlayerState (Variables|/Script/Engine.Pawn|GetPlayerState _output_get)))
      (Variables|Default|SetPlayerState _asbp_player_state))))

(fn ConstructionScript)

(fn SetViewTarget
  (params (PlayerController :type Player%20Controller%20Object%20Reference))
  (bind _returnvalue (Pawn|GetViewTarget PlayerController))
  (bind _self self)
  (bind _returnvalue_2 (== _returnvalue _self))
  (if _returnvalue_2
    _
    (else
      (Game|Player|SetViewTargetwithBlend PlayerController self 0.0 "VTBlend_Linear" 0.0 false)))
  (return _returnvalue_2))