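; Base camera actor for phase three that keeps all players in frame along the X axis.
; Each Tick it averages the locations of every PlayerClass actor, adds an offset and eases its X toward that point within min/max bounds, keeping Y and Z fixed.
; It then finds the largest X distance to a player, scales it by a zoom multiplier and smoothly interpolates the spring arm to that clamped length.
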(event EventTick
  (params (DeltaSeconds :type Float%20%28single-precision%29))
  (bind _returnvalue (Transformation|GetActorLocation))
  (bind _springarm (Variables|Default|GetSpringArm))
  (bind _outactors (Actor|GetAllActorsOfClass (Variables|Default|GetPlayer%20Class)))
  (Utilities|FlowControl|Sequence
    (:then_0
      (for _array_element _outactors
        (Variables|Default|SetPosition (+ (Transformation|GetActorLocation _array_element) (Variables|Default|GetPosition))))
      (if (> (Utilities|Array|Length _outactors) 0)
        (Transformation|SetActorLocation (Math|Vector|MakeVector (Math|Float|Clamp(Float) (.x (Math|Interpolation|VInterpTo (Transformation|GetActorLocation) (Math|Vector|MakeVector (.x (+ (/ (Variables|Default|GetPosition) (Utilities|Array|Length _outactors)) (Variables|Default|GetOffset))) (.y _returnvalue) (.z _returnvalue)) (Utilities|Time|GetWorldDeltaSeconds) 2.6)) (Variables|Default|GetMin_Value_X) (Variables|Default|GetMax_Value_X)) (.y (Math|Interpolation|VInterpTo (Transformation|GetActorLocation) (Math|Vector|MakeVector (.x (+ (/ (Variables|Default|GetPosition) (Utilities|Array|Length _outactors)) (Variables|Default|GetOffset))) (.y _returnvalue) (.z _returnvalue)) (Utilities|Time|GetWorldDeltaSeconds) 2.6)) (.z (Math|Interpolation|VInterpTo (Transformation|GetActorLocation) (Math|Vector|MakeVector (.x (+ (/ (Variables|Default|GetPosition) (Utilities|Array|Length _outactors)) (Variables|Default|GetOffset))) (.y _returnvalue) (.z _returnvalue)) (Utilities|Time|GetWorldDeltaSeconds) 2.6))) false false)
        (Variables|Default|SetPosition "0, 0, 0")))
    (:then_1
      (for _array_element_2 _outactors
        (if (>= (Math|Vector|Distance(Vector) (Math|Vector|MakeVector (.x (Transformation|GetActorLocation)) 0.0 0.0) (Math|Vector|MakeVector (.x (Transformation|GetActorLocation _array_element_2)) 0.0 0.0)) (Variables|Default|GetDistance%20To%20Furthest%20Player))
          (Variables|Default|SetDistance%20To%20Furthest%20Player (Math|Vector|Distance(Vector) (Math|Vector|MakeVector (.x (Transformation|GetActorLocation)) 0.0 0.0) (Math|Vector|MakeVector (.x (Transformation|GetActorLocation _array_element_2)) 0.0 0.0)))))
      (Variables|/Script/Engine.SpringArmComponent|SetTargetArmLength _springarm (Math|Interpolation|FInterpTo (Variables|/Script/Engine.SpringArmComponent|GetTargetArmLength _springarm) (Math|Float|Clamp(Float) (* (Variables|Default|GetDistance%20To%20Furthest%20Player) (Variables|Default|GetCamera%20Zoom%20Multiplier)) (Variables|Default|GetMin%20Arn%20Length) (Variables|Default|GetMax%20Arm%20Length)) (Utilities|Time|GetWorldDeltaSeconds) 2.6))
      (Variables|Default|SetDistance%20To%20Furthest%20Player 0.0))))

(fn ConstructionScript
  (|CallParentFunction))