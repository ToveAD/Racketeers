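; Shared camera actor that frames all actors of PlayerClass by following their averaged horizontal position plus an offset.
; Each tick it finds the players and smoothly interpolates toward that point, ignoring their height.
; The farthest player's distance drives the spring arm length, clamped to a maximum, for dynamic zoom.
; Players at or beyond MaxDistanceForPlayers from the camera actor are teleported to their own KnockbackPosition.
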(event EventTick
  (params (DeltaSeconds :type Float%20%28single-precision%29))
  (bind _outactors (Actor|GetAllActorsOfClass (Variables|Default|GetPlayer%20Class)))
  (for _array_element _outactors
    (Variables|Default|SetPosition (+ (Math|Vector|MakeVector (.x (Transformation|GetActorLocation _array_element)) (.y (Transformation|GetActorLocation _array_element)) 0.0) (Variables|Default|GetPosition))))
  (if (> (Utilities|Array|Length _outactors) 0)
    (Transformation|SetActorLocation (Math|Interpolation|VInterpTo (Transformation|GetActorLocation) (+ (/ (Variables|Default|GetPosition) (Utilities|Array|Length _outactors)) (Variables|Default|GetOffset)) DeltaSeconds 2.6) false false)
    (for _array_element_2 _outactors
      (Utilities|FlowControl|Sequence
        (:then_0
          (if (>= (Math|Vector|Distance(Vector) (Transformation|GetActorLocation _array_element_2) (Transformation|GetActorLocation)) (Variables|Default|GetMaxDistanceForPlayers))
            (Transformation|SetActorLocation _array_element_2 (Transformation|GetWorldLocation (Variables|/Game/Racketeers/Core/BP_Player.BP_Player_C|GetKnockbackPosition _array_element_2)) false false)))
        (:then_1
          (if (>= (Math|Vector|Distance(Vector) (Transformation|GetActorLocation _array_element_2) (Transformation|GetActorLocation)) (Variables|Default|GetDistance%20To%20Furthest%20Player))
            (Variables|Default|SetDistance%20To%20Furthest%20Player (Math|Vector|Distance(Vector) (Transformation|GetActorLocation _array_element_2) (Transformation|GetActorLocation)))))))
    (Variables|/Script/Engine.SpringArmComponent|SetTargetArmLength (Variables|Default|GetSpringArm) (Math|Float|Clamp(Float) (+ (Variables|Default|GetDefault%20Zoom%20value) (* (Variables|Default|GetDistance%20To%20Furthest%20Player) (Variables|Default|GetCamera%20Zoom))) 0.0 (Variables|Default|GetMax%20Arm%20Length)))
    (Variables|Default|SetPosition "0.000000,0.000000,100.000000")
    (Variables|Default|SetDistance%20To%20Furthest%20Player 0.0)))

(fn ConstructionScript)