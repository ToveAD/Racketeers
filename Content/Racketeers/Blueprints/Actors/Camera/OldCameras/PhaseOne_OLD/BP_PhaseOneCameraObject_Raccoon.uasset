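; BP_PhaseOneCameraObject_Raccoon is a camera actor from the old Phase One camera set that makes itself the first player's view target.
; On BeginPlay it continues only if player pawn 0 is a BP_Racoon.
; It then calls SetViewTargetWithBlend on player controller 0 after a short delay and repeats the same call after a second delay.
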(event EventBeginPlay
  (Utilities|Casting|CastToBP_Racoon (Game|Player|GetPlayerPawn 0))
  (Utilities|FlowControl|Delay 0.7)
  (Game|Player|SetViewTargetwithBlend (Game|GetPlayerController 0) self 0.0 "VTBlend_Linear" 0.0 false)
  (Utilities|FlowControl|Delay 1.0)
  (Game|Player|SetViewTargetwithBlend (Game|GetPlayerController 0) self 0.0 "VTBlend_Linear" 0.0 false))

(event Collision|EventActorBeginOverlap
  (params (OtherActor :type Actor%20Object%20Reference)))

(event EventTick
  (params (DeltaSeconds :type Float%20%28single-precision%29))
  (|CallParentFunction DeltaSeconds) ; This node is disabled and will not be called.\nDrag off pins to build functionality.
)

(fn ConstructionScript
  (|CallParentFunction))