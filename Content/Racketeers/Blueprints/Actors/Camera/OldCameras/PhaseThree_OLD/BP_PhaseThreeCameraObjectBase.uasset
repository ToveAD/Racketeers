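; Base camera object for Phase Three (in an OLD cameras folder) that follows the group of players along the X axis.
; Each tick it averages the locations of all PlayerClass actors, adds an offset, then smoothly interpolates toward that X, clamped between set bounds, keeping Y and Z.
; Spring-arm zoom based on the furthest player's X distance is present but disconnected, so it never runs.
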(event EventTick
  (params (DeltaSeconds :type Float%20%28single-precision%29))
  (bind _returnvalue (Transformation|GetActorLocation))
  (bind _outactors (Actor|GetAllActorsOfClass (Variables|Default|GetPlayer%20Class)))
  (Utilities|FlowControl|Sequence
    (:then_0
      (for _array_element _outactors
        (Variables|Default|SetPosition (+ (Transformation|GetActorLocation _array_element) (Variables|Default|GetPosition))))
      (if (> (Utilities|Array|Length _outactors) 0)
        (Transformation|SetActorLocation (Math|Vector|MakeVector (Math|Float|Clamp(Float) (.x (Math|Interpolation|VInterpTo (Transformation|GetActorLocation) (Math|Vector|MakeVector (.x (+ (/ (Variables|Default|GetPosition) (Utilities|Array|Length _outactors)) (Variables|Default|GetOffset))) (.y _returnvalue) (.z _returnvalue)) (Utilities|Time|GetWorldDeltaSeconds) 2.6)) (Variables|Default|GetMin_Value_X) (Variables|Default|GetMax_Value_X)) (.y (Math|Interpolation|VInterpTo (Transformation|GetActorLocation) (Math|Vector|MakeVector (.x (+ (/ (Variables|Default|GetPosition) (Utilities|Array|Length _outactors)) (Variables|Default|GetOffset))) (.y _returnvalue) (.z _returnvalue)) (Utilities|Time|GetWorldDeltaSeconds) 2.6)) (.z (Math|Interpolation|VInterpTo (Transformation|GetActorLocation) (Math|Vector|MakeVector (.x (+ (/ (Variables|Default|GetPosition) (Utilities|Array|Length _outactors)) (Variables|Default|GetOffset))) (.y _returnvalue) (.z _returnvalue)) (Utilities|Time|GetWorldDeltaSeconds) 2.6))) false false)
        (Variables|Default|SetPosition "0, 0, 0")))))

(fn ConstructionScript
  (|CallParentFunction))