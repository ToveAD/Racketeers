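; Raccoon ship actor that takes control from the player on BeginPlay and can fire projectiles from side turrets.
; AttachPlayerToShip disables player collision, makes the controller possess the ship, then after a delay restores the original view target, attaches the controller and changes input mapping contexts.
; Shoot spawns BP_Projectile from the left or right turret with an upward pitch offset.
; It only handles player index 0, and the server attach event is empty.
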(event Custom|AttachPlayerToShip
  (Collision|SetActorEnableCollision (Variables|Default|GetAs%20BP%20Player) false)
  (Pawn|Possess (Game|GetPlayerController (Variables|/Script/Engine.Pawn|GetPlayerState (Variables|Default|GetAs%20BP%20Player))) self)
  (Utilities|FlowControl|Delay 1.0)
  (Game|Player|SetViewTargetwithBlend (Game|GetPlayerController (Variables|/Script/Engine.Pawn|GetPlayerState (Variables|Default|GetAs%20BP%20Player))) (Variables|Default|GetOriginalViewTarget) 0.0 "VTBlend_Linear" 0.0 false)
  (Transformation|AttachActorToActor (Game|GetPlayerController (Variables|/Script/Engine.Pawn|GetPlayerState (Variables|Default|GetAs%20BP%20Player))) self "None" "SnapToTarget" "SnapToTarget" "KeepRelative" false)
  (Input|RemoveMappingContext (PlayerController|LocalPlayerSubsystems|GetEnhancedInputLocalPlayerSubsystem (Game|GetPlayerController (Variables|/Script/Engine.Pawn|GetPlayerState (Variables|Default|GetAs%20BP%20Player)))) "/Game/Racketeers/Characters/Input/IMC_Default.IMC_Default" "(bIgnoreAllPressedKeysUntilRelease=True,bForceImmediately=False,bNotifyUserSettings=False)")
  (Input|AddMappingContext (PlayerController|LocalPlayerSubsystems|GetEnhancedInputLocalPlayerSubsystem (Game|GetPlayerController (Variables|/Script/Engine.Pawn|GetPlayerState (Variables|Default|GetAs%20BP%20Player)))) 0 1 "(bIgnoreAllPressedKeysUntilRelease=True,bForceImmediately=False,bNotifyUserSettings=False)"))

(event Custom|Server_AttachPlayerToShip)

(event EventTick
  (params (DeltaSeconds :type Float%20%28single-precision%29)))

(event EventBeginPlay
  (bind _asbp_player (Utilities|Casting|CastToBP_Player (Game|GetPlayerCharacter 0)))
  (bind _output_get (Variables|Default|SetAs%20BP%20Player _asbp_player))
  (Variables|Default|SetOriginalViewTarget (Pawn|GetViewTarget (Game|GetPlayerController (Variables|/Script/Engine.Pawn|GetPlayerState _output_get))))
  (CallFunction|AttachPlayertoShip))

(event Collision|EventActorBeginOverlap
  (params (OtherActor :type Actor%20Object%20Reference)))

(fn ConstructionScript
  (|CallParentFunction))

(fn Shoot
  (params (ShootLeft :type Boolean))
  (bind _turretone_right (Variables|Default|GetTurretOne_Right))
  (bind _turretone_left (Variables|Default|GetTurretOne_Left))
  (bind _returnvalue (Transformation|GetWorldRotation _turretone_left))
  (bind _returnvalue_2 (Transformation|GetWorldRotation _turretone_right))
  (if ShootLeft
    (Game|SpawnActorfromClass "/Game/Racketeers/Blueprints/Actors/BP_Projectile.BP_Projectile_C" (Math|Transform|MakeTransform (Transformation|GetWorldLocation (Variables|Default|GetProjectileSpawnOne_Left)) (Math|Rotator|MakeRotator (.roll _returnvalue) (+ (.pitch _returnvalue) 15.0) (.yaw _returnvalue)) "1.000000,1.000000,1.000000") "Undefined" "MultiplyWithRoot" 0 0)
    (else
      (Game|SpawnActorfromClass "/Game/Racketeers/Blueprints/Actors/BP_Projectile.BP_Projectile_C" (Math|Transform|MakeTransform (Transformation|GetWorldLocation (Variables|Default|GetProjectileSpawnTwo_Right)) (Math|Rotator|MakeRotator (.roll _returnvalue_2) (+ (.pitch _returnvalue_2) 15.0) (.yaw _returnvalue_2)) "1.000000,1.000000,1.000000") "Undefined" "MultiplyWithRoot" 0 0))))