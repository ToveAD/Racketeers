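; BP_Phase3LandscapeManager picks one landscape at random from its LandScapes array and makes it visible.
; On BeginPlay, the authority runs ServerSetLandscape, which rolls RNGNumber and unhides the actor at that index.
; Remote instances skip the roll and unhide the actor matching their current RNGNumber once, at their own BeginPlay.
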(event Custom|ServerSetLandscape
  (Utilities|FlowControl|Sequence
    (:then_0
      (Networking|SwitchHasAuthority
        (:Authority
          (Variables|Default|SetRNGNumber (Math|Random|RandomInteger (Utilities|Array|Length (Variables|Landscaping|GetLandScapes)))))))
    (:then_1
      (for (_array_element _array_index) (Variables|Landscaping|GetLandScapes)
        (if (== _array_index (Variables|Default|GetRNGNumber))
          (Rendering|SetActorHiddenInGame _array_element false))))))

(event EventBeginPlay
  (Networking|SwitchHasAuthority
    (:Authority
      (CallFunction|ServerSetLandscape))
    (:Remote
      (for (_array_element _array_index) (Variables|Landscaping|GetLandScapes)
        (if (== _array_index (Variables|Default|GetRNGNumber))
          (Rendering|SetActorHiddenInGame _array_element false))))))

(fn ConstructionScript)