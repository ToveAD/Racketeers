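; BP_Timer is an actor that holds a time value and sets up the timer widget for the local player.
; BeginPlay and Tick share one check that, if IsPlayerInSession is false, prints the net ID, adds the widget and registers itself inactive at zero seconds via RacketeersController.
; Tick then disables itself, so it serves as a retry loop.
; SetTime stores the value; GetTime pushes it to the supplied timer.
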(event Custom|SetTime
  (params (Time :type Float%20%28double-precision%29))
  (Variables|Default|SetTime Time))

(event Custom|GetTime
  (params (Timer :type BP%20Timer%20Object%20Reference))
  (CallFunction|SetTime Timer (Variables|Default|GetTime)))

(event EventBeginPlay
  (bind _returnvalue (Game|GetPlayerController 0))
  (bind _returnvalue_2 (Game|GetPlayerController 0))
  (bind _timer_widget (Variables|Default|GetTimer%20Widget))
  (bind _uniquenetid (Class|AdvancedSessionsLibrary|GetUniqueNetID _returnvalue))
  (bind _asbp_player_controller (Utilities|Casting|CastToBP_PlayerController _returnvalue_2))
  (bind _bisinsession (Class|AdvancedSessionsLibrary|IsPlayerinSession _uniquenetid))
  (if (not _bisinsession)
    (Development|PrintText (Utilities|Text|ToText(String) (Class|AdvancedSessionsLibrary|UniqueNetIdtoString _uniquenetid)) true true "(R=1.000000,G=0.000000,B=0.085470,A=1.000000)")
    (Class|RacketeersController|AddWidgettoViewport _asbp_player_controller _timer_widget)
    (Utilities|Casting|CastToWBP_Timer _timer_widget)
    (bind _asracketeers_controller (Utilities|Casting|CastToRacketeersController _returnvalue_2))
    (Class|RacketeersController|SetMultiTimeSeconds _asracketeers_controller self 0.0 false)
    (Actor|Tick|SetActorTickEnabled false)))

(event EventTick
  (params (DeltaSeconds :type Float%20%28single-precision%29))
  (bind _returnvalue (Game|GetPlayerController 0))
  (bind _returnvalue_2 (Game|GetPlayerController 0))
  (bind _timer_widget (Variables|Default|GetTimer%20Widget))
  (bind _uniquenetid (Class|AdvancedSessionsLibrary|GetUniqueNetID _returnvalue))
  (bind _asbp_player_controller (Utilities|Casting|CastToBP_PlayerController _returnvalue_2))
  (bind _bisinsession (Class|AdvancedSessionsLibrary|IsPlayerinSession _uniquenetid))
  (if (not _bisinsession)
    (Development|PrintText (Utilities|Text|ToText(String) (Class|AdvancedSessionsLibrary|UniqueNetIdtoString _uniquenetid)) true true "(R=1.000000,G=0.000000,B=0.085470,A=1.000000)")
    (Class|RacketeersController|AddWidgettoViewport _asbp_player_controller _timer_widget)
    (Utilities|Casting|CastToWBP_Timer _timer_widget)
    (bind _asracketeers_controller (Utilities|Casting|CastToRacketeersController _returnvalue_2))
    (Class|RacketeersController|SetMultiTimeSeconds _asracketeers_controller self 0.0 false)
    (Actor|Tick|SetActorTickEnabled false)))

(fn ConstructionScript)