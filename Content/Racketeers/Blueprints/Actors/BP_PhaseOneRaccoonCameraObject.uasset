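; BP_PhaseOneRaccoonCameraObject is a shared camera actor that becomes player controller 0's view target one second after BeginPlay.
; Each tick it sums the locations of all BP_Player actors and moves to half that sum, a midpoint that assumes exactly two players.
; It sets the spring arm length to that point's vector length, so zoom follows distance from the world origin rather than player separation.
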(event EventBeginPlay
  (Utilities|FlowControl|Delay 1.0)
  (Game|Player|SetViewTargetwithBlend (Game|GetPlayerController 0) self 0.0 "VTBlend_Linear" 0.0 false))

(event Collision|EventActorBeginOverlap
  (params (OtherActor :type Actor%20Object%20Reference)))

(event EventTick
  (params (DeltaSeconds :type Float%20%28single-precision%29))
  (bind _outactors (Actor|GetAllActorsOfClass "/Game/Racketeers/Core/BP_Player.BP_Player_C"))
  (for _array_element _outactors
    (Variables|Default|SetTempVector (+ (Transformation|GetActorLocation _array_element) (Variables|Default|GetTempVector))))
  (Transformation|SetActorLocation (/ (Variables|Default|GetTempVector) 2.0) false false)
  (Variables|/Script/Engine.SpringArmComponent|SetTargetArmLength (Variables|Default|GetSpringArm) (Math|Vector|VectorLength (/ (Variables|Default|GetTempVector) 2.0)))
  (Variables|Default|SetTempVector "0, 0, 0"))

(fn ConstructionScript)