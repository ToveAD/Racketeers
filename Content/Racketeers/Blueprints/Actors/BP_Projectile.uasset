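; BP_Projectile is a replicated cannonball whose replicated LongestRange caps its movement speed and which expires after a fixed lifespan.
; Sphere hits branch on boat or water, routing through Server events to Multicast events for Niagara effects and sounds.
; Boat hits disable collision on the server without destroying the ball or applying damage here.
; Water hits splash at zero height and destroy it.
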(event OnComponentHit(Sphere1)
  (params (HitComponent :type Primitive%20Component%20Object%20Reference) (OtherActor :type Actor%20Object%20Reference) (OtherComp :type Primitive%20Component%20Object%20Reference) (NormalImpulse :type Vector :default "0, 0, 0") (Hit :type Hit%20Result%20Structure%20%28by%20ref%29))
  (bind _returnvalue (Utilities|GetClass OtherActor))
  ;[1 1 1] Hit boat with projectile
  (if (Utilities|ClassIsChildOf _returnvalue "/Game/Developers/jahj7676/Jacob/BP_Water.BP_Water_C")
    (CallFunction|HitWater)
    (elif (Utilities|ClassIsChildOf _returnvalue "/Game/Racketeers/Blueprints/Actors/BP_Boat.BP_Boat_C")
      (CallFunction|HitBoat))))

(event Custom|Server_HitBoat
  ;[1 1 1] Hit boat with projectile
  ;;[1 1 1] Run on Server
  (Collision|SetCollisionEnabled (Variables|Default|GetSphere1) "NoCollision")
  ;;;[1 1 1] Run particles on multi
  (CallFunction|MultiHitBoat))

(event Custom|HitBoat
  ;[1 1 1] Hit boat with projectile
  ;;[1 1 1] Call on Server
  (CallFunction|ServerHitBoat))

(event Custom|Multi_HitBoat
  (bind _sphere1 (Variables|Default|GetSphere1))
  ;[1 1 1] Hit boat with projectile
  ;;[1 1 1] Run on Multi - Spawn Particles
  (Niagara|SpawnSystematLocation "/Game/Racketeers/Art/Niagara/Cannon/FXS_Impact.FXS_Impact" (Transformation|GetWorldLocation _sphere1) (Transformation|GetWorldRotation _sphere1))
  (Audio|PlaySoundatLocation "/Game/Racketeers/Audio/SFX/Ship/SFX_CannonFire.SFX_CannonFire" (Transformation|GetWorldLocation (Variables|Default|GetSphere1)) "0, 0, 0" 0.7 1.0 0.0 0 0 0 0)
  (Audio|PlaySoundatLocation (.OutItem (Utilities|Array|Random (Variables|Default|GetHitSounds))) (Transformation|GetWorldLocation (Variables|Default|GetSphere1)) "0, 0, 0" 3.0 1.4 0.0 0 0 0 0))

(event Custom|HitWater
  ;[1 1 1] Hit Water
  ;;[1 1 1] Call on server
  (CallFunction|ServerHitWater))

(event Custom|Server_HitWater
  ;[1 1 1] Hit Water
  ;;[1 1 1] Server call multi
  (CallFunction|MultiHitWater))

(event Custom|Multi_HitWater
  (bind _sphere1 (Variables|Default|GetSphere1))
  (bind _returnvalue (Transformation|GetWorldLocation _sphere1))
  ;[1 1 1] Hit Water
  ;;[1 1 1] Run on multi
  (Niagara|SpawnSystematLocation "/Game/Racketeers/Art/Niagara/Water/FXS_Splash.FXS_Splash" (Math|Vector|MakeVector (.x _returnvalue) (.y _returnvalue) 0.0))
  (Audio|PlaySoundatLocation "/Game/Racketeers/Audio/SFX/Ship/SFX_CannonballSplash.SFX_CannonballSplash" (Transformation|GetWorldLocation (Variables|Default|GetSphere1)) "0, 0, 0" 0.3 (Math|Random|RandomFloatinRange 1.5 2.0) 0.0 0 0 0 0)
  (Actor|DestroyActor))

(event Custom|IgnoreSelf
  (params (Actor :type Actor%20Object%20Reference))
  ;[1 1 1] Ignore self
  (Collision|IgnoreActorwhenMoving (Variables|Default|GetSphere) Actor true))

(event EventBeginPlay
  ;[1 1 1] Destroys projectile after Set Time
  (Actor|SetLifeSpan 6.0)
  ;[1 1 1] Projectile Range On Hold
  (bind _output_get (Variables|Default|SetLongestRange (Variables|Default|GetLongestRange)))
  (Variables|/Script/Engine.ProjectileMovementComponent|SetMaxSpeed (Variables|Default|GetProjectileMovement) _output_get))

(fn ConstructionScript)

(fn OnRepLongestRange
  (Variables|/Script/Engine.ProjectileMovementComponent|SetMaxSpeed (Variables|Default|GetProjectileMovement) (Variables|Default|GetLongestRange)))