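; BP_BoatSafeZone is an actor with a SafeZone overlap volume meant to mark a safe area for boats in Racketeers.
; Begin and end overlaps print debug messages when the overlapping actor's Instigator is locally controlled.
; Begin overlap also stores any BP_Boat in BoatRef.
; The nodes that set the boat's InSafeZone flag are disconnected, so the zone currently does not change boat state.
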(event OnComponentBeginOverlap(SafeZone)
  (params (OverlappedComponent :type Primitive%20Component%20Object%20Reference) (OtherActor :type Actor%20Object%20Reference) (OtherComp :type Primitive%20Component%20Object%20Reference) (OtherBodyIndex :type Integer) (bFromSweep :type Boolean) (SweepResult :type Hit%20Result%20Structure%20%28by%20ref%29))
  (if (Pawn|IsLocallyControlled (Variables|/Script/Engine.Actor|GetInstigator OtherActor))
    (Development|PrintString "IN SAFE ZONE FOR BOAT" true true "(R=0.131722,G=1.000000,B=0.135433,A=1.000000)")
    (Development|PrintString (Utilities|GetDisplayName OtherActor)))
  (if (Utilities|ClassIsChildOf (Utilities|GetClass OtherActor) "/Game/Racketeers/Blueprints/Actors/BP_Boat.BP_Boat_C")
    (bind _asbp_boat (Utilities|Casting|CastToBP_Boat OtherActor))
    (bind _output_get (Variables|Default|SetBoatRef _asbp_boat))))

(event OnComponentEndOverlap(SafeZone)
  (params (OverlappedComponent :type Primitive%20Component%20Object%20Reference) (OtherActor :type Actor%20Object%20Reference) (OtherComp :type Primitive%20Component%20Object%20Reference) (OtherBodyIndex :type Integer))
  (if (Pawn|IsLocallyControlled (Variables|/Script/Engine.Actor|GetInstigator OtherActor))
    (Development|PrintString "NOT IN SAFE ZONE FOR BOAT" true true "(R=0.212387,G=0.735984,B=1.000000,A=1.000000)"))
  (if (Utilities|ClassIsChildOf (Utilities|GetClass OtherActor) "/Game/Racketeers/Blueprints/Actors/BP_Boat.BP_Boat_C")
    _))

(event EventBeginPlay)

(event Collision|EventActorBeginOverlap
  (params (OtherActor :type Actor%20Object%20Reference)))

(event EventTick
  (params (DeltaSeconds :type Float%20%28single-precision%29)))

(fn ConstructionScript)