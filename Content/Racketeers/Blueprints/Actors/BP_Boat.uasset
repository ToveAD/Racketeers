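; Drivable team boat for Racketeers that a player boards to sail, boost and fire broadside cannons.
; Boarding attaches the player, swaps input mapping and tags the boat as Raccoon or Panda; leaving or map unload detaches them.
; Input events relay through server and multicast events to MovementBoat, timer-based cooldowns and staggered cannon shots with effects and sound.
; Projectile hits send team damage to RacketeersController, chosen by boat tag.
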(event OnComponentHit(StaticMesh)
  (params (HitComponent :type Primitive%20Component%20Object%20Reference) (OtherActor :type Actor%20Object%20Reference) (OtherComp :type Primitive%20Component%20Object%20Reference) (NormalImpulse :type Vector :default "0, 0, 0") (Hit :type Hit%20Result%20Structure%20%28by%20ref%29))
  ;[1 1 1] Take damage from BP_Projectile
  ;;[1 1 1] Tell boat to take damage
  (CallFunction|TakeDamage OtherActor))

(event Custom|StartScurryBoat
  ;[1 1 1] Inputs (Are Called From BP_Player)
  ;;[1 1 1] Start Scurry Boat
  (CallFunction|ServerStartScurryBoat))

(event Custom|Server_BoatShootLeft
  ;[1 1 1] Inputs (Are Called From BP_Player)
  ;;[1 1 1] Shoot Left
  ;;;[1 1 1] Call on Server
  (CallFunction|MultiReloadSound)
  (Utilities|ShootCannons true (Variables|Cannons|GetCannonAmount)))

(event Custom|Multi_StartInteract
  (params (Instigator :type Actor%20Object%20Reference))
  ;[1 1 1] Start Interact
  ;;[1 1 1] 2. Send to all clients
  (CallFunction|SetReferences Instigator)
  (CallFunction|SetTag Instigator)
  (CallFunction|EnterBoat)
  ;;;[1 1 1] Prevent accidental shooting at interact
  (if (Variables|Default|GetbHasEnteredBoat)
    _
    (else
      (Utilities|FlowControl|Delay 0.2)))
  (Class|InputHandler|SwitchInputMapping (Variables|Default|GetInputHandler) true "/Game/Racketeers/Characters/Input/IMC_Boat.IMC_Boat" "/Game/Racketeers/Characters/Input/IMC_Default.IMC_Default" (Variables|Default|GetPlayerController))
  (Variables|Default|SetbHasEnteredBoat true))

(event Custom|BoatShootRight
  ;[1 1 1] Inputs (Are Called From BP_Player)
  ;;[1 1 1] Shoot Right
  (Utilities|SetTimerShoot false)
  (CallFunction|ServerBoatShootRight))

(event Custom|Server_MoveBoat
  (params (Value :type Vector%202D%20Structure))
  ;[1 1 1] Inputs (Are Called From BP_Player)
  ;;[1 1 1] Move Boat
  ;;;[1 1 1] Call on Server
  (Class|MovementBoat|Move (Variables|Default|GetMovementBoat) Value true))

(event Custom|StopScurryBoat
  ;[1 1 1] Stop Scurry Boat
  (CallFunction|ServerStopScurryBoat))

(event Custom|Server_StopBoat
  (params (Value :type Vector%202D%20Structure))
  ;[1 1 1] Inputs (Are Called From BP_Player)
  ;;[1 1 1] Stop Boat
  ;;;[1 1 1] Call on Server
  (Class|MovementBoat|Move (Variables|Default|GetMovementBoat) Value false))

(event Custom|Unload
  ;[1 1 1] Detach Player When Switching Level
  ;;[1 1 1] Unload On Server (Game Mode Already Runs On Server)
  (CallFunction|MultiUnload))

(event Custom|Multi_StopInteract
  ;[1 1 1] Stop Interact
  ;;[1 1 1] 3. Send to all clients
  (CallFunction|StopInteract)
  (Collision|SetActorEnableCollision (Variables|Default|GetPlayerRef) true))

(event Custom|Server_StopScurryBoat
  ;[1 1 1] Stop Scurry Boat
  ;;[1 1 1] Call on Server
  (Class|MovementBoat|Scurry (Variables|Default|GetMovementBoat) false))

(event Custom|Multi_StartScurry
  (Audio|PlaySoundatLocation "/Game/Racketeers/Audio/SFX/Ship/SFX_ShipSailBoost.SFX_ShipSailBoost" (Transformation|GetWorldLocation (Variables|Default|GetStaticMesh)) "0, 0, 0" 1.2 1.0 0.3 0 0 0 0))

(event Custom|SetCannonAmount
  (Variables|Cannons|SetCannonAmount (Variables|Cannons|GetCannonAmount)))

(event Custom|Server_TakeDamage
  (params (OtherActor :type Object%20Object%20Reference))
  ;[1 1 1] Take damage from BP_Projectile
  ;;[1 1 1] Run on Server
  (if (Utilities|ClassIsChildOf (Utilities|GetClass OtherActor) "/Game/Racketeers/Blueprints/Actors/BP_Projectile.BP_Projectile_C")
    (Development|PrintString (Utilities|GetDisplayName OtherActor) true true "(R=0.000000,G=0.000000,B=0.000000,A=1.000000)")
    (bind _returnvalue (Actor|GetActorOfClass "/Script/Racketeers.RacketeersController"))
    (switch string (Utilities|String|ToString(Name) (Variables|Default|GetTag))
      (:BoatRaccoon
        (Variables|Default|SetTeam "Team_Raccoon"))
      (:BoatPanda
        (Variables|Default|SetTeam "Team_Panda")))
    (Class|RacketeersController|DamageBoat _returnvalue (Variables|Default|GetDamageToTake) (Variables|Default|GetTeam))
    (bind _asprojectile (Utilities|Casting|CastToProjectile OtherActor))
    (Actor|DestroyActor _asprojectile)
    (bind _asracketeers_game_state_base (Utilities|Casting|CastToRacketeersGameStateBase (Game|GetGameState))
      (:then
        (Development|PrintString (Utilities|String|ToString(Float) (Variables|/Script/Racketeers.RacketeersGameStateBase|GetRaccoonsBoatHealth _asracketeers_game_state_base)) true true "(R=0.345617,G=0.395833,B=0.340169,A=1.000000)")
        (Development|PrintString (Utilities|String|ToString(Float) (Variables|/Script/Racketeers.RacketeersGameStateBase|GetRedPandasBoatHealth _asracketeers_game_state_base)) true true "(R=1.000000,G=0.273319,B=0.193599,A=1.000000)"))
      (:CastFailed
        (Development|PrintString "Cast failed" true true "(R=1.000000,G=0.032542,B=0.000000,A=1.000000)" 1e+01)))))

(event Custom|Multi_ReloadSound
  (Audio|PlaySoundatLocation "/Game/Racketeers/Audio/SFX/Ship/SFX_ShipReloadAlt.SFX_ShipReloadAlt" (Transformation|GetWorldLocation (Variables|Default|GetStaticMesh)) "0, 0, 0" 0.7 (Math|Random|RandomFloatinRange 0.8 1.2) 0.0 0 0 0 0))

(event Custom|SetBoatMaterial
  (params (Material0 :type Material%20Interface%20Object%20Reference) (Material1 :type Material%20Interface%20Object%20Reference))
  ;[1 1 1] Set boat material
  (CallFunction|MultiSetBoatMaterial Material0 Material1))

(event Custom|Multi_SetBoatMaterial
  (params (Material0 :type Material%20Interface%20Object%20Reference) (Material1 :type Material%20Interface%20Object%20Reference))
  ;[1 1 1] Set boat material
  ;;[1 1 1] Send to all clients
  (Rendering|Material|SetMaterial (Variables|Default|GetStaticMesh) 0 Material0)
  (Rendering|Material|SetMaterial (Variables|Default|GetStaticMesh) 1 Material1))

(event Custom|EnableBoatIndicator
  ;[1 1 1] Player indicator
  (if (Pawn|IsLocallyControlled (Variables|Default|GetPlayerRef))
    (Rendering|SetVisibility (Variables|Default|GetPlayerIndicator) true false)))

(event Custom|DisableBoatIndicator
  ;[1 1 1] Player indicator
  (if (Pawn|IsLocallyControlled (Variables|Default|GetPlayerRef))
    (Rendering|SetVisibility (Variables|Default|GetPlayerIndicator) false false)))

(event Custom|MoveBoat
  (params (ActionValue :type Vector%202D%20Structure))
  ;[1 1 1] Inputs (Are Called From BP_Player)
  ;;[1 1 1] Move Boat
  (CallFunction|ServerMoveBoat ActionValue))

(event Custom|Server_StopInteract
  (params (Target :type Actor%20Object%20Reference))
  ;[1 1 1] Stop Interact
  ;;[1 1 1] 2. Server telling Multicast to send to all clients
  (CallFunction|MultiStopInteract))

(event Custom|TakeDamage
  (params (OtherActor :type Object%20Object%20Reference))
  ;[1 1 1] Take damage from BP_Projectile
  ;;[1 1 1] Call on Server
  (CallFunction|ServerTakeDamage OtherActor))

(event Custom|Multi_ShootSound
  (Audio|PlaySoundatLocation "/Game/Racketeers/Audio/SFX/Ship/SFX_CannonFire.SFX_CannonFire" (Transformation|GetWorldLocation (Variables|Default|GetStaticMesh)) "0, 0, 0" 1.0 (Math|Random|RandomFloatinRange 0.7 1.1) 0.0 0 0 0 0))

(event Custom|Server_StartScurryBoat
  ;[1 1 1] Inputs (Are Called From BP_Player)
  ;;[1 1 1] Start Scurry Boat
  ;;;[1 1 1] Call on Server
  (Utilities|SetTimerScurry)
  (CallFunction|MultiStartScurry)
  (Class|MovementBoat|Scurry (Variables|Default|GetMovementBoat) true)
  (Utilities|FlowControl|Delay (Variables|Default|GetLengthOfScurry))
  (CallFunction|StopScurryBoat))

(event Custom|Multi_Unload
  ;[1 1 1] Detach Player When Switching Level
  ;;[1 1 1] Send To All Clients
  (CallFunction|ServerStopInteract))

(event Custom|Server_BoatShootRight
  ;[1 1 1] Inputs (Are Called From BP_Player)
  ;;[1 1 1] Shoot Right
  ;;;[1 1 1] Call on Server
  (CallFunction|MultiReloadSound)
  (Utilities|ShootCannons false (Variables|Cannons|GetCannonAmount)))

(event Custom|StopBoat
  (params (Value :type Vector%202D%20Structure))
  ;[1 1 1] Inputs (Are Called From BP_Player)
  ;;[1 1 1] Stop Boat
  (CallFunction|ServerStopBoat Value))

(event Custom|LeaveBoatInteract
  ;[1 1 1] Stop Interact
  ;;[1 1 1] 1. Player sending to server
  (if (Variables|Default|GetbDetachLogicActive)
    (bind _returnvalue (CallFunction|CanLeaveBoatCheck))
    (if _returnvalue
      _
      (else
        _))
    (CallFunction|ServerStopInteract)))

(event Custom|BoatShootLeft
  ;[1 1 1] Inputs (Are Called From BP_Player)
  ;;[1 1 1] Shoot Left
  (Utilities|SetTimerShoot true)
  (CallFunction|ServerBoatShootLeft))

(event EventTick
  (params (DeltaSeconds :type Float%20%28single-precision%29))
  (bind _asracketeers_game_state_base (Utilities|Casting|CastToRacketeersGameStateBase (Game|GetGameState)))
  (if (or (== (Variables|/Script/Racketeers.RacketeersGameStateBase|GetRaccoonsBoatHealth _asracketeers_game_state_base) 1.0) (== (Variables|/Script/Racketeers.RacketeersGameStateBase|GetRedPandasBoatHealth _asracketeers_game_state_base) 1.0))
    (CallFunction|StopInteract (Variables|Default|GetPlayerRef))))

(event EventStartInteract
  (params (Instigator :type Actor%20Object%20Reference) (bIsServer :type Boolean))
  ;[1 1 1] Start Interact
  ;;[1 1 1] 1. Run On Server & Send To Multicast (Already Runs On Server In BP_Player)
  (CallFunction|MultiStartInteract Instigator))

(event EventStopInteract
  (params (Instigator :type Actor%20Object%20Reference))
  ;[1 1 1] Stop Interact
  ;;[1 1 1] 4: Hande logic
  (CallFunction|LeaveBoat))

(event EventBeginPlay
  ;[1 1 1] Detach Player When Switching Level
  ;;[1 1 1] Unload On Server (Game Mode Already Runs On Server)
  (bind _asracketeers_gmbase (Utilities|Casting|CastToRacketeersGMBase (Game|GetGameMode)))
  (EventDispatchers|BindEventtoOnUnloadingMap _asracketeers_gmbase (delegate Custom|Unload))
  (CallFunction|SetCannons))

(event EventDestroyed)

(fn ConstructionScript)

(fn Timer
  (Variables|Default|SetbCanAccelerate true))

(fn EnterBoat
  (Collision|SetActorEnableCollision (Variables|Default|GetInstigatorRef) false)
  (Transformation|AttachComponentToComponent (Variables|Default|GetPlayerRef) (Variables|Default|GetPlayerPos) "None" "SnapToTarget" "SnapToTarget" "KeepWorld" false)
  (Actor|SetOwner self (Variables|Default|GetPlayerRef))
  (Pawn|Components|CharacterMovement|DisableMovement (Variables|/Script/Engine.Character|GetCharacterMovement (Variables|Default|GetPlayerRef)))
  (Collision|SetCollisionProfileName (Variables|Default|GetStaticMesh) "BoatAttached" true :!class /Script/Engine.PrimitiveComponent)
  (Default|DisablePlayerIndicator (Variables|Default|GetPlayerRef))
  (CallFunction|EnableBoatIndicator)
  (return))

(fn LeaveBoat
  (Transformation|DetachFromActor (Variables|Default|GetPlayerRef) "KeepWorld" "KeepWorld" "KeepWorld")
  (Transformation|SetActorLocation (Variables|Default|GetPlayerRef) (Transformation|GetWorldLocation (Variables|Default|GetDetachPos)) false false)
  (Actor|SetOwner self (Variables|Default|GetPlayerRef))
  (Utilities|IsValid (Variables|Default|GetPlayerRef)
    (:Is%20Valid
      (Utilities|IsValid (Variables|Default|GetPlayerController)
        (:Is%20Valid
          (Pawn|Components|CharacterMovement|SetMovementMode (Variables|/Script/Engine.Character|GetCharacterMovement (Variables|Default|GetPlayerRef)) "MOVE_Walking" 0)
          (Class|InputHandler|SwitchInputMapping (Variables|Default|GetInputHandler) false "/Game/Racketeers/Characters/Input/IMC_Boat.IMC_Boat" "/Game/Racketeers/Characters/Input/IMC_Default.IMC_Default" (Variables|Default|GetPlayerController))
          (Collision|SetCollisionProfileName (Variables|Default|GetStaticMesh) "BoatDetached" true :!class /Script/Engine.PrimitiveComponent)
          (Default|EnablePlayerIndicator (Variables|Default|GetPlayerRef))
          (CallFunction|DisableBoatIndicator)
          (Variables|Default|SetbCanInteract true))))))

(fn CanLeaveBoatCheck
  (bind _staticmesh (Variables|Default|GetStaticMesh))
  (bind _returnvalue (Transformation|GetWorldLocation _staticmesh))
  (bind _returnvalue_2 (Actor|GetActorOfClass "/Script/Water.WaterBodyCustom"))
  (bind (_outhits _returnvalue_3) (Class|KismetSystemLibrary|BoxTraceMultiforObjects _returnvalue _returnvalue (Variables|/Script/Engine.BoxComponent|GetBoxExtent (Variables|Default|GetIslandCheck)) (Transformation|GetActorRotation) (Utilities|Array|MakeArray "ObjectTypeQuery1") false (Utilities|Array|MakeArray _returnvalue_2 0) "ForDuration" true))
  (if _returnvalue_3
    (bind _array_element (Utilities|Array|ForEachLoopwithBreak _outhits)
      (:LoopBody
        (Development|PrintString (Utilities|GetDisplayName (.HitComponent (Collision|BreakHitResult _array_element))))
        (Development|PrintString (Utilities|String|ToString(Boolean) (Actor|ActorHasTag (.HitActor (Collision|BreakHitResult _array_element)) "Island"))))
      (:Completed
        (return (Actor|ActorHasTag (.HitActor (Collision|BreakHitResult _array_element)) "Island"))))))

(fn SetReferences
  (params (Instigator :type Actor%20Object%20Reference))
  (bind _output_get (Variables|Default|SetInstigatorRef Instigator))
  (bind _asbp_player (Utilities|Casting|CastToBP_Player _output_get))
  (bind _output_get_2 (Variables|Default|SetPlayerRef _asbp_player))
  (Utilities|IsValid _output_get_2
    (:Is%20Valid
      (bind _asbp_player_controller (Utilities|Casting|CastToBP_PlayerController (Pawn|GetController (Variables|Default|GetPlayerRef))))
      (bind _output_get_3 (Variables|Default|SetPlayerController _asbp_player_controller))
      (Utilities|IsValid _output_get_3
        (:Is%20Valid
          (Variables|Default|SetbCanInteract false)
          (return))
        (:Is%20Not%20Valid
          (Development|PrintString "Player Controller Not Valid" true true "(R=1.000000,G=0.154444,B=0.000000,A=1.000000)"))))
    (:Is%20Not%20Valid
      (Development|PrintString "PlayerRef Not Valid" true true "(R=1.000000,G=0.181028,B=0.000000,A=1.000000)"))))

(fn OnRepNewLocation
  (Transformation|SetActorLocation (Transformation|GetActorLocation) false false))

(fn OnRepNewRotation
  (Transformation|SetActorRotation (Transformation|GetActorRotation)))

(fn Shoot
  (params (ShootLeft :type Boolean) (CannonAmount :type Integer))
  (LocalVariables|SetbShootLeft ShootLeft)
  (switch int CannonAmount
    (:1
      (if (LocalVariables|GetbShootLeft)
        (bind _returnvalue (CallFunction|SpawnProjectile (Variables|Default|GetProjectile1_L) (Variables|Default|GetCannon1_L)))
        (CallFunction|SetShootRange _returnvalue)
        (else
          (bind _returnvalue_2 (CallFunction|SpawnProjectile (Variables|Default|GetProjectile1_R) (Variables|Default|GetCannon1_R)))
          (CallFunction|SetShootRange _returnvalue_2))))
    (:2
      (if (LocalVariables|GetbShootLeft)
        (bind _returnvalue_3 (CallFunction|SpawnProjectile (Variables|Default|GetProjectile1_L) (Variables|Default|GetCannon1_L)))
        (CallFunction|SetShootRange _returnvalue_3)
        (bind _returnvalue_4 (CallFunction|SpawnProjectile (Variables|Default|GetProjectile2_L) (Variables|Default|GetCannon2_L)))
        (CallFunction|SetShootRange _returnvalue_4)
        (else
          (bind _returnvalue_5 (CallFunction|SpawnProjectile (Variables|Default|GetProjectile1_R) (Variables|Default|GetCannon1_R)))
          (CallFunction|SetShootRange _returnvalue_5)
          (bind _returnvalue_6 (CallFunction|SpawnProjectile (Variables|Default|GetProjectile2_R) (Variables|Default|GetCannon2_R)))
          (CallFunction|SetShootRange _returnvalue_6))))
    (:3
      (if (LocalVariables|GetbShootLeft)
        (bind _returnvalue_7 (CallFunction|SpawnProjectile (Variables|Default|GetProjectile1_L) (Variables|Default|GetCannon1_L)))
        (CallFunction|SetShootRange _returnvalue_7)
        (bind _returnvalue_8 (CallFunction|SpawnProjectile (Variables|Default|GetProjectile2_L) (Variables|Default|GetCannon2_L)))
        (CallFunction|SetShootRange _returnvalue_8)
        (bind _returnvalue_9 (CallFunction|SpawnProjectile (Variables|Default|GetProjectile3_L) (Variables|Default|GetCannon3_L)))
        (CallFunction|SetShootRange _returnvalue_9)
        (else
          (bind _returnvalue_10 (CallFunction|SpawnProjectile (Variables|Default|GetProjectile1_R) (Variables|Default|GetCannon1_R)))
          (CallFunction|SetShootRange _returnvalue_10)
          (bind _returnvalue_11 (CallFunction|SpawnProjectile (Variables|Default|GetProjectile2_R) (Variables|Default|GetCannon2_R)))
          (CallFunction|SetShootRange _returnvalue_11)
          (bind _returnvalue_12 (CallFunction|SpawnProjectile (Variables|Default|GetProjectile3_R) (Variables|Default|GetCannon3_R)))
          (CallFunction|SetShootRange _returnvalue_12))))))

(fn TimerShootLeft
  (Variables|Default|SetbCanShootLeft true))

(fn TimerAccelerate
  (Variables|Default|SetbCanAccelerate true))

(fn TimerShootRight
  (Variables|Default|SetbCanShootRight true))

(fn SetShootRange
  (params (Projectile :type BP%20Projectile%20Object%20Reference))
  (Variables|/Game/Racketeers/Blueprints/Actors/BP_Projectile.BP_Projectile_C|SetLongestRange Projectile (* (Variables|/Game/Racketeers/Blueprints/Actors/BP_Projectile.BP_Projectile_C|GetShortestRange Projectile) (Variables|/Game/Racketeers/Core/BP_Player.BP_Player_C|GetShootTime (Variables|Default|GetPlayerRef)))))

(fn SpawnProjectile
  (params (SpawnPoint :type Scene%20Component%20Object%20Reference) (Cannon :type Scene%20Component%20Object%20Reference))
  (bind _returnvalue (Transformation|GetWorldRotation Cannon))
  (bind _returnvalue_2 (Game|SpawnActorfromClass "/Game/Racketeers/Blueprints/Actors/BP_Projectile.BP_Projectile_C" (Math|Transform|MakeTransform (Transformation|GetWorldLocation SpawnPoint) (Math|Rotator|MakeRotator (.roll _returnvalue) (+ (.pitch _returnvalue) 15.0) (.yaw _returnvalue)) "1.000000,1.000000,1.000000") "Undefined" "MultiplyWithRoot" 0 0))
  (return _returnvalue_2))

(fn SetTag
  (params (Instigator :type Actor%20Object%20Reference))
  (if (Utilities|ClassIsChildOf (Utilities|GetClass Instigator) "/Game/Racketeers/Characters/Blueprints/BP_Racoon.BP_Racoon_C")
    (Variables|Default|SetTag "BoatRaccoon")
    (else
      (Variables|Default|SetTag "BoatPanda")))
  (Utilities|Array|Add (Variables|Actor|GetTags) (Variables|Default|GetTag))
  (Development|PrintString (Utilities|String|ToString(Name) (Variables|Default|GetTag)) true true "(R=0.961847,G=0.000000,B=1.000000,A=1.000000)" 1e+02))

(fn ServerRaccoonTakeDamage
  (params (OtherActor1 :type Object%20Object%20Reference)))

(fn ShootCannon
  (params (ShootLeft :type Boolean) (CannonIndex :type Integer))
  (if ShootLeft
    (switch int CannonIndex
      (:1
        (CallFunction|SetandSpawnCannons (Variables|Default|GetProjectile1_L) (Variables|Default|GetCannon1_L) (Variables|Default|GetShootingEffect1_L)))
      (:2
        (CallFunction|SetandSpawnCannons (Variables|Default|GetProjectile2_L) (Variables|Default|GetCannon2_L) (Variables|Default|GetShootingEffect2_L)))
      (:3
        (CallFunction|SetandSpawnCannons (Variables|Default|GetProjectile3_L) (Variables|Default|GetCannon3_L) (Variables|Default|GetShootingEffect3_L))))
    (else
      (switch int CannonIndex
        (:1
          (CallFunction|SetandSpawnCannons (Variables|Default|GetProjectile1_R) (Variables|Default|GetCannon1_R) (Variables|Default|GetShootingEffect1_R)))
        (:2
          (CallFunction|SetandSpawnCannons (Variables|Default|GetProjectile2_R) (Variables|Default|GetCannon2_R) (Variables|Default|GetShootingEffect2_R)))
        (:3
          (CallFunction|SetandSpawnCannons (Variables|Default|GetProjectile3_R) (Variables|Default|GetCannon3_R) (Variables|Default|GetShootingEffect3_R)))))))

(fn TimerScurry
  (Variables|Default|SetbCanScurry true))

(fn SetandSpawnCannons
  (params (ProjectileSpawnPoint :type Scene%20Component%20Object%20Reference) (CannonIndex :type Scene%20Component%20Object%20Reference) (EffectIndex :type Niagara%20Component%20Object%20Reference))
  (Variables|Default|SetProjectileSpawnPoint ProjectileSpawnPoint)
  (Variables|Default|SetCannonIndex CannonIndex)
  (Variables|Default|SetEffectIndex EffectIndex)
  (bind _returnvalue (CallFunction|SpawnProjectile (Variables|Default|GetProjectileSpawnPoint) (Variables|Default|GetCannonIndex)))
  (CallFunction|SetShootRange _returnvalue)
  (Default|ServerOneEffectCall (Variables|Default|GetEffectsComponent) (Variables|Default|GetEffectIndex))
  (CallFunction|MultiShootSound)
  (return))

(fn TimerCannons
  (Variables|Cannons|SetbCannonCanShoot true))

(fn SetCannons
  (switch int (Variables|Cannons|GetCannonAmount)
    (:0
      (Rendering|SetVisibility (Variables|Default|GetCannon1_L) false false))
    (:1
      (Rendering|SetVisibility (Variables|Default|GetCannon2_L) false false))
    (:2
      (Rendering|SetVisibility (Variables|Default|GetCannon3_L) false false))))

(fn OnRepInteractCounter
  (Variables|Default|SetInteractCounter (+ (Variables|Default|GetInteractCounter) 1)))

(fn CanInteract
  (return (Variables|Default|GetbCanInteract)))