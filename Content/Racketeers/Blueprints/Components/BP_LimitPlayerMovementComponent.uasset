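; Pawn component meant to keep players within the phase-one camera's maximum distance, though it currently only prints debug vectors.
; After a one-second startup delay, Tick measures the pawn's horizontal offset from its BP_PhaseOneCameraObject view target against MaxDistanceForPlayers.
; Both in-range and out-of-range branches print the offset scaled to that limit, differing only in Z.
; The teleporting SetActorLocation is disconnected and uses that offset without adding the camera's location.
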(event EventBeginPlay
  (bind _aspawn (Utilities|Casting|CastToPawn (Components|GetOwner)))
  (Variables|Default|SetOwner _aspawn)
  (Utilities|FlowControl|Delay 1.0)
  (Variables|Default|SetShouldTick true))

(event EventTick
  (params (DeltaSeconds :type Float%20%28single-precision%29))
  (bind _owner (Variables|Default|GetOwner))
  (bind _returnvalue (Transformation|GetActorLocation _owner))
  (bind _returnvalue_2 (Pawn|GetController _owner))
  (bind _returnvalue_3 (Pawn|GetViewTarget _returnvalue_2))
  (bind _returnvalue_4 (Transformation|GetActorLocation _returnvalue_3))
  (bind _returnvalue_5 (- _returnvalue _returnvalue_4))
  (bind _returnvalue_6 (Math|Vector|MakeVector (.x _returnvalue_5) (.y _returnvalue_5) 0.0))
  (if (Variables|Default|GetShouldTick)
    (Utilities|IsValid _returnvalue_3
      (:Is%20Valid
        (bind _asbp_phase_one_camera_object (Utilities|Casting|CastToBP_PhaseOneCameraObject _returnvalue_3))
        (if (> (Math|Vector|VectorLength _returnvalue_6) (Variables|/Game/Racketeers/Blueprints/Actors/BP_PhaseOneCameraObject.BP_PhaseOneCameraObject_C|GetMaxDistanceForPlayers _asbp_phase_one_camera_object))
          (Development|PrintString (Utilities|String|ToString(Vector) (Math|Vector|MakeVector (.x (* (Math|Vector|Normalize _returnvalue_6) (Variables|/Game/Racketeers/Blueprints/Actors/BP_PhaseOneCameraObject.BP_PhaseOneCameraObject_C|GetMaxDistanceForPlayers _asbp_phase_one_camera_object))) (.y (* (Math|Vector|Normalize _returnvalue_6) (Variables|/Game/Racketeers/Blueprints/Actors/BP_PhaseOneCameraObject.BP_PhaseOneCameraObject_C|GetMaxDistanceForPlayers _asbp_phase_one_camera_object))) (.z (Transformation|GetActorLocation (Variables|Default|GetOwner))))))
          (else
            (Development|PrintString (Utilities|String|ToString(Vector) (Math|Vector|MakeVector (.x (* (Math|Vector|Normalize _returnvalue_6) (Variables|/Game/Racketeers/Blueprints/Actors/BP_PhaseOneCameraObject.BP_PhaseOneCameraObject_C|GetMaxDistanceForPlayers _asbp_phase_one_camera_object))) (.y (* (Math|Vector|Normalize _returnvalue_6) (Variables|/Game/Racketeers/Blueprints/Actors/BP_PhaseOneCameraObject.BP_PhaseOneCameraObject_C|GetMaxDistanceForPlayers _asbp_phase_one_camera_object))) (.z (* (Math|Vector|Normalize _returnvalue_6) (Variables|/Game/Racketeers/Blueprints/Actors/BP_PhaseOneCameraObject.BP_PhaseOneCameraObject_C|GetMaxDistanceForPlayers _asbp_phase_one_camera_object))))))))))))