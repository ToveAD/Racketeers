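; Player component for BP_Player that provides Scurry, a timed speed boost with a sound, followed by a cooldown.
; StartScurry multiplies walk speed and StopScurry divides it back, applying the change locally and sending it to the server from non-authority clients.
; The scurrying flag propagates through server and multicast toggle events.
; OnCollision stuns the player by briefly disabling input and launching them away from the hit actor via the server.
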(event Custom|StartScurry
  (bind _owner (Variables|Default|GetOwner))
  (bind _charactermovement (Variables|/Script/Engine.Character|GetCharacterMovement _owner))
  ;[1 1 1] Starts Scurry Logic, Stops after certain time
  (if (and (not (Variables|Default|GetIsScurrying)) (not (Variables|Default|GetIsOnCooldown)))
    (CallFunction|SRToggleScurry true)
    (Networking|SwitchHasAuthority
      (:Authority
        _)
      (:Remote
        (CallFunction|ServerSetSpeed (* (Variables|/Script/Engine.CharacterMovementComponent|GetMaxWalkSpeed _charactermovement) (Variables|Default|GetSpeedMultiplier)) _charactermovement)))
    (Variables|/Script/Engine.CharacterMovementComponent|SetMaxWalkSpeed _charactermovement (* (Variables|/Script/Engine.CharacterMovementComponent|GetMaxWalkSpeed _charactermovement) (Variables|Default|GetSpeedMultiplier)))
    (bind _returnvalue (Audio|SpawnSoundatLocation "/Game/Racketeers/Audio/SFX/Player/SFX_PlayerScurry.SFX_PlayerScurry" (Transformation|GetActorLocation (Variables|Default|GetOwner)) "0, 0, 0" 1.0 1.0 0.0 0 0))
    (Variables|Default|SetScurryAudioComp _returnvalue)
    (Utilities|FlowControl|Delay (Variables|Default|GetScurryTime))
    (Development|PrintString "Stop Scurry")
    (CallFunction|StopScurry)))

(event Custom|StopScurry
  (bind _owner (Variables|Default|GetOwner))
  (bind _charactermovement (Variables|/Script/Engine.Character|GetCharacterMovement _owner))
  ;[1 1 1] Stop Scurry Logic
  (Networking|SwitchHasAuthority
    (:Authority
      _)
    (:Remote
      (CallFunction|ServerSetSpeed (/ (Variables|/Script/Engine.CharacterMovementComponent|GetMaxWalkSpeed _charactermovement) (Variables|Default|GetSpeedMultiplier)) _charactermovement)))
  (Variables|/Script/Engine.CharacterMovementComponent|SetMaxWalkSpeed _charactermovement (/ (Variables|/Script/Engine.CharacterMovementComponent|GetMaxWalkSpeed _charactermovement) (Variables|Default|GetSpeedMultiplier)))
  (CallFunction|SRToggleScurry false)
  (Variables|Default|SetIsOnCooldown true)
  (Utilities|FlowControl|Delay (Variables|Default|GetCooldown))
  (Variables|Default|SetIsOnCooldown false))

(event Custom|ToggleScurry_Event
  (params (ShouldScurry :type Boolean))
  ;[1 1 1] Server Toggle Scurry Events
  (Variables|Default|SetIsScurrying ShouldScurry))

(event Custom|SR_ToggleScurry
  (params (ShouldScurry :type Boolean))
  ;[1 1 1] Server Toggle Scurry Events
  (CallFunction|MCToggleScurry ShouldScurry))

(event Custom|Server_SetSpeed
  (params (NewSpeed :type Float%20%28double-precision%29) (Instigator :type Character%20Movement%20Component%20Object%20Reference))
  (Variables|/Script/Engine.CharacterMovementComponent|SetMaxWalkSpeed Instigator NewSpeed))

(event Custom|MC_ToggleScurry
  (params (ShouldScurry :type Boolean))
  ;[1 1 1] Server Toggle Scurry Events
  (CallFunction|ToggleScurryEvent ShouldScurry))

(event Custom|OnCollision
  (params (Hit :type Actor%20Object%20Reference))
  ;[1 1 1] Collision event to stun character
  (Input|DisableInput (Variables|Default|GetOwner) (Game|GetPlayerController 0))
  (CallFunction|ServerLaunchCharacter (* (Math|Vector|Normalize (- (Transformation|GetActorLocation (Variables|Default|GetOwner)) (Transformation|GetActorLocation Hit))) 5e+02))
  (Utilities|FlowControl|Delay (Variables|Default|GetStunDuration))
  (Input|EnableInput (Variables|Default|GetOwner) (Game|GetPlayerController 0)))

(event Custom|Server_LaunchCharacter
  (params (Velocity :type Vector))
  ;[1 1 1] Launch Character
  (Character|LaunchCharacter (Variables|Default|GetOwner) Velocity true false))

(event EventBeginPlay
  ;[1 1 1] Set Owner
  (bind _asbp_player (Utilities|Casting|CastToBP_Player (Components|GetOwner)))
  (Variables|Default|SetOwner _asbp_player))