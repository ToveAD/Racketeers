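; BP_PusherComponent lets its owner shove a BP_Player in front of it.
; Push sphere-traces forward, then stuns the hit player, makes them throw any held resource upward and launches them away along the owner's facing.
; It spawns a shove effect near the victim through MC-prefixed events.
; A DoOnce gate resets after the push cooldown, but only when the player cast succeeds.
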(event Custom|Push
  (bind _returnvalue (Components|GetOwner))
  (bind _returnvalue_2 (Components|GetOwner))
  (bind _returnvalue_3 (Transformation|GetActorLocation _returnvalue))
  (bind _returnvalue_4 (Transformation|GetActorLocation _returnvalue_2))
  (bind _returnvalue_5 (Transformation|GetActorForwardVector _returnvalue))
  (bind _returnvalue_6 (* _returnvalue_5 1.5e+03))
  (bind (_outhit _returnvalue_7) (Collision|SphereTraceForObjects _returnvalue_4 (+ _returnvalue_4 (* (Transformation|GetActorForwardVector _returnvalue_2) 1.2e+02)) 135.0 (Utilities|Array|MakeArray "ObjectTypeQuery8" "ObjectTypeQuery7") false 0 "None" true "(R=1.000000,G=0.000000,B=0.000000,A=1.000000)" "(R=0.000000,G=1.000000,B=0.000000,A=1.000000)" 1.0))
  (if _returnvalue_7
    (Utilities|FlowControl|DoOnce false :!label _label
      (:Completed
        (bind _asbp_player (Utilities|Casting|CastToBP_Player (.HitActor (Collision|BreakHitResult _outhit))))
        (Default|PushStun _asbp_player)
        (if (> (.amount (Variables|/Game/Racketeers/Core/BP_Player.BP_Player_C|GetHoldingResourceInfo _asbp_player)) 0)
          (Default|ServerThrow _asbp_player _asbp_player 0.0 true))
        (Character|LaunchCharacter _asbp_player (Math|Vector|MakeVector (.x _returnvalue_6) (.y _returnvalue_6) 4e+02) true true)
        (CallFunction|MCSpawnEffect (- _returnvalue_3 (* (Math|Vector|Normalize (- _returnvalue_3 (Transformation|GetActorLocation _asbp_player))) (- (Math|Vector|Distance(Vector) _returnvalue_3 (Transformation|GetActorLocation _asbp_player)) 5e+01))))
        (Utilities|FlowControl|Delay (Variables|Default|GetPushCooldown))
        (goto _label Reset)))))

(event Custom|MC_Spawn_Effect
  (params (LaunchedCharacter :type Vector))
  (CallFunction|SpawnEffect LaunchedCharacter))

(event Custom|Spawn_Effect
  (params (LaunchedCharacter :type Vector))
  (Niagara|SpawnSystematLocation "/Game/Racketeers/Art/Niagara/Player/FXS_Shove.FXS_Shove" LaunchedCharacter))

(event Custom|MC_ThrowItem
  (params (Player :type BP%20Player%20Object%20Reference))
  (CallFunction|ThrowItemEvent Player))

(event Custom|ThrowItem_Event
  (params (Player :type BP%20Player%20Object%20Reference))
  (Default|ThrowResource Player true 0 0.0))