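; Custom PCG Blueprint node that spawns Barrel actors at generated points for the Racketeers islands.
; It converts the first input's spatial data to point data and runs a point loop over it.
; Each loop iteration spawns a barrel slightly above the point, keeping its rotation, and returns false so no point is kept.
; The node works purely by side effect, as its output collection is left unconnected.
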(fn ExecutewithContext
  (params (InContext :type PCG%20Context%20Structure%20%28by%20ref%29) (Input :type PCG%20Data%20Collection%20Structure%20%28by%20ref%29))
  (bind _returnvalue (Class|PCGDataFunctionLibrary|GetInputs Input))
  (bind _aspcgspatial_data (Utilities|Casting|CastToPCGSpatialData (.Data (Utilities|Struct|BreakPCGTaggedData (Utilities|Array|Get(acopy) _returnvalue))))
    (:then
      (bind _outdata (PCG|FlowControl|PointLoop InContext (SpatialData|ToPointDatawithContext _aspcgspatial_data InContext) 0)))
    (:CastFailed
      (return ""))))

(fn PointLoopBody
  (params (InContext :type PCG%20Context%20Structure%20%28by%20ref%29) (InData :type PCG%20Point%20Data%20Object%20Reference) (InPoint :type PCG%20Point%20Structure%20%28by%20ref%29) (OutMetadata :type PCG%20Metadata%20Object%20Reference) (Iteration :type Integer64))
  (Game|SpawnActorfromClass (Variables|Default|GetBarrel) (Math|Transform|MakeTransform (+ (.location (.transform InPoint)) "0.000000,0.000000,50.000000") (.rotation (.transform InPoint)) "1.000000,1.000000,1.000000") "Undefined" "MultiplyWithRoot" 0 0)
  (return (Utilities|Struct|MakePCGPoint (Math|Transform|MakeTransform (.location (.transform InPoint)) (.rotation (.transform InPoint)) (.scale (.transform InPoint))) (.density InPoint) (.boundsmin InPoint) (.boundsmax InPoint) (.color InPoint) (.steepness InPoint) (.seed InPoint)) false))