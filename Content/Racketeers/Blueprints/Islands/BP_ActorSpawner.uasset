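; Custom PCG Blueprint element that scatters rock, bush and tree resource actors across an island.
; PointLoopBody gathers input point transforms, then the server spawns each actor at a randomly picked one, removing it to avoid reuse and recording it per type.
; GenerateResources sets the counts by randomly splitting the island tier's TierValue total between the three types, with one tier yielding none.
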(fn ExecutewithContext
  (params (InContext :type PCG%20Context%20Structure%20%28by%20ref%29) (Input :type PCG%20Data%20Collection%20Structure%20%28by%20ref%29))
  (bind _pointlocations (Variables|Default|GetPointLocations))
  (bind _pointlocations_2 (Variables|Default|GetPointLocations))
  (bind _pointlocations_3 (Variables|Default|GetPointLocations))
  ;[1 1 1] Gets all points
  (bind _returnvalue (Class|PCGDataFunctionLibrary|GetInputs Input))
  (bind _aspcgspatial_data (Utilities|Casting|CastToPCGSpatialData (.Data (Utilities|Struct|BreakPCGTaggedData (Utilities|Array|Get(acopy) _returnvalue))))
    (:then
      ;[1 1 1] Calls PointLoopBody Function
      (bind _outdata (PCG|FlowControl|PointLoop InContext (SpatialData|ToPointDatawithContext _aspcgspatial_data InContext) 0))
      (if (Networking|IsServer)
        (Development|PrintString (Utilities|String|EnumtoString (Variables|Default|GetIslandEnumTier)))
        (bind (_trees _bushes _rocks) (CallFunction|GenerateResources (Variables|Default|GetIslandEnumTier)))
        (for _index (range 1 _rocks)
          (bind _output_get (LocalVariables|SetCurrentTransform (Utilities|Array|Get(acopy) _pointlocations_2 (Math|Random|RandomIntegerinRange 0 (- (Utilities|Array|Length _pointlocations_2) 1)))))
          (Game|SpawnActorfromClass "/Game/Developers/fape6979/Gatherables/BP_Rock.BP_Rock_C" _output_get "AlwaysSpawn" "MultiplyWithRoot" 0 0)
          (Utilities|Array|AddUnique (Variables|Default|GetRockTransforms) (LocalVariables|GetCurrentTransform))
          (Utilities|Array|RemoveItem (Variables|Default|GetPointLocations) (LocalVariables|GetCurrentTransform)))
        (for _index_2 (range 1 _bushes)
          (bind _output_get_2 (LocalVariables|SetCurrentTransform (Utilities|Array|Get(acopy) _pointlocations_3 (Math|Random|RandomIntegerinRange 0 (- (Utilities|Array|Length _pointlocations_3) 1)))))
          (Game|SpawnActorfromClass "/Game/Developers/fape6979/Gatherables/BP_Bush.BP_Bush_C" _output_get_2 "AlwaysSpawn" "MultiplyWithRoot" 0 0)
          (Utilities|Array|AddUnique (Variables|Default|GetBushTransforms) (LocalVariables|GetCurrentTransform))
          (Utilities|Array|RemoveItem (Variables|Default|GetPointLocations) (LocalVariables|GetCurrentTransform)))
        (for _index_3 (range 1 _trees)
          (bind _output_get_3 (LocalVariables|SetCurrentTransform (Utilities|Array|Get(acopy) _pointlocations (Math|Random|RandomIntegerinRange 0 (- (Utilities|Array|Length _pointlocations) 1)))))
          (Game|SpawnActorfromClass "/Game/Developers/fape6979/Gatherables/BP_Tree.BP_Tree_C" _output_get_3 "AlwaysSpawn" "MultiplyWithRoot" 0 0)
          (Utilities|Array|AddUnique (Variables|Default|GetTreeTransforms) (LocalVariables|GetCurrentTransform))
          (Utilities|Array|RemoveItem (Variables|Default|GetPointLocations) (LocalVariables|GetCurrentTransform)))
        (return "")))
    (:CastFailed
      (return (Utilities|Struct|MakePCGDataCollection 0 false)))))

(fn PointLoopBody
  (params (InContext :type PCG%20Context%20Structure%20%28by%20ref%29) (InData :type PCG%20Point%20Data%20Object%20Reference) (InPoint :type PCG%20Point%20Structure%20%28by%20ref%29) (OutMetadata :type PCG%20Metadata%20Object%20Reference) (Iteration :type Integer64))
  (Utilities|Array|AddUnique (Variables|Default|GetPointLocations) (.transform InPoint))
  (return (Utilities|Struct|MakePCGPoint (.transform InPoint) (.density InPoint) (.boundsmin InPoint) (.boundsmax InPoint) (.color InPoint) (.steepness InPoint) (.seed InPoint)) false))

(fn GenerateResources
  (params (IslandTier :type ETier%20Enum :default "NewEnumerator3"))
  (bind _tiervalue (LocalVariables|GetTierValue))
  (bind _value (Utilities|Map|Find _tiervalue IslandTier))
  (if (Utilities|Enum|Equal(Enum) IslandTier "NewEnumerator3")
    (return 0 0 0)
    (else
      (bind _output_get (LocalVariables|SetRemainingRatio (- (LocalVariables|GetRemainingRatio) 0.6)))
      (LocalVariables|SetTreeRatio (+ (LocalVariables|GetTreeRatio) (Math|Random|RandomFloatinRange 0.0 _output_get)))
      (bind _output_get_2 (LocalVariables|SetRemainingRatio (- (LocalVariables|GetRemainingRatio) (Math|Random|RandomFloatinRange 0.0 _output_get))))
      (LocalVariables|SetBushRatio (+ (LocalVariables|GetBushRatio) (Math|Random|RandomFloatinRange 0.0 _output_get_2)))
      (bind _output_get_3 (LocalVariables|SetRemainingRatio (- (LocalVariables|GetRemainingRatio) (Math|Random|RandomFloatinRange 0.0 _output_get_2))))
      (LocalVariables|SetRockRatio (+ (LocalVariables|GetRockRatio) _output_get_3))
      (Development|PrintString (Utilities|String|Append "Rock ratio: " (Utilities|String|ToString(Float) (LocalVariables|GetRockRatio)) "||" "Bush ratio: " (Utilities|String|ToString(Float) (LocalVariables|GetBushRatio)) "||" "Tree ratio: " (Utilities|String|ToString(Float) (LocalVariables|GetTreeRatio))))
      (bind _output_get_4 (LocalVariables|SetRockAmount (Math|Float|Round (* _value (LocalVariables|GetRockRatio)))))
      (bind _output_get_5 (LocalVariables|SetBushAmount (Math|Float|Round (* _value (LocalVariables|GetBushRatio)))))
      (bind _output_get_6 (LocalVariables|SetTreeAmount (Math|Float|Round (* _value (LocalVariables|GetTreeRatio)))))
      (return _output_get_6 _output_get_5 _output_get_4))))