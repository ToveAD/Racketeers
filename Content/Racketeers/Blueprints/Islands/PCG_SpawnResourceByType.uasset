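; Custom PCG Blueprint element that spawns harvestable resource actors on generated points, chosen by its Type setting.
; It iterates the point data on the In pin and spawns a tree, bush or rock Blueprint actor at each point's transform for wood, fiber or metal, printing a warning for no type.
; After the loops, it forwards the last point data, unmodified, to OutPoints.
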(fn ExecutewithContext
  (params (InContext :type PCG%20Context%20Structure%20%28by%20ref%29) (Input :type PCG%20Data%20Collection%20Structure%20%28by%20ref%29))
  (bind _returnvalue (Data|GetTypedInputsbyPinLabel Input "In" "/Script/PCG.PCGPointData"))
  (for _array_element _returnvalue
    (bind _output_get (LocalVariables|SetInPointData _array_element))
    (bind _output_get_2 (LocalVariables|SetInPoints (SpatialData|GetPoints _output_get)))
    (for _array_element_2 _output_get_2
      (LocalVariables|SetCurrentPoint _array_element_2)
      (switch Utilities|FlowControl|Switch|SwitchonEResources (Variables|Default|GetType)
        (:WOOD
          (Game|SpawnActorfromClass "/Game/Racketeers/Blueprints/GatherableItems/GatherableResource/BP_Tree.BP_Tree_C" (.Transform (Utilities|Struct|BreakPCGPoint (LocalVariables|GetCurrentPoint))) "Undefined" "MultiplyWithRoot" 0 0))
        (:FIBER
          (Game|SpawnActorfromClass "/Game/Racketeers/Blueprints/GatherableItems/GatherableResource/BP_Bush.BP_Bush_C" (.Transform (Utilities|Struct|BreakPCGPoint (LocalVariables|GetCurrentPoint))) "Undefined" "MultiplyWithRoot" 0 0))
        (:METAL
          (Game|SpawnActorfromClass "/Game/Racketeers/Blueprints/GatherableItems/GatherableResource/BP_Rock.BP_Rock_C" (.Transform (Utilities|Struct|BreakPCGPoint (LocalVariables|GetCurrentPoint))) "Undefined" "MultiplyWithRoot" 0 0))
        (:NONE
          (Development|PrintString "No type Selected")))))
  (Class|PCGDataFunctionLibrary|AddtoCollection (LocalVariables|GetOutputCollection) (LocalVariables|GetInPointData) "OutPoints" (Utilities|Array|MakeArray ""))
  (return (LocalVariables|GetOutputCollection)))