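; BP_Island is an island actor that generates tiered resources through a PCG component.
; The construction script stores the island mesh's world location in Point and passes its Tier to the PCG graph as an enum parameter.
; GenerateResources forces PCG generation on the server only and prints a debug message.
; Nothing in this Blueprint's active event logic calls GenerateResources, as its authority-switch call is disconnected.
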(event EventBeginPlay)

(event Collision|EventActorBeginOverlap
  (params (OtherActor :type Actor%20Object%20Reference)))

(event EventTick
  (params (DeltaSeconds :type Float%20%28single-precision%29)))

(fn ConstructionScript
  (Variables|Default|SetPoint (Transformation|GetWorldLocation (Variables|Default|GetIsland)))
  (Class|PCGGraphParametersHelpers|SetEnumParameter (Variables|/Script/PCG.PCGComponent|GetGraphInstance (Variables|Default|GetPCG)) "ISlandTier" (Variables|Default|GetTier) "/Game/Racketeers/Blueprints/Islands/ETier.ETier"))

(fn GenerateResources
  (if (Networking|IsServer)
    (PCG|Generate (Variables|Default|GetPCG) true)
    (Development|PrintString "Resources generated" true true "(R=0.000000,G=0.660000,B=1.000000,A=1.000000)" 5e+01)))