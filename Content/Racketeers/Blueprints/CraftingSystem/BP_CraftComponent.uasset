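; BP_CraftComponent is a player component that relays crafting interactions and manages the resource the player holds.
; OnInteract goes through a server event into a multicast, which messages every overlapping BP_CraftingBaseClass actor with the team and the player.
; Helper functions check and clear the player's HoldingResourceInfo, while GiveResrouces only writes a fixed wood entry with zero amount and prints it.
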(event Custom|On%20Interact
  (params (Team :type ETeams%20Enum :default "Team_Raccoon"))
  (Networking|SwitchHasAuthority
    (:Authority
      _)
    (:Remote
      _))
  (CallFunction|SRonInteract Team))

(event Custom|SR_On%20Interact
  (params (Team :type ETeams%20Enum :default "Team_Raccoon"))
  (CallFunction|MConInteract Team))

(event Custom|MC_On%20Interact
  (params (Team :type ETeams%20Enum :default "Team_Raccoon"))
  (CallFunction|OnInteractEvent Team))

(event Custom|OnInteract_Event
  (params (Team :type ETeams%20Enum :default "Team_Raccoon"))
  (for _array_element (Collision|GetOverlappingActors (Components|GetOwner) "/Game/Racketeers/Blueprints/CraftingSystem/BP_CraftingBaseClass.BP_CraftingBaseClass_C" :!class /Script/Engine.Actor)
    (bind _asbp_player (Utilities|Casting|CastToBP_Player (Components|GetOwner)))
    (Class|BPICrafting|OnInteract(Message) _array_element Team _asbp_player)))

(event EventTick
  (params (DeltaSeconds :type Float%20%28single-precision%29)))

(fn GiveResrouces
  (params (NewResource :type BP%20Player%20Object%20Reference))
  (bind _output_get (Variables|/Game/Racketeers/Core/BP_Player.BP_Player_C|SetHoldingResourceInfo NewResource (Utilities|Struct|MakeFCraftableResource "WOOD" 0)))
  (Development|PrintString (Utilities|String|Append (Utilities|GetDisplayName (Components|GetOwner)) " Picked up " (Utilities|String|EnumtoString (.resource _output_get)) ", " (Utilities|String|ToString(Integer) (.amount _output_get)))))

(fn HasResources
  (bind _asbp_player (Utilities|Casting|CastToBP_Player (Components|GetOwner)))
  (return (!= (.amount (Variables|/Game/Racketeers/Core/BP_Player.BP_Player_C|GetHoldingResourceInfo _asbp_player)) 0)))

(fn ClearResources
  (params (instigator :type BP%20Player%20Object%20Reference))
  (Variables|/Game/Racketeers/Core/BP_Player.BP_Player_C|SetHoldingResourceInfo instigator (Utilities|Struct|MakeFCraftableResource "NONE" 0))
  (Development|PrintString "Removed player item"))