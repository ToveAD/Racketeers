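; Material crate that hands players one unit of its wood, metal or fiber type from their team's stock in the GameState.
; On interact, any held resources return to the team pool, then the crate dispenses from stock or, if empty, attempts a scavenge.
; Scavenging odds rise with each failure, comparing a progress counter against a 1-100 GameState roll, refreshed through server and multicast events.
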(event Custom|GenerateRandomNumber
  (params (NewParam :type Integer))
  (bind _asracketeers_game_state_base (Utilities|Casting|CastToRacketeersGameStateBase (Game|GetGameState)))
  (Class|RacketeersGameStateBase|SetRandomNumber _asracketeers_game_state_base NewParam))

(event Custom|SR_GenerateRandomNumber
  (CallFunction|MCGenerateRandomNumber (Math|Random|RandomIntegerinRange 1 100)))

(event Custom|MC_GenerateRandomNumber
  (params (NewParam :type Integer))
  (CallFunction|GenerateRandomNumber NewParam))

(event EventBeginPlay
  (Networking|SwitchHasAuthority
    (:Authority
      (CallFunction|SRGenerateRandomNumber))))

(event EventOnInteract
  (params (Team :type ETeams%20Enum :default "Team_Racoon") (Instigator :type BP%20Craft%20Component%20Object%20Reference))
  (bind _does_have_resources (Default|HasResources Instigator))
  (if _does_have_resources
    (CallFunction|RemoveResourcesfromPlayer Instigator Team))
  (bind _hasmaterials (CallFunction|CheckTeamMaterials Team))
  (if _hasmaterials
    (CallFunction|GiveResourcestoPlayer Instigator Team :!label _label)
    (CallFunction|RemoveResource Team (Variables|Default|GetCrateType) 1)
    (else
      (bind _didgetmaterial (CallFunction|TryRandomMaterial))
      (CallFunction|SRGenerateRandomNumber)
      (if _didgetmaterial
        (CallFunction|AddResource Team (Variables|Default|GetCrateType) 1)
        (goto _label)))))

(fn ConstructionScript)

(fn TryRandomMaterial
  (Niagara|SpawnSystematLocation "/Game/Racketeers/Art/Niagara/Crafting/FXS_Scavenging.FXS_Scavenging" (+ (Transformation|GetActorLocation) "0.000000,0.000000,100.000000"))
  (bind _asracketeers_game_state_base (Utilities|Casting|CastToRacketeersGameStateBase (Game|GetGameState)))
  (Development|PrintString (Utilities|String|Append "Scavenge: " (Utilities|String|ToString(Integer) (Variables|Default|GetCurrent%20Scavenge%20Progress))))
  (if (<= (Variables|/Script/Racketeers.RacketeersGameStateBase|GetPhase2RandomNumber _asracketeers_game_state_base) (Variables|Default|GetCurrent%20Scavenge%20Progress))
    (Variables|Default|SetCurrent%20Scavenge%20Progress 1)
    (return true)
    (else
      (Math|Integer|IncrementInt (Variables|Default|GetCurrent%20Scavenge%20Progress)
        (:%20%20
          (return false))))))

(fn GiveResourcestoPlayer
  (params (PlayerCraftComponent :type BP%20Craft%20Component%20Object%20Reference) (Team :type ETeams%20Enum :default "Team_Racoon"))
  (bind _holdingresource (Variables|/Game/Racketeers/Blueprints/CraftingSystem/BP_CraftComponent.BP_CraftComponent_C|GetHoldingResource PlayerCraftComponent))
  (bind (_resource _amount) (Utilities|Struct|BreakFCraftableResource _holdingresource))
  (if (or (== _amount 0) (Utilities|Enum|NotEqual(Enum) _resource "NewEnumerator3"))
    (CallFunction|AddResource Team _resource _amount)
    (Default|GiveResrouces PlayerCraftComponent (Utilities|Struct|MakeFCraftableResource (Variables|Default|GetCrateType) 1))))

(fn RemoveResourcesfromPlayer
  (params (CraftComponent :type BP%20Craft%20Component%20Object%20Reference) (Team :type ETeams%20Enum :default "Team_Racoon"))
  (bind _holdingresource (Variables|/Game/Racketeers/Blueprints/CraftingSystem/BP_CraftComponent.BP_CraftComponent_C|GetHoldingResource CraftComponent))
  (bind (_resource _amount) (Utilities|Struct|BreakFCraftableResource _holdingresource))
  (CallFunction|AddResource Team _resource _amount)
  (Default|ClearResources CraftComponent))

(fn GiveResourcestoTeam
  (params (Team :type ETeams%20Enum :default "Team_Racoon"))
  (CallFunction|AddResource Team (Variables|Default|GetCrateType) 1))

(fn AddResource
  (params (Team :type ETeams%20Enum :default "Team_Racoon") (ResourceType :type EResourceType%20Enum :default "NewEnumerator0") (Amount :type Integer))
  (bind _asracketeers_game_state_base (Utilities|Casting|CastToRacketeersGameStateBase (Game|GetGameState)))
  (switch Utilities|FlowControl|Switch|SwitchonEResourceType ResourceType
    (:NewEnumerator0
      (Class|RacketeersGameStateBase|AddResource _asracketeers_game_state_base Amount "WOOD" Team))
    (:NewEnumerator1
      (Class|RacketeersGameStateBase|AddResource _asracketeers_game_state_base Amount "METAL" Team))
    (:NewEnumerator2
      (Class|RacketeersGameStateBase|AddResource _asracketeers_game_state_base Amount "FIBER" Team))))

(fn RemoveResource
  (params (Team :type ETeams%20Enum :default "Team_Racoon") (ResourceType :type EResourceType%20Enum :default "NewEnumerator0") (Amount :type Integer))
  (bind _asracketeers_game_state_base (Utilities|Casting|CastToRacketeersGameStateBase (Game|GetGameState)))
  (switch Utilities|FlowControl|Switch|SwitchonEResourceType ResourceType
    (:NewEnumerator0
      (Class|RacketeersGameStateBase|RemoveResource _asracketeers_game_state_base Amount "WOOD" Team))
    (:NewEnumerator1
      (Class|RacketeersGameStateBase|RemoveResource _asracketeers_game_state_base Amount "METAL" Team))
    (:NewEnumerator2
      (Class|RacketeersGameStateBase|RemoveResource _asracketeers_game_state_base Amount "FIBER" Team))))

(fn CheckTeamMaterials
  (params (Team :type ETeams%20Enum :default "Team_Racoon"))
  (bind _asracketeers_game_state_base (Utilities|Casting|CastToRacketeersGameStateBase (Game|GetGameState))
    (:then
      (switch Utilities|FlowControl|Switch|SwitchonETeams Team
        (:Team_Racoon
          (switch Utilities|FlowControl|Switch|SwitchonEResourceType (Variables|Default|GetCrateType)
            (:NewEnumerator0
              (return (> (.Wood (Utilities|Struct|BreakResources (Variables|/Script/Racketeers.RacketeersGameStateBase|GetRacconResource _asracketeers_game_state_base))) 0)))
            (:NewEnumerator1
              (return (> (.Metal (Utilities|Struct|BreakResources (Variables|/Script/Racketeers.RacketeersGameStateBase|GetRacconResource _asracketeers_game_state_base))) 0)))
            (:NewEnumerator2
              (return (> (.Fiber (Utilities|Struct|BreakResources (Variables|/Script/Racketeers.RacketeersGameStateBase|GetRacconResource _asracketeers_game_state_base))) 0)))))
        (:Team_Panda
          (switch Utilities|FlowControl|Switch|SwitchonEResourceType (Variables|Default|GetCrateType)
            (:NewEnumerator0
              (return (> (.Wood (Utilities|Struct|BreakResources (Variables|/Script/Racketeers.RacketeersGameStateBase|GetRedPandasResource _asracketeers_game_state_base))) 0)))
            (:NewEnumerator1
              (return (> (.Metal (Utilities|Struct|BreakResources (Variables|/Script/Racketeers.RacketeersGameStateBase|GetRedPandasResource _asracketeers_game_state_base))) 0)))
            (:NewEnumerator2
              (return (> (.Fiber (Utilities|Struct|BreakResources (Variables|/Script/Racketeers.RacketeersGameStateBase|GetRedPandasResource _asracketeers_game_state_base))) 0)))))))
    (:CastFailed
      (return false))))