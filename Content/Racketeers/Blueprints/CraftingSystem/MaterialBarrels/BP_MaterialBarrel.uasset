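; Interactable material barrel that hands players one unit of its wood, fiber or metal type from their team's stock in the game state.
; Interacting fills the player's held resource, sets its mesh and blocks throw charging.
; With empty stock, it scavenges: a shared random number is tested against a progress counter that rises per failure and resets on success.
; The number rerolls on BeginPlay and after each attempt through server and multicast events.
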(event Custom|GenerateRandomNumber
  (params (NewParam :type Integer))
  (bind _asracketeers_game_state_base (Utilities|Casting|CastToRacketeersGameStateBase (Game|GetGameState)))
  (Class|RacketeersGameStateBase|SetRandomNumber _asracketeers_game_state_base NewParam))

(event Custom|SR_GenerateRandomNumber
  (CallFunction|MCGenerateRandomNumber (Math|Random|RandomIntegerinRange 1 100)))

(event Custom|MC_GenerateRandomNumber
  (params (NewParam :type Integer))
  (CallFunction|GenerateRandomNumber NewParam))

(event Custom|OnInteract_1
  (params (Team :type ETeams%20Enum :default "Team_Raccoon") (Instigator :type BP%20Player%20Object%20Reference)))

(event EventBeginPlay
  (Networking|SwitchHasAuthority
    (:Authority
      (CallFunction|SRGenerateRandomNumber))))

(event EventStartInteract
  (params (Instigator :type Actor%20Object%20Reference) (bIsServer :type Boolean))
  (bind _asbp_player (Utilities|Casting|CastToBP_Player Instigator))
  (bind _asbp_player_state (Utilities|Casting|CastToBP_PlayerState (Variables|/Script/Engine.Pawn|GetPlayerState _asbp_player)))
  (Development|PrintString (Utilities|String|Append "Team: " (Utilities|String|EnumtoString (.team (Variables|/Script/Racketeers.PS_Base|GetPlayerInfo _asbp_player_state)))))
  ;[1 1 1] Checks if the team has materials of the barrels resource type
  (bind _hasmaterials (CallFunction|CheckTeamMaterials (.team (Variables|/Script/Racketeers.PS_Base|GetPlayerInfo _asbp_player_state))))
  (if _hasmaterials
    ;[1 1 1] Give player a resource
    (Variables|/Game/Racketeers/Core/BP_Player.BP_Player_C|SetHoldingResourceInfo _asbp_player (Utilities|Struct|MakeFCraftableResource (Variables|Default|GetCrateType) 1) :!label _label)
    ;[1 1 1] Removes resource from team resource deposit
    (Development|PrintString (Utilities|String|EnumtoString (.team (Variables|/Script/Racketeers.PS_Base|GetPlayerInfo _asbp_player_state))))
    (CallFunction|RemoveResource (.team (Variables|/Script/Racketeers.PS_Base|GetPlayerInfo _asbp_player_state)) (Variables|Default|GetCrateType) 1)
    ;[1 1 1] Set a mesh to represent the holding resource
    (switch Utilities|FlowControl|Switch|SwitchonEResources (Variables|Default|GetCrateType)
      (:WOOD
        (Components|StaticMesh|SetStaticMesh (Variables|/Game/Racketeers/Core/BP_Player.BP_Player_C|GetHoldingObject _asbp_player) "/Game/Racketeers/Art/Meshes/Whitebox_V1/SM_WoodResource.SM_WoodResource"))
      (:FIBER
        (Components|StaticMesh|SetStaticMesh (Variables|/Game/Racketeers/Core/BP_Player.BP_Player_C|GetHoldingObject _asbp_player) "/Game/Racketeers/Art/Meshes/Whitebox_V1/SM_FiberResource.SM_FiberResource"))
      (:METAL
        (Components|StaticMesh|SetStaticMesh (Variables|/Game/Racketeers/Core/BP_Player.BP_Player_C|GetHoldingObject _asbp_player) "/Game/Racketeers/Art/Meshes/Whitebox_V1/SM_OreResource.SM_OreResource")))
    ;[1 1 1] this ensures the player dont throws the resource direct after recieving it
    (Variables|/Game/Racketeers/Core/BP_Player.BP_Player_C|SetCanChargeThrow _asbp_player false)
    (Variables|/Game/Racketeers/Core/BP_Player.BP_Player_C|SetIsHoldingResource _asbp_player true)
    (else
      ;[1 1 1] Scavenge Stuff
      (bind _didgetmaterial (CallFunction|TryRandomMaterial))
      (CallFunction|SRGenerateRandomNumber)
      (if _didgetmaterial
        (CallFunction|AddResource (.team (Variables|/Script/Racketeers.PS_Base|GetPlayerInfo _asbp_player_state)) (Variables|Default|GetCrateType) 1)
        (goto _label)))))

(fn ConstructionScript)

(fn TryRandomMaterial
  (Niagara|SpawnSystematLocation "/Game/Racketeers/Art/Niagara/Crafting/FXS_Scavenging.FXS_Scavenging" (+ (Transformation|GetActorLocation) "0.000000,0.000000,100.000000"))
  (bind _asracketeers_game_state_base (Utilities|Casting|CastToRacketeersGameStateBase (Game|GetGameState)))
  (Development|PrintString (Utilities|String|Append "Scavenge: " (Utilities|String|ToString(Integer) (Variables|Default|GetCurrent%20Scavenge%20Progress))))
  (if (<= (Variables|/Script/Racketeers.RacketeersGameStateBase|GetPhase2RandomNumber _asracketeers_game_state_base) (Variables|Default|GetCurrent%20Scavenge%20Progress))
    (Variables|Default|SetCurrent%20Scavenge%20Progress 1)
    (return true)
    (else
      (Math|Integer|IncrementInt (Variables|Default|GetCurrent%20Scavenge%20Progress)
        (:%20%20
          (return false))))))

(fn GiveResourcestoPlayer
  (params (PlayerCraftComponent :type BP%20Craft%20Component%20Object%20Reference) (Team :type ETeams%20Enum :default "Team_Raccoon") (instigator :type BP%20Player%20Object%20Reference))
  (bind _holdingresourceinfo (Variables|/Game/Racketeers/Core/BP_Player.BP_Player_C|GetHoldingResourceInfo instigator))
  ;[1 1 1] Explain plz
  (if (== (.amount _holdingresourceinfo) 0)
    (CallFunction|AddResource "Team_Raccoon" (.resource _holdingresourceinfo) (.amount _holdingresourceinfo))
    (Default|GiveResrouces (Variables|/Game/Racketeers/Core/BP_Player.BP_Player_C|GetBP_CraftComponent instigator) instigator)))

(fn RemoveResourcesfromPlayer
  (params (CraftComponent :type BP%20Craft%20Component%20Object%20Reference) (Team :type ETeams%20Enum :default "Team_Raccoon") (Instigator :type BP%20Player%20Object%20Reference))
  ;[1 1 1] Adds the current holding resource of the player to the teams resource account
  (CallFunction|AddResource Team (.Resource (Utilities|Struct|BreakFCraftableResource (Variables|/Game/Racketeers/Core/BP_Player.BP_Player_C|GetHoldingResourceInfo Instigator))) (.Amount (Utilities|Struct|BreakFCraftableResource (Variables|/Game/Racketeers/Core/BP_Player.BP_Player_C|GetHoldingResourceInfo Instigator))))
  ;[1 1 1] Removes the current resource the player is holding
  (Variables|/Game/Racketeers/Core/BP_Player.BP_Player_C|SetHoldingResourceInfo Instigator (Utilities|Struct|MakeFCraftableResource "NONE" 0)))

(fn GiveResourcestoTeam
  (params (Team :type ETeams%20Enum :default "Team_Raccoon"))
  (CallFunction|AddResource Team (Variables|Default|GetCrateType) 1))

(fn AddResource
  (params (Team :type ETeams%20Enum :default "Team_Raccoon") (ResourceType :type EResources%20Enum :default "WOOD") (Amount :type Integer))
  (bind _asracketeers_game_state_base (Utilities|Casting|CastToRacketeersGameStateBase (Game|GetGameState)))
  (Class|RacketeersGameStateBase|AddResource _asracketeers_game_state_base Amount ResourceType Team))

(fn RemoveResource
  (params (Team :type ETeams%20Enum :default "Team_Raccoon") (ResourceType :type EResources%20Enum :default "WOOD") (Amount :type Integer))
  (bind _asracketeers_game_state_base (Utilities|Casting|CastToRacketeersGameStateBase (Game|GetGameState)))
  (Class|RacketeersGameStateBase|RemoveResource _asracketeers_game_state_base Amount ResourceType Team))

(fn CheckTeamMaterials
  (params (Team :type ETeams%20Enum :default "Team_Raccoon"))
  (bind _asracketeers_game_state_base (Utilities|Casting|CastToRacketeersGameStateBase (Game|GetGameState))
    (:then
      (switch Utilities|FlowControl|Switch|SwitchonETeams Team
        (:Team_Raccoon
          (switch Utilities|FlowControl|Switch|SwitchonEResources (Variables|Default|GetCrateType)
            (:WOOD
              (Development|PrintString "Raccoon")
              (return (> (.Wood (Utilities|Struct|BreakResources (Variables|/Script/Racketeers.RacketeersGameStateBase|GetRacconResource _asracketeers_game_state_base))) 0)))
            (:FIBER
              (return (> (.Fiber (Utilities|Struct|BreakResources (Variables|/Script/Racketeers.RacketeersGameStateBase|GetRacconResource _asracketeers_game_state_base))) 0)))
            (:METAL
              (return (> (.Metal (Utilities|Struct|BreakResources (Variables|/Script/Racketeers.RacketeersGameStateBase|GetRacconResource _asracketeers_game_state_base))) 0)))))
        (:Team_Panda
          (switch Utilities|FlowControl|Switch|SwitchonEResources (Variables|Default|GetCrateType)
            (:WOOD
              (Development|PrintString (Utilities|String|ToString(Integer) (.Wood (Utilities|Struct|BreakResources (Variables|/Script/Racketeers.RacketeersGameStateBase|GetRedPandasResource _asracketeers_game_state_base)))))
              (return (> (.Wood (Utilities|Struct|BreakResources (Variables|/Script/Racketeers.RacketeersGameStateBase|GetRedPandasResource _asracketeers_game_state_base))) 0)))
            (:FIBER
              (Development|PrintString (Utilities|String|ToString(Integer) (.Fiber (Utilities|Struct|BreakResources (Variables|/Script/Racketeers.RacketeersGameStateBase|GetRedPandasResource _asracketeers_game_state_base)))))
              (return (> (.Fiber (Utilities|Struct|BreakResources (Variables|/Script/Racketeers.RacketeersGameStateBase|GetRedPandasResource _asracketeers_game_state_base))) 0)))
            (:METAL
              (Development|PrintString (Utilities|String|ToString(Integer) (.Metal (Utilities|Struct|BreakResources (Variables|/Script/Racketeers.RacketeersGameStateBase|GetRedPandasResource _asracketeers_game_state_base)))))
              (return (> (.Metal (Utilities|Struct|BreakResources (Variables|/Script/Racketeers.RacketeersGameStateBase|GetRedPandasResource _asracketeers_game_state_base))) 0)))))))
    (:CastFailed
      (return false))))

(fn CanInteract
  (return true))