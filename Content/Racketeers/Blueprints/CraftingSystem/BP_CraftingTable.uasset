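; BP_CraftingTable is a work-in-progress crafting bench that stores resource counts and checks whether an item can be crafted.
; AddResource accumulates amounts in a map keyed by resource type, with debug prints.
; OnInteract checks the hard-coded HullUpgrade_1 row in DT_CraftableItem against bench type and stock, but returns after the first resource.
; CraftItem is an empty stub, and a failed check just adds zero of a resource.
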(event EventBeginPlay)

(event Collision|EventActorBeginOverlap
  (params (OtherActor :type Actor%20Object%20Reference)))

(event EventTick
  (params (DeltaSeconds :type Float%20%28single-precision%29)))

(fn ConstructionScript)

(fn AddResource
  (params (Resource%20Type :type EResourceType%20Enum :default "NewEnumerator0") (Amount :type Integer))
  (bind _numberofresources (Variables|Default|GetNumberOfResources))
  (bind _value (Utilities|Map|Find _numberofresources Resource%20Type))
  (bind _returnvalue (+ _value Amount))
  (if (Utilities|Map|Contains _numberofresources Resource%20Type)
    (Utilities|Map|Add (Variables|Default|GetNumberOfResources) Resource%20Type _returnvalue)
    (Development|PrintString (Utilities|String|EnumtoString Resource%20Type))
    (Development|PrintString (Utilities|String|ToString(Integer) _returnvalue))
    (else
      (Utilities|Map|Add (Variables|Default|GetNumberOfResources) Resource%20Type Amount)
      (Development|PrintString "Hello"))))

(fn CraftItem)

(fn OnInteract
  (bind _cancraft (CallFunction|CheckifCanCraft))
  (if _cancraft
    (CallFunction|CraftItem)
    (else
      (CallFunction|AddResource "NewEnumerator0"))))

(fn CheckifCanCraft
  (bind _returnvalue (Utilities|GetDataTableRow "/Game/Racketeers/Blueprints/CraftingSystem/DT_CraftableItem.DT_CraftableItem" "HullUpgrade_1")
    (:then
      (if (Utilities|Enum|Equal(Enum) (.CraftingTable (Utilities|Struct|BreakFCraftableItem _returnvalue)) (Variables|Default|GetBenchType))
        (for _array_element (.Resources (Utilities|Struct|BreakFCraftableItem _returnvalue))
          (if (and (.ReturnValue (Utilities|Map|Find (Variables|Default|GetNumberOfResources) (.Resource (Utilities|Struct|BreakFCraftableResource _array_element)))) (>= (.Value (Utilities|Map|Find (Variables|Default|GetNumberOfResources) (.Resource (Utilities|Struct|BreakFCraftableResource _array_element)))) (.Amount (Utilities|Struct|BreakFCraftableResource _array_element))))
            (Development|PrintString "Can craft!")
            (return true)
            (else
              (Development|PrintString "Not enough resources")
              (return false))))
        (else
          (Development|PrintString "Wrong Crafting bench for this item!"))))
    (:RowNotFound
      (return false))))