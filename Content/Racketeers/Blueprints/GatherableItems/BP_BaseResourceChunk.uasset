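; Base actor for gatherable resource chunks that players pick up and that can launch as projectiles.
; Interacting copies type, value and mesh to the player's held state, disables charge throw, plays a sound and destroys the chunk.
; Construction applies velocity to ProjectileMovement, OnReps update its initial and max speed, and mesh hits enable physics.
; Pickup requires passing a ground check and not being held; older hide-instead-of-destroy pickup logic remains disconnected.
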(event OnComponentHit(ResourceMesh)
  (params (HitComponent :type Primitive%20Component%20Object%20Reference) (OtherActor :type Actor%20Object%20Reference) (OtherComp :type Primitive%20Component%20Object%20Reference) (NormalImpulse :type Vector :default "0, 0, 0") (Hit :type Hit%20Result%20Structure%20%28by%20ref%29))
  ;[1 1 1] OnHit
  (Physics|SetSimulatePhysics (Variables|Default|GetResourceMesh) true))

(event OnComponentActivated(ProjectileMovement)
  (params (Component :type Actor%20Component%20Object%20Reference) (bReset :type Boolean))
  ;[1 1 1] Old
  ;;[1 1 1] ProjectileActivate
)

(event EventBeginPlay)

(event EventStartInteract
  (params (Instigator :type Actor%20Object%20Reference) (bIsServer :type Boolean))
  ;[1 1 1] Player
  (bind _asbp_player (Utilities|Casting|CastToBP_Player Instigator))
  (Variables|/Game/Racketeers/Core/BP_Player.BP_Player_C|SetIsHoldingResource _asbp_player true)
  (Variables|/Game/Racketeers/Core/BP_Player.BP_Player_C|SetHoldingResourceInfo _asbp_player (Utilities|Struct|MakeFCraftableResource (Variables|Default|Gettype) (Variables|Default|Getvalue)))
  (Variables|/Game/Racketeers/Core/BP_Player.BP_Player_C|SetCanChargeThrow _asbp_player false)
  (Components|StaticMesh|SetStaticMesh (Variables|/Game/Racketeers/Core/BP_Player.BP_Player_C|GetHoldingObject _asbp_player) (Variables|/Script/Engine.StaticMeshComponent|GetStaticMesh (Variables|Default|GetResourceMesh)))
  (Audio|PlaySoundatLocation "/Game/Racketeers/Audio/SFX/Player/SFX_PickUp.SFX_PickUp" (Transformation|GetActorLocation) "0, 0, 0" 1.0 1.0 0.0 0 0 0 0)
  (Actor|DestroyActor))

(event EventStopInteract
  (params (Instigator :type Actor%20Object%20Reference))
  (Variables|Default|SetisBeingHeld false))

(fn ConstructionScript
  (Variables|/Script/Engine.MovementComponent|SetVelocity (Variables|Default|GetProjectileMovement) (Variables|Default|Getvelocity)))

(fn CanInteract
  ;[1 1 1] Checks if player can interact with the object
  (bind _returnvalue (Class|BaseResourceChunk|GroundCheck))
  (if (and _returnvalue (not (Variables|Default|GetisBeingHeld)))
    (return true)
    (else
      (return false))))

(fn OnRepInitialSpeed
  ;[1 1 1] Lags more than setting maxspeed
  ;;[1 1 1] SetsTheInitialSpeed
  (Variables|/Script/Engine.ProjectileMovementComponent|SetInitialSpeed (Variables|Default|GetProjectileMovement) (Variables|Default|GetInitialSpeed)))

(fn OnRepMaxSpeed
  ;[1 1 1] Lags less than setting the initialspeed
  ;;[1 1 1] Sets maxSpeed
  (Variables|/Script/Engine.ProjectileMovementComponent|SetMaxSpeed (Variables|Default|GetProjectileMovement) (Variables|Default|GetMaxSpeed)))