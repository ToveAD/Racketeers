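; BP_PickUp is a floating, spinning resource pickup that players collect by touching it.
; Tick rotates it and eases it between points above and below its spawn height, lerping by DeltaSeconds and flip-flopping the target on arrival.
; When a BP_Player overlaps its sphere, it calls AddResource on that player's controller with its value, resource type and the player's team, then destroys itself.
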(event OnComponentBeginOverlap(Sphere)
  (params (OverlappedComponent :type Primitive%20Component%20Object%20Reference) (OtherActor :type Actor%20Object%20Reference) (OtherComp :type Primitive%20Component%20Object%20Reference) (OtherBodyIndex :type Integer) (bFromSweep :type Boolean) (SweepResult :type Hit%20Result%20Structure%20%28by%20ref%29))
  ;[1 1 1] Player overlap
  (bind _asbp_player (Utilities|Casting|CastToBP_Player OtherActor))
  (bind _asbp_player_state (Utilities|Casting|CastToBP_PlayerState (Variables|/Script/Engine.Pawn|GetPlayerState _asbp_player)))
  (bind _asbp_player_controller (Utilities|Casting|CastToBP_PlayerController (Game|GetPlayerController (Variables|/Script/Engine.Pawn|GetPlayerState _asbp_player))))
  (Class|RacketeersController|AddResource _asbp_player_controller (Variables|Default|GetValue) (Variables|Default|GetResourceType) (.team (Variables|/Script/Racketeers.PS_Base|GetPlayerInfo _asbp_player_state)))
  (Actor|DestroyActor))

(event EventBeginPlay
  ;[1 1 1] BeginPlay
  (bind _output_get (Variables|Default|SetSpawnLocation (Transformation|GetActorLocation)))
  (Variables|Default|SetTopLocation (Math|Vector|MakeVector (.x _output_get) (.y _output_get) (+ (.z _output_get) (Variables|Default|GetMovingZDistance))))
  (Variables|Default|SetDownLocation (Math|Vector|MakeVector (.x (Variables|Default|GetSpawnLocation)) (.y (Variables|Default|GetSpawnLocation)) (- (.z (Variables|Default|GetSpawnLocation)) (/ (Variables|Default|GetMovingZDistance) 4.0))))
  (Variables|Default|SetCurrentTargetLocation (Variables|Default|GetTopLocation)))

(event EventTick
  (params (DeltaSeconds :type Float%20%28single-precision%29))
  ;[1 1 1] Tick
  (Transformation|AddActorLocalRotation "0.000000,1.000000,0.000000" false false)
  ;;[1 1 1] LerpsActor to current targetLocation
  (Transformation|SetActorLocation (Math|Vector|Lerp(Vector) (Transformation|GetActorLocation) (Variables|Default|GetCurrentTargetLocation) DeltaSeconds) false false)
  ;;[1 1 1] Switches current targetLocation
  (if (Utilities|Operators|EqualEqual (Transformation|GetActorLocation) (Variables|Default|GetCurrentTargetLocation) 1.0)
    (Utilities|FlowControl|FlipFlop
      (:A
        (Variables|Default|SetCurrentTargetLocation (Variables|Default|GetDownLocation)))
      (:B
        (Variables|Default|SetCurrentTargetLocation (Variables|Default|GetTopLocation))))))

(fn ConstructionScript)