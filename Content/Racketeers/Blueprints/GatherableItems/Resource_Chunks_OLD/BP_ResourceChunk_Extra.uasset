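; BP_ResourceChunk_Extra is a resource chunk actor that a BP_Player can pick up.
; StartInteract records the player as owner, copies the chunk's mesh onto their HoldingObject, clears HoldingObjectVar, then hides the chunk and disables mesh collision.
; CanInteract requires a short downward trace to hit and the chunk not to be held.
; StopInteract only clears the held flag, without restoring visibility or collision.
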(event EventBeginPlay
  (bind _returnvalue (Actor|GetActorOfClass "/Game/Racketeers/Core/BP_Player.BP_Player_C"))
  (Variables|Default|SetLastOwner _returnvalue))

(event Collision|EventActorBeginOverlap
  (params (OtherActor :type Actor%20Object%20Reference)))

(event EventTick
  (params (DeltaSeconds :type Float%20%28single-precision%29)))

(event EventStartInteract
  (params (Instigator :type Actor%20Object%20Reference) (bIsServer :type Boolean))
  ;[1 1 1] Start Interact
  (bind _asbp_player (Utilities|Casting|CastToBP_Player Instigator))
  (Variables|Default|SetLastOwner _asbp_player)
  (Variables|Default|SetIsBeingHeld true)
  (Components|StaticMesh|SetStaticMesh (Variables|/Game/Racketeers/Core/BP_Player.BP_Player_C|GetHoldingObject _asbp_player) (Variables|/Script/Engine.StaticMeshComponent|GetStaticMesh (Variables|Default|GetStaticMesh)))
  (Variables|/Game/Racketeers/Core/BP_Player.BP_Player_C|SetHoldingObjectVar _asbp_player 0)
  (Collision|SetCollisionEnabled (Variables|Default|GetStaticMesh) "NoCollision")
  (Rendering|SetActorHiddenInGame true))

(event EventStopInteract
  (params (Instigator :type Actor%20Object%20Reference))
  ;[1 1 1] Stop Interact
  (Variables|Default|SetIsBeingHeld false))

(fn ConstructionScript)

(fn FloorCheck
  (bind _staticmesh (Variables|Default|GetStaticMesh))
  (bind _returnvalue (Transformation|GetWorldLocation _staticmesh))
  ;[1 1 1] FloorCheck
  (bind _returnvalue_2 (Collision|LineTraceByChannel _returnvalue (- _returnvalue "0.000000,0.000000,10.000000") "TraceTypeQuery1" false 0 "ForOneFrame"))
  (if _returnvalue_2
    (return true)
    (else
      (return false))))

(fn CanInteract
  ;[1 1 1] CanInteract
  (bind _isgrounded (CallFunction|FloorCheck))
  (if (and _isgrounded (not (Variables|Default|GetIsBeingHeld)))
    (return true)
    (else
      (return false))))