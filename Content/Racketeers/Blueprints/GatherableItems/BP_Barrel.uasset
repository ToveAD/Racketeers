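; BP_Barrel is a deposit point that turns resource chunks entering its sphere into team resources.
; On overlap, it follows the chunk's last owner to that player's state and controller, calls AddResource with the chunk's type, value and team, then destroys it.
; Each deposit spawns an effect at a marker and a sound at world origin.
; CanInteract returns true, but StartInteract is empty and the held-item deposit logic is disconnected.
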(event OnComponentBeginOverlap(Sphere)
  (params (OverlappedComponent :type Primitive%20Component%20Object%20Reference) (OtherActor :type Actor%20Object%20Reference) (OtherComp :type Primitive%20Component%20Object%20Reference) (OtherBodyIndex :type Integer) (bFromSweep :type Boolean) (SweepResult :type Hit%20Result%20Structure%20%28by%20ref%29))
  ;[1 1 1] On begin overlap with resource chunks
  (bind _asbp_resource_chunk (Utilities|Casting|CastToBP_ResourceChunk OtherActor))
  (bind _asbp_player (Utilities|Casting|CastToBP_Player (Variables|/Game/Racketeers/Blueprints/GatherableItems/BP_ResourceChunk.BP_ResourceChunk_C|GetLastOwner _asbp_resource_chunk))
    (:then
      (bind _asbp_player_state (Utilities|Casting|CastToBP_PlayerState (Variables|/Script/Engine.Pawn|GetPlayerState _asbp_player))
        (:then
          (bind _asbp_player_controller (Utilities|Casting|CastToBP_PlayerController (Game|GetPlayerController (Variables|/Script/Engine.Pawn|GetPlayerState _asbp_player)))
            (:then
              (Class|RacketeersController|AddResource _asbp_player_controller (Variables|/Game/Racketeers/Blueprints/GatherableItems/BP_ResourceChunk.BP_ResourceChunk_C|GetValue _asbp_resource_chunk) (Variables|/Game/Racketeers/Blueprints/GatherableItems/BP_ResourceChunk.BP_ResourceChunk_C|GetResourecType _asbp_resource_chunk) (.team (Variables|/Script/Racketeers.PS_Base|GetPlayerInfo _asbp_player_state)))
              (Actor|DestroyActor OtherActor)
              (CallFunction|OnDepositSFX))
            (:CastFailed
              (Development|PrintString "null playerController"))))
        (:CastFailed
          (Development|PrintString "Null playerstate"))))
    (:CastFailed
      (Development|PrintString "Null Lastplayer ref"))))

(event Custom|OnDepositSFX
  ;[1 1 1] On deposit SFX
  (Niagara|SpawnSystematLocation (Variables|Default|GetSFX_OnDeposit) (Transformation|GetWorldLocation (Variables|Default|GetSFX_pointLocation)) "0, 0, 0" "1.000000,1.000000,1.000000" true true "AutoRelease")
  (Audio|SpawnSoundatLocation "/Game/Racketeers/Audio/SFX/Environment/SFX_MaterialDeposited.SFX_MaterialDeposited" "0, 0, 0" "0, 0, 0" 1.0 1.0 0.0 0 0))

(event EventBeginPlay)

(event Collision|EventActorBeginOverlap
  (params (OtherActor :type Actor%20Object%20Reference)))

(event EventTick
  (params (DeltaSeconds :type Float%20%28single-precision%29)))

(event EventStartInteract
  (params (Instigator :type Actor%20Object%20Reference) (bIsServer :type Boolean))
  ;[1 1 1] Interact
)

(fn ConstructionScript)

(fn CanInteract
  (return true))