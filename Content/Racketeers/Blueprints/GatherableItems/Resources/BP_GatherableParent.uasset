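; Parent Blueprint for gatherable resources that players interact with to damage and break into loot.
; Each StartInteract lowers ResourceHP, spawns hit FX at a line-trace impact and plays a scale timeline.
; At zero HP, SpawnOnServer waits briefly, launches one resource chunk upward in a random cone and destroys the actor.
; The multi-loot SpawnLoot path is disconnected, and the computed random spawn location is unused.
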(event Custom|OnHitAnimation
  ;[1 1 1] On hit animation
  (bind _scaletrack (Timeline|Timeline PlayFromStart)
    (:Update
      (Transformation|SetWorldScale3D (Variables|Default|GetStaticMesh) (Math|Conversions|ToVector(Float) _scaletrack)))))

(event Custom|OnHitFXS
  (params (Instigator :type Actor%20Object%20Reference))
  ;[1 1 1] On Hit FXS
  (bind _outhit (Collision|LineTraceForObjects (Transformation|GetWorldLocation (Actor|GetComponentbyClass Instigator "/Script/Engine.SpringArmComponent")) (Transformation|GetWorldLocation (Variables|Default|GetGatherPoint)) (Variables|Default|GetObject%20Types) false (Utilities|Array|MakeArray Instigator) "None" false "(R=1.000000,G=0.916018,B=0.957652,A=1.000000)" "(R=0.000000,G=0.109944,B=1.000000,A=1.000000)"))
  (Niagara|SpawnSystematLocation (Variables|Default|GetOnHit_FXS) (.ImpactPoint (Collision|BreakHitResult _outhit)) "0, 0, 0" "1.000000,1.000000,1.000000" true true "AutoRelease"))

(event Custom|SpawnOnServer
  ;[1 1 1] SpawnLoot on server
  (Utilities|FlowControl|Delay 0.2)
  (CallFunction|CustomEvent)
  (Actor|DestroyActor))

(event Custom|CustomEvent
  (bind _locationtospawn (CallFunction|GenerateRandomLocation))
  (bind _returnvalue (Game|SpawnActorfromClass (Variables|Default|GetLootToSpawn) (Math|Conversions|ToTransform(Vector) (Transformation|GetActorLocation)) "Undefined" "MultiplyWithRoot" 0 0))
  (bind _asbp_resource_chunk (Utilities|Casting|CastToBP_ResourceChunk _returnvalue))
  (Physics|AddImpulse (Variables|/Game/Racketeers/Blueprints/GatherableItems/ResourceChunks/BP_ResourceChunk.BP_ResourceChunk_C|GetStaticMesh _asbp_resource_chunk) (* (Math|Random|RandomUnitVectorinConeinDegrees "0.000000,0.000000,1.000000" 45.0) "500.000000,500.000000,500.000000") "None" true))

(event EventBeginPlay)

(event Collision|EventActorBeginOverlap
  (params (OtherActor :type Actor%20Object%20Reference)))

(event EventTick
  (params (DeltaSeconds :type Float%20%28single-precision%29)))

(event EventStartInteract
  (params (Instigator :type Actor%20Object%20Reference) (bIsServer :type Boolean))
  ;[1 1 1] InteractInterface
  (CallFunction|ApplyGatheringdamage Instigator))

(fn ConstructionScript)

(fn ApplyGatheringdamage
  (params (Instigator :type Actor%20Object%20Reference))
  ;[1 1 1] Apply damaged to the object
  (CallFunction|OnHitFXS Instigator)
  (CallFunction|OnHitAnimation)
  (bind _output_get (Variables|Default|SetResourceHP (- (Variables|Default|GetResourceHP) (Variables|Default|GetInitialGatheringDamage))))
  (if (<= _output_get 0.0)
    (CallFunction|SpawnonServer)))

(fn SpawnLoot
  ;[1 1 1] Spawns loot near to the parent object
  (Collision|SetCollisionEnabled (Variables|Default|GetStaticMesh) "NoCollision")
  (for _index (range 1 (Variables|Default|GetAmountLootToSpawn))
    (bind _returnvalue (Game|SpawnActorfromClass (Variables|Default|GetLootToSpawn) (Math|Conversions|ToTransform(Vector) (Transformation|GetActorLocation)) "Undefined" "MultiplyWithRoot" 0 0))
    (bind _asbp_resource_chunk (Utilities|Casting|CastToBP_ResourceChunk _returnvalue))
    (Physics|AddImpulse (Variables|/Game/Racketeers/Blueprints/GatherableItems/ResourceChunks/BP_ResourceChunk.BP_ResourceChunk_C|GetStaticMesh _asbp_resource_chunk) (* (Math|Random|RandomUnitVectorinConeinDegrees "0.000000,0.000000,1.000000" 45.0) "500.000000,500.000000,500.000000") "None" true)))

(fn GenerateRandomLocation
  ;[1 1 1] Generates random locations close to a specific point
  (return (+ (Transformation|GetWorldLocation (Variables|Default|GetStaticMesh)) (* (Math|Vector|RotateVector "1.000000,0.000000,0.000000" (Math|Rotator|MakeRotator 0.0 0.0 (Math|Random|RandomFloatinRange 0.0 3.6e+02))) (Math|Random|RandomFloatinRange (* (Variables|Default|GetLootSpawnMaxDistance) -1.0) (Variables|Default|GetLootSpawnMaxDistance))))))

(fn CanInteract
  ;[1 1 1] CanInteract
  (if (> (Variables|Default|GetResourceHP) 0.0)
    (return true)
    (else
      (return false))))