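; Player controller for Racketeers that shows the score widget on the local player's screen and switches input to game-only with a hidden cursor.
; Check functions fill empty accelerate, steer and gun role arrays for the Racoon or Panda team, always with player character 0.
; Macros branch on team and team player ID from the player state.
; Nothing in this Blueprint calls these helpers, and TEST and SetUpMappingContext are empty stubs.
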(event EventBeginPlay
  (if (Pawn|IsLocalPlayerController self)
    (bind _returnvalue (UserInterface|CreateWidget "/Game/Racketeers/Blueprints/Widgets/WBP_Score.WBP_Score_C" self))
    (UserInterface|Viewport|AddtoViewport _returnvalue 0)
    (Variables|Default|SetbShowMouseCursor false)
    (Input|SetInputModeGameOnly self false)))

(fn ConstructionScript)

(fn CheckAccelerateArray
  (params (IsRacoon :type Boolean))
  (if IsRacoon
    (if (Utilities|Array|IsEmpty (Variables|Default|GetRacoonAccelerate))
      (Utilities|Array|Add (Variables|Default|GetRacoonAccelerate) (Game|GetPlayerCharacter 0))
      (return))
    (elif (Utilities|Array|IsEmpty (Variables|Default|GetPandaAccelerate))
      (Utilities|Array|Add (Variables|Default|GetPandaAccelerate) (Game|GetPlayerCharacter 0))
      (return))))

(fn CheckSteerArray
  (params (IsRacoon :type Boolean))
  (if IsRacoon
    (if (Utilities|Array|IsEmpty (Variables|Default|GetRacoonSteer))
      (Utilities|Array|Add (Variables|Default|GetRacoonSteer) (Game|GetPlayerCharacter 0))
      (return))
    (elif (Utilities|Array|IsEmpty (Variables|Default|GetPandaSteer))
      (Utilities|Array|Add (Variables|Default|GetPandaSteer) (Game|GetPlayerCharacter 0))
      (return))))

(fn CheckShootArray
  (params (IsRacoon :type Boolean))
  (if IsRacoon
    (if (Utilities|Array|IsEmpty (Variables|Default|GetRacoonGun))
      (Utilities|Array|Add (Variables|Default|GetRacoonGun) (Game|GetPlayerCharacter 0))
      (return))
    (elif (Utilities|Array|IsEmpty (Variables|Default|GetPandaGun))
      (Utilities|Array|Add (Variables|Default|GetPandaGun) (Game|GetPlayerCharacter 0))
      (return))))

(fn TEST
  (params (TeamID :type ETeams%20Enum :default "Team_Racoon") (PlayerID :type Integer)))

(fn SetUpMappingContext)