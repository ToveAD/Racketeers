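; Lobby player controller for Racketeers that creates the lobby UI for the local player and reports that player's lobby info to BP_LobbyGameMode.
; Ready toggling (R key) and name changes edit the PlayerLobbyInfoPC struct through OnServer events, then push it to the game mode.
; The game mode update also runs on BeginPlay, with a delayed retry event available.
; Match start shows the UI's loading screen and disables input.
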(event Custom|TryAgainUpdatingLobbyPC
  (Utilities|FlowControl|Delay 0.1)
  (bind _asbp_lobby_game_mode (Utilities|Casting|CastToBP_LobbyGameMode (Game|GetGameMode)))
  (Default|UpdatePlayerLobbyInfo _asbp_lobby_game_mode self))

(event Custom|ToggleReadyStatusOnServer
  (bind _playerlobbyinfopc (Variables|Default|GetPlayerLobbyInfoPC))
  (Utilities|Struct|SetmembersinFPlayerLobbyInfo _playerlobbyinfopc (not (.bReady (Utilities|Struct|BreakFPlayerLobbyInfo _playerlobbyinfopc))))
  (bind _asbp_lobby_game_mode (Utilities|Casting|CastToBP_LobbyGameMode (Game|GetGameMode)))
  (Default|UpdatePlayerLobbyInfo _asbp_lobby_game_mode self))

(event Custom|SetPlayerNameOnServer
  (params (PlayerName :type Text))
  (Utilities|Struct|SetmembersinFPlayerLobbyInfo (Variables|Default|GetPlayerLobbyInfoPC) PlayerName)
  (bind _asbp_lobby_game_mode (Utilities|Casting|CastToBP_LobbyGameMode (Game|GetGameMode)))
  (Default|UpdatePlayerLobbyInfo _asbp_lobby_game_mode self))

(event Custom|OnStartMatch
  (Default|ShowLoadingScreen (Variables|Default|GetLobbyUIREF))
  (Input|DisableInput self))

(event EventBeginPlay
  (CallFunction|SetUp)
  (bind _asbp_lobby_game_mode (Utilities|Casting|CastToBP_LobbyGameMode (Game|GetGameMode)))
  (Default|UpdatePlayerLobbyInfo _asbp_lobby_game_mode self))

(event Input|KeyboardEvents|R
  (params (Key :type Key%20Structure :default "None"))
  (:Pressed
    (CallFunction|ToggleReadyStatusonServer)))

(fn ConstructionScript)

(fn SetUp
  (if (Pawn|IsLocalPlayerController)
    (Variables|Default|SetbShowMouseCursor true)
    (Input|SetInputModeGameandUI self 0 "DoNotLock" false false)
    (bind _returnvalue (UserInterface|CreateWidget "/Game/Racketeers/Blueprints/Widgets/WBP_LobbyUI.WBP_LobbyUI_C"))
    (bind _output_get (Variables|Default|SetLobbyUIREF _returnvalue))
    (UserInterface|Viewport|AddtoViewport _output_get 0)))