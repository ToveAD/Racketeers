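; Player character for Racketeers that routes input to interacting, crafting, throwing, pushing, scurrying and boat controls.
; Tapped (cooldown-limited) or held interaction box-traces for Interactable actors, predicts locally, then runs through server and multicast events.
; Throws and work-in-progress scurry collisions also replicate via server-to-multicast, while boat inputs forward to the BP_Boat stored as InteractableObject.
; PlayerInfo's OnRep refreshes the lobby info widget, retrying until it exists.
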(event Custom|Server_Interact
  (params (Target :type Actor%20Object%20Reference) (Instigator :type Actor%20Object%20Reference))
  ;[1 1 1] Server Logic
  (CallFunction|MultiInteract Target Instigator))

(event Custom|Multi_Interact
  (params (Target :type Object%20Object%20Reference) (Instigator :type Actor%20Object%20Reference))
  ;[1 1 1] Server Logic
  (bind _returnvalue (Class|Interactable|CanInteract(Message) Target))
  (if _returnvalue
    (Class|Interactable|StartInteract(Message) Target Instigator true)))

(event Custom|Server_Throw
  (CallFunction|MultiThrow))

(event Custom|ScurryOnCollision_Event
  (params (HitActor :type Actor%20Object%20Reference) (ScurryComponent :type BP%20Scurry%20Component%20Object%20Reference))
  (Default|OnCollision ScurryComponent HitActor))

(event Custom|Server_ScurryOnCollision
  (params (HitActor :type Actor%20Object%20Reference) (ScurryComponent :type BP%20Scurry%20Component%20Object%20Reference))
  (CallFunction|MultiScurryonCollision HitActor ScurryComponent))

(event Custom|Multi_Throw
  (CallFunction|ThrowEvent))

(event Custom|Multi_ScurryOnCollision
  (params (HitActor :type Actor%20Object%20Reference) (ScurryComponent :type BP%20Scurry%20Component%20Object%20Reference))
  (CallFunction|ScurryonCollisionEvent HitActor ScurryComponent))

(event Custom|Throw_Event
  (bind _holdingobjectvar (Variables|Default|GetHoldingObjectVar))
  (bind _staticmesh (Variables|/Game/Racketeers/Blueprints/GatherableItems/ResourceChunks/BP_ResourceChunk.BP_ResourceChunk_C|GetStaticMesh _holdingobjectvar))
  (Transformation|SetActorLocation (Variables|Default|GetHoldingObjectVar) (Transformation|GetWorldLocation (Variables|Default|GetHoldingObject)) false false)
  (Rendering|SetActorHiddenInGame _holdingobjectvar false)
  (Collision|SetCollisionEnabled _staticmesh "QueryAndPhysics")
  (Physics|SetSimulatePhysics _staticmesh true)
  (Physics|AddImpulse _staticmesh (* (Transformation|GetActorForwardVector) 3e+03) "None" true))

(event Input|EnhancedActionEvents|EnhancedInputActionIA_Interact
  (params (ActionValue :type Boolean) (ElapsedSeconds :type Float%20%28double-precision%29) (TriggeredSeconds :type Float%20%28double-precision%29) (InputAction :type Input%20Action%20Object%20Reference :default "/Game/Racketeers/Characters/Input/Actions/IA_Interact.IA_Interact"))
  (bind _asracketeers_controller (Utilities|Casting|CastToRacketeersController (Game|GetPlayerController 0)))
  (Class|RacketeersController|RequestRemoveWidget _asracketeers_controller))

(event Input|EnhancedActionEvents|EnhancedInputActionIA_Interact
  (params (ActionValue :type Boolean) (ElapsedSeconds :type Float%20%28double-precision%29) (TriggeredSeconds :type Float%20%28double-precision%29) (InputAction :type Input%20Action%20Object%20Reference :default "/Game/Racketeers/Characters/Input/Actions/IA_Interact.IA_Interact"))
  (bind _returnvalue (Pawn|GetController))
  (bind _holdinginteracttimeinterval (Variables|Default|GetHoldingInteractTimeInterval))
  (bind _returnvalue_2 (Pawn|IsLocalController _returnvalue))
  (:Triggered
    (Networking|SwitchHasAuthority
      (:Authority
        (if _returnvalue_2
          (Development|PrintString "Server Interact")
          ;[1 1 1] GatherHolding
          (if (and (Variables|Default|GetCanInteract) (>= TriggeredSeconds _holdinginteracttimeinterval)) :!label _label
            (if (< (Math|Float|%(Float) (* TriggeredSeconds 6e+01) (* _holdinginteracttimeinterval 6e+01)) 0.2)
              (bind (_foundinteractable _interactableobject) (CallFunction|LookforInteractables :!label _label_2))
              ;[1 1 1] GatherObejct
              (Variables|Default|SetInteractable%20Object _interactableobject)
              (if _foundinteractable
                (bind _returnvalue_3 (Class|Interactable|CanInteract(Message) _interactableobject))
                (if _returnvalue_3
                  ;;[1 1 1] Client Prediction
                  (Class|Interactable|StartInteract(Message) _interactableobject self false)
                  (CallFunction|ServerInteract _interactableobject self)))))))
      (:Remote
        (if _returnvalue_2
          (Development|PrintString "Client Interact")
          (goto _label)))))
  (:Started
    (Utilities|FlowControl|Sequence
      (:then_0
        ;[1 1 1] GatherTap
        (if (Variables|Default|GetCanInteract)
          (Variables|Default|SetCanInteract false)
          (Utilities|Time|SetTimerbyFunctionName 0 "EnableInteraction" (Variables|Default|GetInteractionTimeIntervalLimit))
          (goto _label_2)))
      (:then_1
        (bind _asbp_player_state (Utilities|Casting|CastToBP_PlayerState (Variables|/Script/Engine.Controller|GetPlayerState (Game|GetPlayerController 0))))
        (Default|OnInteract (Variables|Default|GetBP_CraftComponent) (.Team (Utilities|Struct|BreakPlayerInfo (Variables|/Script/Racketeers.PS_Base|GetPlayerInfo _asbp_player_state)))))))
  (:Completed
    (Utilities|IsValid (Variables|Default|GetHoldingObjectVar)
      (:Is%20Valid
        (CallFunction|ServerThrow)))))

(event Input|EnhancedActionEvents|EnhancedInputActionIA_Boat_Steer
  (params (ActionValue :type Float%20%28double-precision%29) (ElapsedSeconds :type Float%20%28double-precision%29) (TriggeredSeconds :type Float%20%28double-precision%29) (InputAction :type Input%20Action%20Object%20Reference :default "/Game/Racketeers/Characters/Input/Actions/IA_Boat_Steer.IA_Boat_Steer"))
  ;[1 1 1] Ship Inputs
  (bind _asbp_boat (Utilities|Casting|CastToBP_Boat (Variables|Default|GetInteractable%20Object)))
  (Default|SteerBoat _asbp_boat ActionValue))

(event Input|EnhancedActionEvents|EnhancedInputActionIA_Boat_Interact
  (params (ActionValue :type Boolean) (ElapsedSeconds :type Float%20%28double-precision%29) (TriggeredSeconds :type Float%20%28double-precision%29) (InputAction :type Input%20Action%20Object%20Reference :default "/Game/Racketeers/Characters/Input/Actions/IA_Boat_Interact.IA_Boat_Interact"))
  ;[1 1 1] Ship Inputs
  (:Started
    (bind _asbp_boat (Utilities|Casting|CastToBP_Boat (Variables|Default|GetInteractable%20Object)))
    (Default|LeaveBoatInteract _asbp_boat)))

(event Input|EnhancedActionEvents|EnhancedInputActionIA_Boat_ShootLeft
  (params (ActionValue :type Vector%202D%20Structure) (ElapsedSeconds :type Float%20%28double-precision%29) (TriggeredSeconds :type Float%20%28double-precision%29) (InputAction :type Input%20Action%20Object%20Reference :default "/Game/Racketeers/Characters/Input/Actions/IA_Boat_ShootLeft.IA_Boat_ShootLeft"))
  ;[1 1 1] Ship Inputs
  (:Started
    (bind _asbp_boat (Utilities|Casting|CastToBP_Boat (Variables|Default|GetInteractable%20Object)))
    (Default|BoatShootLeft _asbp_boat)))

(event Input|EnhancedActionEvents|EnhancedInputActionIA_Boat_ShootRight
  (params (ActionValue :type Vector%202D%20Structure) (ElapsedSeconds :type Float%20%28double-precision%29) (TriggeredSeconds :type Float%20%28double-precision%29) (InputAction :type Input%20Action%20Object%20Reference :default "/Game/Racketeers/Characters/Input/Actions/IA_Boat_ShootRight.IA_Boat_ShootRight"))
  ;[1 1 1] Ship Inputs
  (bind _asbp_boat (Utilities|Casting|CastToBP_Boat (Variables|Default|GetInteractable%20Object)))
  (Default|BoatShootRight _asbp_boat))

(event Input|EnhancedActionEvents|EnhancedInputActionIA_Push
  (params (ActionValue :type Boolean) (ElapsedSeconds :type Float%20%28double-precision%29) (TriggeredSeconds :type Float%20%28double-precision%29) (InputAction :type Input%20Action%20Object%20Reference :default "/Game/Racketeers/Characters/Input/Actions/IA_Push.IA_Push"))
  (:Started
    (Default|Push (Variables|Default|GetBP_PusherComponent))))

(event Input|EnhancedActionEvents|EnhancedInputActionIA_InteractCrafting
  (params (ActionValue :type Boolean) (ElapsedSeconds :type Float%20%28double-precision%29) (TriggeredSeconds :type Float%20%28double-precision%29) (InputAction :type Input%20Action%20Object%20Reference :default "/Game/Racketeers/Characters/Input/Actions/IA_InteractCrafting.IA_InteractCrafting")))

(event Input|EnhancedActionEvents|EnhancedInputActionIA_Scurry
  (params (ActionValue :type Boolean) (ElapsedSeconds :type Float%20%28double-precision%29) (TriggeredSeconds :type Float%20%28double-precision%29) (InputAction :type Input%20Action%20Object%20Reference :default "/Game/Racketeers/Characters/Input/Actions/IA_Scurry.IA_Scurry"))
  (:Started
    (Default|StartScurry (Variables|Default|GetBP_ScurryComponent))))

(event Input|EnhancedActionEvents|EnhancedInputActionIA_Boat_Accelerate
  (params (ActionValue :type Float%20%28double-precision%29) (ElapsedSeconds :type Float%20%28double-precision%29) (TriggeredSeconds :type Float%20%28double-precision%29) (InputAction :type Input%20Action%20Object%20Reference :default "/Game/Racketeers/Characters/Input/Actions/IA_Boat_Accelerate.IA_Boat_Accelerate"))
  ;[1 1 1] Ship Inputs
  (bind _asbp_boat (Utilities|Casting|CastToBP_Boat (Variables|Default|GetInteractable%20Object)))
  (Default|BoatAccelerate _asbp_boat ActionValue))

(event Input|EnhancedActionEvents|EnhancedInputActionIA_Boat_Deaccelerate
  (params (ActionValue :type Float%20%28double-precision%29) (ElapsedSeconds :type Float%20%28double-precision%29) (TriggeredSeconds :type Float%20%28double-precision%29) (InputAction :type Input%20Action%20Object%20Reference :default "/Game/Racketeers/Characters/Input/Actions/IA_Boat_Deaccelerate.IA_Boat_Deaccelerate"))
  ;[1 1 1] Ship Inputs
  (bind _asbp_boat (Utilities|Casting|CastToBP_Boat (Variables|Default|GetInteractable%20Object)))
  (Default|BoatAccelerate _asbp_boat ActionValue))

(event EventBeginPlay)

(event Collision|EventHit
  (params (MyComp :type Primitive%20Component%20Object%20Reference) (Other :type Actor%20Object%20Reference) (OtherComp :type Primitive%20Component%20Object%20Reference) (bSelfMoved :type Boolean) (HitLocation :type Vector :default "0, 0, 0") (HitNormal :type Vector :default "0, 0, 0") (NormalImpulse :type Vector :default "0, 0, 0") (Hit :type Hit%20Result%20Structure%20%28by%20ref%29))
  (bind _returnvalue (Actor|GetComponentbyClass Other "/Game/Racketeers/Blueprints/Components/BP_ScurryComponent.BP_ScurryComponent_C"))
  ;[1 1 1] Scurry stuff (WIP)
  (Utilities|IsValid _returnvalue
    (:Is%20Valid
      (if (and (Variables|/Game/Racketeers/Blueprints/Components/BP_ScurryComponent.BP_ScurryComponent_C|GetIsScurrying (Variables|Default|GetBP_ScurryComponent)) (Variables|/Game/Racketeers/Blueprints/Components/BP_ScurryComponent.BP_ScurryComponent_C|GetIsScurrying _returnvalue))
        (CallFunction|ServerScurryonCollision Other (Variables|Default|GetBP_ScurryComponent))
        (CallFunction|ServerScurryonCollision self _returnvalue)))))

(fn ConstructionScript)

(fn UpdatePlayerLobbyInfo
  (params (PlayerLobbyInfo :type Player%20Info%20Structure))
  (Variables|Default|SetPlayerInfo PlayerLobbyInfo))

(fn EnableInteraction
  (Variables|Default|SetCanInteract true))

(fn GatherHold
  (params (End :type Vector) (Start :type Vector) (Orientation :type Rotator) (ObjectTypes :type Array%20of%20EObjectTypeQuery%20Enums :default "ObjectTypeQuery1"))
  (bind _self self)
  (bind (_outhit _returnvalue) (Class|KismetSystemLibrary|BoxTraceSingleforObjects Start End "32.000000,32.000000,64.000000" Orientation ObjectTypes false 0 "ForDuration" true))
  (if (and _returnvalue (Utilities|DoesObjectImplementInterface (.HitActor (Collision|BreakHitResult _outhit)) "/Script/Racketeers.Interactable"))
    (bind _returnvalue_2 (Class|Interactable|CanInteract(Message) (.HitActor (Collision|BreakHitResult _outhit))))
    (if _returnvalue_2
      (Networking|SwitchHasAuthority
        (:Authority
          _)
        (:Remote
          ;[1 1 1] Client Prediction
          (Class|Interactable|StartInteract(Message) (.HitActor (Collision|BreakHitResult _outhit)) _self false)))
      (CallFunction|ServerInteract (.HitActor (Collision|BreakHitResult _outhit)) _self))))

(fn EnableHoldingInteraction
  (Variables|Default|SetHoldGatherTimmer true))

(fn LookforInteractables
  (bind _interactionlocation (Variables|Default|GetInteractionLocation))
  (bind _returnvalue (Transformation|GetWorldLocation _interactionlocation))
  (bind (_outhit _returnvalue_2) (Class|KismetSystemLibrary|BoxTraceSingleforObjects _returnvalue _returnvalue "32.000000,32.000000,64.000000" (Transformation|GetActorRotation) (Utilities|Array|MakeArray "ObjectTypeQuery2") false 0 "ForDuration" true))
  (return (and _returnvalue_2 (Utilities|DoesObjectImplementInterface (.HitActor (Collision|BreakHitResult _outhit)) "/Script/Racketeers.Interactable")) (.HitActor (Collision|BreakHitResult _outhit))))

(fn OnRepPlayerInfo
  (bind _lobbyinfo (Variables|Default|GetLobbyInfo))
  (bind _returnvalue (UserInterface|GetWidget _lobbyinfo))
  (Utilities|IsValid _returnvalue
    (:Is%20Valid
      (bind _aswbp_player_lobby_info (Utilities|Casting|CastToWBP_PlayerLobbyInfo _returnvalue))
      (Default|Update _aswbp_player_lobby_info (Variables|Default|GetPlayerInfo))
      (Rendering|SetVisibility (Variables|Default|GetLobbyInfo) true false))
    (:Is%20Not%20Valid
      (Utilities|Time|SetTimerbyFunctionName 0 "OnRep_PlayerInfo" 0.1))))