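; Base game mode that brings players from the lobby into the game with their team identity and spawn setup.
; On controller swap, it copies lobby name, team and team player ID into BP_PlayerState.
; Pawn class follows team (racoon or red panda, else BP_Player), but reads player controller 0 instead of InController.
; Player starts are matched by a tag combining team name and team player ID, falling back to the parent choice.
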(event EventOnSwapPlayerControllers
  (params (OldPC :type Player%20Controller%20Object%20Reference) (NewPC :type Player%20Controller%20Object%20Reference))
  ;[1 1 1] Bring PC from lobby to game
  (bind _asbp_lobby_pc (Utilities|Casting|CastToBP_LobbyPC OldPC))
  (bind _asbp_player_controller (Utilities|Casting|CastToBP_PlayerController NewPC))
  (bind _asbp_player_state (Utilities|Casting|CastToBP_PlayerState (Variables|/Script/Engine.Controller|GetPlayerState _asbp_player_controller)))
  (Variables|/Script/Racketeers.PS_Base|SetPlayerInfo _asbp_player_state (Utilities|Struct|MakePlayerInfo NewPC (.PlayerName (Utilities|Struct|BreakPlayerInfo (Variables|/Game/Racketeers/Characters/Blueprints/PCs/BP_LobbyPC.BP_LobbyPC_C|GetPlayerInfoPC _asbp_lobby_pc))) false _asbp_player_state (.Team (Utilities|Struct|BreakPlayerInfo (Variables|/Game/Racketeers/Characters/Blueprints/PCs/BP_LobbyPC.BP_LobbyPC_C|GetPlayerInfoPC _asbp_lobby_pc))) (.TeamPlayerID (Utilities|Struct|BreakPlayerInfo (Variables|/Game/Racketeers/Characters/Blueprints/PCs/BP_LobbyPC.BP_LobbyPC_C|GetPlayerInfoPC _asbp_lobby_pc)))))
  (Variables|/Script/Racketeers.PS_Base|SetTeam _asbp_player_state (.Team (Utilities|Struct|BreakPlayerInfo (Variables|/Game/Racketeers/Characters/Blueprints/PCs/BP_LobbyPC.BP_LobbyPC_C|GetPlayerInfoPC _asbp_lobby_pc))))
  (Variables|/Script/Racketeers.PS_Base|SetTeamPlayerID _asbp_player_state (.TeamPlayerID (Utilities|Struct|BreakPlayerInfo (Variables|/Game/Racketeers/Characters/Blueprints/PCs/BP_LobbyPC.BP_LobbyPC_C|GetPlayerInfoPC _asbp_lobby_pc))))
  (Variables|/Script/Racketeers.PS_Base|SetPlayerController _asbp_player_state NewPC))

(fn ConstructionScript)

(fn GetDefaultPawnClassforController
  (params (InController :type Controller%20Object%20Reference))
  (bind _asbp_player_state (Utilities|Casting|CastToBP_PlayerState (Variables|/Script/Engine.Controller|GetPlayerState (Game|GetPlayerController 0))))
  (if (Utilities|IsValidClass (Utilities|Select :Index (.team (Variables|/Script/Racketeers.PS_Base|GetPlayerInfo _asbp_player_state)) :Team_Racoon "/Game/Racketeers/Characters/Blueprints/BP_Racoon.BP_Racoon_C" :Team_Panda "/Game/Racketeers/Characters/Blueprints/BP_RedPanda.BP_RedPanda_C"))
    (return (Utilities|Select :Index (.team (Variables|/Script/Racketeers.PS_Base|GetPlayerInfo _asbp_player_state)) :Team_Racoon "/Game/Racketeers/Characters/Blueprints/BP_Racoon.BP_Racoon_C" :Team_Panda "/Game/Racketeers/Characters/Blueprints/BP_RedPanda.BP_RedPanda_C"))
    (else
      (return "/Game/Racketeers/Core/BP_Player.BP_Player_C"))))

(fn ChoosePlayerStart
  (params (Player :type Controller%20Object%20Reference))
  (bind _asbp_player_state (Utilities|Casting|CastToBP_PlayerState (Variables|/Script/Engine.Controller|GetPlayerState Player)))
  (bind _outactors (Actor|GetAllActorsOfClass "/Script/Engine.PlayerStart"))
  (for _array_element _outactors
    (if (== (Variables|/Script/Engine.PlayerStart|GetPlayerStartTag _array_element) (Utilities|Name|MakeLiteralName (Utilities|String|StringToName (Utilities|String|Append (Utilities|String|EnumtoString (.Team (Utilities|Struct|BreakPlayerInfo (Variables|/Script/Racketeers.PS_Base|GetPlayerInfo _asbp_player_state)))) (Utilities|String|ToString(Integer) (.TeamPlayerID (Utilities|Struct|BreakPlayerInfo (Variables|/Script/Racketeers.PS_Base|GetPlayerInfo _asbp_player_state))))))))
      (return _array_element)))
  (bind _returnvalue (|CallParentFunction 0))
  (return _returnvalue))