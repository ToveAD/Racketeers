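; Game mode for the winner screen, placing raccoon characters on podiums and returning players to the lobby.
; BeginPlay caches all BP_Podeum actors and spawns a BP_Racoon at the first available one matching player 0's team and ID.
; PostLogin repeats that search for joining players, but with a hardcoded raccoon team and ID 0.
; IncrementLobbyRequestCount tallies return requests, server-traveling to Lobby when they equal the player count.
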(event Custom|LoadIntoLobby
  (Class|AdvancedSessionsLibrary|ServerTravel "Lobby" false false))

(event EventBeginPlay
  (bind _outactors (Actor|GetAllActorsOfClass "/Game/Racketeers/Blueprints/Actors/BP_Podeum.BP_Podeum_C"))
  (Variables|Default|SetPodeums _outactors)
  (Development|PrintString "Logged in")
  (bind _asbp_player_state (Utilities|Casting|CastToBP_PlayerState (Variables|/Script/Engine.Controller|GetPlayerState (Game|GetPlayerController 0)))
    (:then
      (bind _array_element (Utilities|Array|ForEachLoopwithBreak (Variables|Default|GetPodeums) :!label _label)
        (:LoopBody
          (Development|PrintString "Check AVALIBLE")
          (bind _avalible (Default|CheckAvalability _array_element (Variables|/Script/Racketeers.PS_Base|GetTeam _asbp_player_state) (Variables|/Script/Racketeers.PS_Base|GetTeamPlayerID _asbp_player_state)))
          (if _avalible
            (Development|PrintString (Utilities|String|ToString(Boolean) _avalible))
            (Game|SpawnActorfromClass "/Game/Racketeers/Characters/Blueprints/BP_Racoon.BP_Racoon_C" (Transformation|GetWorldTransform (Variables|/Game/Racketeers/Blueprints/Actors/BP_Podeum.BP_Podeum_C|GetPlayerSpot _array_element)) "AdjustIfPossibleButAlwaysSpawn" "MultiplyWithRoot" 0 0)
            (goto _label Break)
            (else
              (Development|PrintString (Utilities|String|ToString(Boolean) _avalible)))))))
    (:CastFailed
      (Development|PrintString "Failed To Cast"))))

(event EventTick
  (params (DeltaSeconds :type Float%20%28single-precision%29)))

(event EventPostLogin
  (params (NewPlayer :type Player%20Controller%20Object%20Reference))
  (Development|PrintString "Logged in")
  (bind _asbp_player_state (Utilities|Casting|CastToBP_PlayerState (Variables|/Script/Engine.Controller|GetPlayerState NewPlayer))
    (:then
      (bind _array_element (Utilities|Array|ForEachLoopwithBreak (Variables|Default|GetPodeums) :!label _label)
        (:LoopBody
          (Development|PrintString "Check AVALIBLE")
          (bind _avalible (Default|CheckAvalability _array_element "Team_Racoon"))
          (if _avalible
            (Development|PrintString (Utilities|String|ToString(Boolean) _avalible))
            (Game|SpawnActorfromClass "/Game/Racketeers/Characters/Blueprints/BP_Racoon.BP_Racoon_C" (Transformation|GetWorldTransform (Variables|/Game/Racketeers/Blueprints/Actors/BP_Podeum.BP_Podeum_C|GetPlayerSpot _array_element)) "AdjustIfPossibleButAlwaysSpawn" "MultiplyWithRoot" 0 0)
            (goto _label Break)
            (else
              (Development|PrintString (Utilities|String|ToString(Boolean) _avalible)))))))
    (:CastFailed
      (Development|PrintString "Failed To Cast"))))

(fn ConstructionScript)

(fn IncrementLobbyRequestCount
  (bind _result (Math|Integer|IncrementInt (Variables|Default|GetGoToLobbyCount))
    (:%20%20
      (if (== _result (Utilities|Array|Length (Variables|/Script/Engine.GameStateBase|GetPlayerArray (Game|GetGameState))))
        (CallFunction|LoadIntoLobby)
        (Variables|Default|SetGoToLobbyCount 0)
        (return)))))