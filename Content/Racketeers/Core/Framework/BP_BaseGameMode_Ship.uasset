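; Game mode for the ship game in Racketeers that sorts players into Racoon and Panda teams and hands out roles.
; Five seconds after each login, it loops over every player state, adding each controller to its team's array without clearing earlier entries.
; That array's length after the add selects the role recorded and passed to BP_PlayerController's SetRole.
; AssignRoles is an unfinished alternative that switches on TeamPlayerID with no actions.
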(event Custom|AssignRoles
  (for _array_element (Variables|/Script/Engine.GameStateBase|GetPlayerArray (Game|GetGameState))
    (bind _asbp_player_state (Utilities|Casting|CastToBP_PlayerState _array_element))
    (switch int (.TeamPlayerID (Utilities|Struct|BreakPlayerInfo (Variables|/Script/Racketeers.PS_Base|GetPlayerInfo _asbp_player_state))))))

(event EventBeginPlay)

(event EventPostLogin
  (params (NewPlayer :type Player%20Controller%20Object%20Reference))
  (Utilities|FlowControl|Delay 5.0)
  (Development|PrintString "OnPostLogin")
  (for _array_element (Variables|/Script/Engine.GameStateBase|GetPlayerArray (Game|GetGameState))
    (bind _asbp_player_state (Utilities|Casting|CastToBP_PlayerState _array_element))
    (Variables|Default|SetPlayerRef (Game|GetPlayerController _asbp_player_state))
    (switch Utilities|FlowControl|Switch|SwitchonETeams (.Team (Utilities|Struct|BreakPlayerInfo (Variables|/Script/Racketeers.PS_Base|GetPlayerInfo _asbp_player_state)))
      (:Team_Racoon
        (Utilities|Array|Add (Variables|Default|GetPlayerControllersRacoon) (Variables|Default|GetPlayerRef))
        (switch int (Utilities|Array|Length (Variables|Default|GetPlayerControllersRacoon))
          (:0
            (Utilities|Array|Add (Variables|Default|GetEPlayerRoles) "NewEnumerator0")
            (bind _asbp_player_controller (Utilities|Casting|CastToBP_PlayerController (Variables|Default|GetPlayerRef)))
            (Default|SetRole _asbp_player_controller "NewEnumerator0"))
          (:1
            (Utilities|Array|Add (Variables|Default|GetEPlayerRoles) "NewEnumerator1")
            (bind _asbp_player_controller_2 (Utilities|Casting|CastToBP_PlayerController (Variables|Default|GetPlayerRef)))
            (Default|SetRole _asbp_player_controller_2 "NewEnumerator1"))
          (:2
            (Utilities|Array|Add (Variables|Default|GetEPlayerRoles) "NewEnumerator2")
            (bind _asbp_player_controller_3 (Utilities|Casting|CastToBP_PlayerController (Variables|Default|GetPlayerRef)))
            (Default|SetRole _asbp_player_controller_3 "NewEnumerator2"))))
      (:Team_Panda
        (Utilities|Array|Add (Variables|Default|GetPlayerControllersPanda) (Variables|Default|GetPlayerRef))
        (switch int (Utilities|Array|Length (Variables|Default|GetPlayerControllersPanda))
          (:0
            (Utilities|Array|Add (Variables|Default|GetEPlayerRoles) "NewEnumerator0")
            (bind _asbp_player_controller_4 (Utilities|Casting|CastToBP_PlayerController (Variables|Default|GetPlayerRef)))
            (Default|SetRole _asbp_player_controller_4 "NewEnumerator0"))
          (:1
            (Utilities|Array|Add (Variables|Default|GetEPlayerRoles) "NewEnumerator1")
            (bind _asbp_player_controller_5 (Utilities|Casting|CastToBP_PlayerController (Variables|Default|GetPlayerRef)))
            (Default|SetRole _asbp_player_controller_5 "NewEnumerator1"))
          (:2
            (Utilities|Array|Add (Variables|Default|GetEPlayerRoles) "NewEnumerator2")
            (bind _asbp_player_controller_6 (Utilities|Casting|CastToBP_PlayerController (Variables|Default|GetPlayerRef)))
            (Default|SetRole _asbp_player_controller_6 "NewEnumerator2")))))))

(event EventTick
  (params (DeltaSeconds :type Float%20%28single-precision%29)))

(fn ConstructionScript
  (|CallParentFunction))