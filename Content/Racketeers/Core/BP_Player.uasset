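; Player character Blueprint for the Raccoon and Panda teams, handling on-foot actions, boat controls and lobby info display, plus debug keys.
; Interact drives crafting, pushing, tap or hold gathering via box traces for Interactable actors, and charged throws of held resources.
; Interactions, throws and work-in-progress scurry collisions use Server-to-Multicast events.
; Boat inputs forward movement, shooting, scurry and exit to the interacted BP_Boat, while OnRep_PlayerInfo refreshes the lobby widget.
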(event Custom|Server_Interact
  (params (Target :type Actor%20Object%20Reference) (Instigator :type Actor%20Object%20Reference))
  ;[1 1 1] Server Logic
  (CallFunction|MultiInteract Target Instigator))

(event Custom|Multi_Interact
  (params (Target :type Object%20Object%20Reference) (Instigator :type Actor%20Object%20Reference))
  ;[1 1 1] Server Logic
  (Class|Interactable|StartInteract(Message) Target Instigator true))

(event Custom|KickPlayer
  (params (Controller :type Player%20Controller%20Object%20Reference) (Bool :type Boolean))
  (if Bool
    (Class|GameModeBase|ReturntoMainMenuHost (Game|GetGameMode))
    (else
      (Class|AdvancedSessionsLibrary|KickPlayer Controller))))

(event Custom|Server_Throw
  (params (Instigator :type BP%20Player%20Object%20Reference) (NewParam :type Float%20%28double-precision%29%20%28by%20ref%29))
  (CallFunction|ThrowResource false Instigator NewParam)
  (CallFunction|MultiThrow Instigator))

(event Custom|ScurryOnCollision_Event
  (params (HitActor :type Actor%20Object%20Reference) (ScurryComponent :type BP%20Scurry%20Component%20Object%20Reference))
  (Default|OnCollision ScurryComponent HitActor))

(event Custom|Server_ScurryOnCollision
  (params (HitActor :type Actor%20Object%20Reference) (ScurryComponent :type BP%20Scurry%20Component%20Object%20Reference))
  (CallFunction|MultiScurryonCollision HitActor ScurryComponent))

(event Custom|Multi_Throw
  (params (Instigator :type BP%20Player%20Object%20Reference))
  (Variables|BP_Player_C|SetIsHoldingResource Instigator false))

(event Custom|Multi_ScurryOnCollision
  (params (HitActor :type Actor%20Object%20Reference) (ScurryComponent :type BP%20Scurry%20Component%20Object%20Reference))
  (CallFunction|ScurryonCollisionEvent HitActor ScurryComponent))

(event Custom|Throw_Event)

(event Custom|Server_StartHoldShoot
  ;[1 1 1] Ship Inputs
  (Variables|Default|SetbIsHoldingShoot true)
  (Variables|Default|SetShootTime 1.0))

(event Custom|Server_StopHoldShoot
  ;[1 1 1] Ship Inputs
  (Variables|Default|SetbIsHoldingShoot false))

(event Input|EnhancedActionEvents|EnhancedInputActionIA_Interact
  (params (ActionValue :type Boolean) (ElapsedSeconds :type Float%20%28double-precision%29) (TriggeredSeconds :type Float%20%28double-precision%29) (InputAction :type Input%20Action%20Object%20Reference :default "/Game/Racketeers/Characters/Input/Actions/IA_Interact.IA_Interact"))
  (:Started
    (Default|CallOnPressReadyButton (Subsystems|GetWidgetSubsystem))))

(event Input|EnhancedActionEvents|EnhancedInputActionIA_Interact
  (params (ActionValue :type Boolean) (ElapsedSeconds :type Float%20%28double-precision%29) (TriggeredSeconds :type Float%20%28double-precision%29) (InputAction :type Input%20Action%20Object%20Reference :default "/Game/Racketeers/Characters/Input/Actions/IA_Interact.IA_Interact"))
  (bind _returnvalue (Pawn|GetController))
  (bind _holdinginteracttimeinterval (Variables|Default|GetHoldingInteractTimeInterval))
  (bind _returnvalue_2 (Pawn|IsLocalController _returnvalue))
  (:Triggered
    (if (not (Variables|Default|GetIsHoldingResource))
      (Networking|SwitchHasAuthority
        (:Authority
          (if _returnvalue_2
            (Development|PrintString "Server Interact")
            ;[1 1 1] GatherHolding
            (if (and (Variables|Default|GetCanInteract) (>= TriggeredSeconds _holdinginteracttimeinterval)) :!label _label
              (if (< (Math|Float|%(Float) (* TriggeredSeconds 6e+01) (* _holdinginteracttimeinterval 6e+01)) 0.2)
                (bind (_foundinteractable _interactableobject) (CallFunction|LookforInteractables :!label _label_2))
                ;[1 1 1] GatherObejct
                (Variables|Default|SetInteractable%20Object _interactableobject)
                (if _foundinteractable
                  (bind _returnvalue_3 (Class|Interactable|CanInteract(Message) _interactableobject))
                  (if _returnvalue_3
                    (CallFunction|ServerInteract _interactableobject self)))))))
        (:Remote
          (if _returnvalue_2
            (Development|PrintString "Client Interact")
            (goto _label))))))
  (:Started
    (Utilities|FlowControl|Sequence
      (:then_0
        (Variables|Default|SetCanChargeThrow true)
        (Variables|Default|SetThrowTime 0.0))
      (:then_1
        ;[1 1 1] GatherTap
        (if (not (Variables|Default|GetIsHoldingResource))
          (if (Variables|Default|GetCanInteract)
            (Variables|Default|SetCanInteract false)
            (Utilities|Time|SetTimerbyFunctionName 0 "EnableInteraction" (Variables|Default|GetInteractionTimeIntervalLimit))
            (goto _label_2))))
      (:then_2
        (bind _asbp_player_state (Utilities|Casting|CastToBP_PlayerState (Variables|/Script/Engine.Controller|GetPlayerState (Game|GetPlayerController 0))))
        (Default|OnInteract (Variables|Default|GetBP_CraftComponent) (.Team (Utilities|Struct|BreakPlayerInfo (Variables|/Script/Racketeers.PS_Base|GetPlayerInfo _asbp_player_state)))))
      (:then_3
        (if (== (Variables|Default|GetHoldingObjectVar) 0)
          (Default|Push (Variables|Default|GetBP_PusherComponent))))))
  (:Completed
    (Utilities|IsValid (Variables|Default|GetHoldingObjectVar)
      (:Is%20Valid
        (if (and (Variables|Default|GetCanChargeThrow) (Variables|Default|GetIsChargingThrow))
          (CallFunction|ServerThrow self (* (Variables|Default|GetThrowTime) 1e+03)))))))

(event Input|EnhancedActionEvents|EnhancedInputActionIA_Boat_Interact
  (params (ActionValue :type Boolean) (ElapsedSeconds :type Float%20%28double-precision%29) (TriggeredSeconds :type Float%20%28double-precision%29) (InputAction :type Input%20Action%20Object%20Reference :default "/Game/Racketeers/Characters/Input/Actions/IA_Boat_Interact.IA_Boat_Interact"))
  ;[1 1 1] Ship Inputs
  (:Started
    (bind _asbp_boat (Utilities|Casting|CastToBP_Boat (Variables|Default|GetInteractable%20Object)))
    (Default|LeaveBoatInteract _asbp_boat)))

(event Input|EnhancedActionEvents|EnhancedInputActionIA_Boat_ShootLeft
  (params (ActionValue :type Vector%202D%20Structure) (ElapsedSeconds :type Float%20%28double-precision%29) (TriggeredSeconds :type Float%20%28double-precision%29) (InputAction :type Input%20Action%20Object%20Reference :default "/Game/Racketeers/Characters/Input/Actions/IA_Boat_ShootLeft.IA_Boat_ShootLeft"))
  ;[1 1 1] Ship Inputs
  (:Started
    (CallFunction|ServerStartHoldShoot))
  (:Completed
    (CallFunction|ServerStopHoldShoot)
    (bind _asbp_boat (Utilities|Casting|CastToBP_Boat (Variables|Default|GetInteractable%20Object)))
    (Default|BoatShootLeft _asbp_boat)))

(event Input|EnhancedActionEvents|EnhancedInputActionIA_Boat_ShootRight
  (params (ActionValue :type Vector%202D%20Structure) (ElapsedSeconds :type Float%20%28double-precision%29) (TriggeredSeconds :type Float%20%28double-precision%29) (InputAction :type Input%20Action%20Object%20Reference :default "/Game/Racketeers/Characters/Input/Actions/IA_Boat_ShootRight.IA_Boat_ShootRight"))
  ;[1 1 1] Ship Inputs
  (:Started
    (CallFunction|ServerStartHoldShoot))
  (:Completed
    (CallFunction|ServerStopHoldShoot)
    (bind _asbp_boat (Utilities|Casting|CastToBP_Boat (Variables|Default|GetInteractable%20Object)))
    (Default|BoatShootRight _asbp_boat)))

(event Input|EnhancedActionEvents|EnhancedInputActionIA_Boat_Scurry
  (params (ActionValue :type Boolean) (ElapsedSeconds :type Float%20%28double-precision%29) (TriggeredSeconds :type Float%20%28double-precision%29) (InputAction :type Input%20Action%20Object%20Reference :default "/Game/Racketeers/Characters/Input/Actions/IA_Boat_Scurry.IA_Boat_Scurry"))
  ;[1 1 1] Ship Inputs
  (:Started
    (bind _asbp_boat (Utilities|Casting|CastToBP_Boat (Variables|Default|GetInteractable%20Object)))
    (Default|StartScurryBoat _asbp_boat)))

(event Input|EnhancedActionEvents|EnhancedInputActionIA_Scurry
  (params (ActionValue :type Boolean) (ElapsedSeconds :type Float%20%28double-precision%29) (TriggeredSeconds :type Float%20%28double-precision%29) (InputAction :type Input%20Action%20Object%20Reference :default "/Game/Racketeers/Characters/Input/Actions/IA_Scurry.IA_Scurry"))
  (:Started
    (Default|StartScurry (Variables|Default|GetBP_ScurryComponent))
    (Default|ServerRunningEffects (Variables|Default|GetEffectsComponent) (Variables|Default|GetStress) (Variables|Default|GetRunningEffect))))

(event Input|EnhancedActionEvents|EnhancedInputActionIA_Boat_Move
  (params (ActionValue :type Vector%202D%20Structure) (ElapsedSeconds :type Float%20%28double-precision%29) (TriggeredSeconds :type Float%20%28double-precision%29) (InputAction :type Input%20Action%20Object%20Reference :default "/Game/Racketeers/Characters/Input/Actions/IA_Boat_Move.IA_Boat_Move"))
  ;[1 1 1] Ship Inputs
  (:Triggered
    (bind _asbp_boat (Utilities|Casting|CastToBP_Boat (Variables|Default|GetInteractable%20Object)))
    (Default|MoveBoat _asbp_boat ActionValue))
  (:Completed
    (bind _asbp_boat_2 (Utilities|Casting|CastToBP_Boat (Variables|Default|GetInteractable%20Object)))
    (Default|StopBoat _asbp_boat_2 ActionValue)))

(event EventBeginPlay
  ;[1 1 1] Player indicator
  (if (Pawn|IsLocallyControlled)
    (Rendering|SetVisibility (Variables|Default|GetPlayerIndicator) true false)))

(event EventTick
  (params (DeltaSeconds :type Float%20%28single-precision%29))
  (Utilities|FlowControl|Sequence
    (:then_0
      (Variables|Default|SetShootTime (+ (Variables|Default|GetShootTime) DeltaSeconds))
      (if (Variables|Default|GetCanChargeThrow)
        (Variables|Default|SetThrowTime (+ (Variables|Default|GetThrowTime) DeltaSeconds))))))

(event Collision|EventHit
  (params (MyComp :type Primitive%20Component%20Object%20Reference) (Other :type Actor%20Object%20Reference) (OtherComp :type Primitive%20Component%20Object%20Reference) (bSelfMoved :type Boolean) (HitLocation :type Vector :default "0, 0, 0") (HitNormal :type Vector :default "0, 0, 0") (NormalImpulse :type Vector :default "0, 0, 0") (Hit :type Hit%20Result%20Structure%20%28by%20ref%29))
  (bind _returnvalue (Actor|GetComponentbyClass Other "/Game/Racketeers/Blueprints/Components/BP_ScurryComponent.BP_ScurryComponent_C"))
  ;[1 1 1] Scurry stuff (WIP)
  (Utilities|IsValid _returnvalue
    (:Is%20Valid
      (if (and (Variables|/Game/Racketeers/Blueprints/Components/BP_ScurryComponent.BP_ScurryComponent_C|GetIsScurrying (Variables|Default|GetBP_ScurryComponent)) (Variables|/Game/Racketeers/Blueprints/Components/BP_ScurryComponent.BP_ScurryComponent_C|GetIsScurrying _returnvalue))
        (CallFunction|ServerScurryonCollision Other (Variables|Default|GetBP_ScurryComponent))
        (CallFunction|ServerScurryonCollision self _returnvalue)))))

(event Input|KeyboardEvents|DebugKey3
  (params (Key :type Key%20Structure :default "None") (ActionValue :type Input%20Action%20Value%20Structure))
  (:Pressed
    (CallFunction|KickPlayer (Game|GetPlayerController 0) (Networking|IsServer))))

(event Input|KeyboardEvents|1
  (params (Key :type Key%20Structure :default "None"))
  (:Pressed
    (Networking|SwitchHasAuthority
      (:Authority
        (bind _asracketeers_controller (Utilities|Casting|CastToRacketeersController (Game|GetPlayerController 0)))
        (for _index (range 0 2)
          (Class|RacketeersController|AddResource _asracketeers_controller 50 (Utilities|Enum|ByteToEnumEResources (Math|Conversions|ToByte(Integer) _index)) "Team_Raccoon")
          (Class|RacketeersController|AddResource _asracketeers_controller 50 (Utilities|Enum|ByteToEnumEResources (Math|Conversions|ToByte(Integer) _index)) "Team_Panda"))))))

(event Input|KeyboardEvents|2
  (params (Key :type Key%20Structure :default "None"))
  (:Pressed
    (Networking|SwitchHasAuthority
      (:Authority
        (Class|TimerInfo|SetTime 0.0)))))

(event Input|KeyboardEvents|3
  (params (Key :type Key%20Structure :default "None"))
  (:Pressed
    (Networking|SwitchHasAuthority
      (:Authority
        (Class|TimerInfo|SetTime 1.2e+02)))))

(fn ConstructionScript)

(fn UpdatePlayerLobbyInfo
  (params (PlayerLobbyInfo :type Player%20Info%20Structure))
  (Variables|Default|SetPlayerInfo PlayerLobbyInfo))

(fn EnableInteraction
  (Variables|Default|SetCanInteract true))

(fn GatherHold
  (params (End :type Vector) (Start :type Vector) (Orientation :type Rotator) (ObjectTypes :type Array%20of%20EObjectTypeQuery%20Enums :default "ObjectTypeQuery1"))
  (bind _self self)
  (bind (_outhit _returnvalue) (Class|KismetSystemLibrary|BoxTraceSingleforObjects Start End "32.000000,32.000000,64.000000" Orientation ObjectTypes false 0 "ForDuration" true))
  (if (and _returnvalue (Utilities|DoesObjectImplementInterface (.HitActor (Collision|BreakHitResult _outhit)) "/Script/Racketeers.Interactable"))
    (bind _returnvalue_2 (Class|Interactable|CanInteract(Message) (.HitActor (Collision|BreakHitResult _outhit))))
    (if _returnvalue_2
      (Networking|SwitchHasAuthority
        (:Authority
          _)
        (:Remote
          ;[1 1 1] Client Prediction
          (Class|Interactable|StartInteract(Message) (.HitActor (Collision|BreakHitResult _outhit)) _self false)))
      (CallFunction|ServerInteract (.HitActor (Collision|BreakHitResult _outhit)) _self))))

(fn EnableHoldingInteraction
  (Variables|Default|SetHoldGatherTimmer true))

(fn LookforInteractables
  (bind _interactionlocation (Variables|Default|GetInteractionLocation))
  (bind _returnvalue (Transformation|GetWorldLocation _interactionlocation))
  (bind (_outhit _returnvalue_2) (Class|KismetSystemLibrary|BoxTraceSingleforObjects _returnvalue _returnvalue "32.000000,32.000000,64.000000" (Transformation|GetActorRotation) (Utilities|Array|MakeArray "ObjectTypeQuery2" "ObjectTypeQuery4") false 0 "ForDuration" true))
  (return (and _returnvalue_2 (Utilities|DoesObjectImplementInterface (.HitActor (Collision|BreakHitResult _outhit)) "/Script/Racketeers.Interactable")) (.HitActor (Collision|BreakHitResult _outhit))))

(fn OnRepPlayerInfo
  (bind _lobbyinfo (Variables|Default|GetLobbyInfo))
  (bind _returnvalue (UserInterface|GetWidget _lobbyinfo))
  (Utilities|IsValid _returnvalue
    (:Is%20Valid
      (bind _aswbp_player_lobby_info (Utilities|Casting|CastToWBP_PlayerLobbyInfo _returnvalue))
      (Default|Update _aswbp_player_lobby_info (Variables|Default|GetPlayerInfo))
      (Rendering|SetVisibility (Variables|Default|GetLobbyInfo) true false))
    (:Is%20Not%20Valid
      (Utilities|Time|SetTimerbyFunctionName 0 "OnRep_PlayerInfo" 0.1))))

(fn ThrowResource
  (params (IsUpwards :type Boolean) (Instigator :type Actor%20Object%20Reference) (ThrowForce :type Float%20%28double-precision%29))
  (bind _returnvalue (Math|Float|Clamp(Float) ThrowForce 3e+02 1e+03))
  (Utilities|FlowControl|Sequence
    (:then_0
      (switch Utilities|FlowControl|Switch|SwitchonEResources (Variables|Default|GetHoldingResourceType)
        (:WOOD
          (Variables|Default|SetSpawning%20Class "/Game/Racketeers/Blueprints/GatherableItems/BP_BaseResourceChunkWood.BP_BaseResourceChunkWood_C"))
        (:FIBER
          (Variables|Default|SetSpawning%20Class "/Game/Racketeers/Blueprints/GatherableItems/BP_BaseResourceChunkFiber.BP_BaseResourceChunkFiber_C"))
        (:METAL
          (Variables|Default|SetSpawning%20Class "/Game/Racketeers/Blueprints/GatherableItems/BP_BaseResourceChunkMetal.BP_BaseResourceChunkMetal_C"))))
    (:then_1
      (if (not IsUpwards)
        (bind _returnvalue_2 (Game|SpawnActorfromClass (Variables|Default|GetSpawning%20Class) (Transformation|GetWorldTransform (Variables|Default|GetHoldingObject)) "Undefined" "MultiplyWithRoot" self "1.000000,0.000000,0.000000" _returnvalue 0))
        (Variables|/Game/Racketeers/Blueprints/GatherableItems/BP_BaseResourceChunk.BP_BaseResourceChunk_C|SetMaxSpeed _returnvalue_2 _returnvalue)
        (Variables|/Script/Racketeers.BaseResourceChunk|SetLastOwner _returnvalue_2 self)
        (Variables|/Script/Racketeers.BaseResourceChunk|SetisBeingHeld _returnvalue_2 false)
        (Actor|DestroyActor (Variables|Default|GetHoldingObjectVar))
        (Variables|Default|SetHoldingObjectVar 0)
        (Components|StaticMesh|SetStaticMesh (Variables|Default|GetHoldingObject) 0)
        (Variables|Default|SetIsHoldingResource false)
        (Audio|PlaySoundatLocation "/Game/Racketeers/Audio/SFX/Player/SFX_Throw.SFX_Throw" (Transformation|GetActorLocation self) "0, 0, 0" 1.0 1.0 0.0 0 0 0 0)))))