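; Player Blueprint for Racketeers that handles networked interaction with world objects.
; The Interact input runs a debug-drawn box trace at InteractionLocation for a WorldDynamic actor implementing the Interactable interface.
; If the target allows interaction, the client predicts it by calling InteractMessage immediately, then forwards the request to a server event, which rechecks CanInteractMessage before applying it.
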(event Custom|Server_Interact
  (params (Target :type Actor%20Object%20Reference) (Instigator :type Actor%20Object%20Reference))
  ;[1 1 1] Server Logic
  (bind _returnvalue (Class|Interactable|CanInteract(Message) Target))
  (if _returnvalue
    (Class|Interactable|Interact(Message) Target Instigator)))

(event Input|EnhancedActionEvents|EnhancedInputActionIA_Interact
  (params (ActionValue :type Boolean) (ElapsedSeconds :type Float%20%28double-precision%29) (TriggeredSeconds :type Float%20%28double-precision%29) (InputAction :type Input%20Action%20Object%20Reference :default "/Game/Racketeers/Input/Actions/IA_Interact.IA_Interact"))
  (bind _self self)
  (bind _interactionlocation (Variables|Default|GetInteractionLocation))
  (bind _returnvalue (Transformation|GetWorldLocation _interactionlocation))
  (:Started
    (bind (_outhit _returnvalue_2) (Class|KismetSystemLibrary|BoxTraceSingleforObjects _returnvalue _returnvalue "32.000000,32.000000,64.000000" (Transformation|GetActorRotation) (Utilities|Array|MakeArray "ObjectTypeQuery2") false 0 "ForDuration" true))
    (if (and _returnvalue_2 (Utilities|DoesObjectImplementInterface (.HitActor (Collision|BreakHitResult _outhit)) "/Script/Racketeers.Interactable"))
      (bind _returnvalue_3 (Class|Interactable|CanInteract(Message) (.HitActor (Collision|BreakHitResult _outhit))))
      (if _returnvalue_3
        ;[1 1 1] Client Prediction
        (Class|Interactable|Interact(Message) (.HitActor (Collision|BreakHitResult _outhit)) _self)
        (CallFunction|ServerInteract (.HitActor (Collision|BreakHitResult _outhit)) _self)))))

(fn ConstructionScript)